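; Save-game manager for Super Fabio that persists the player's remaining lives between sessions.
; On BeginPlay it loads the SG_SuperFabio save from its slot, or creates and saves one if none exists, then copies LivesLeft into the player character's PlayerHealth.
; SaveNewLives writes a new lives count to the save object and saves it, using a hardcoded slot name rather than the SaveGameName variable.
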(event `self.ReceiveBeginPlay`
  ; Does Save Game Exist?
  (bind _returnvalue (`GameplayStatics.DoesSaveGameExist` (`self.SaveGameName`)))
  (if _returnvalue
    ; Load Save Game
    (bind _returnvalue_2 (`GameplayStatics.LoadGameFromSlot` (`self.SaveGameName`)))
    (bind _assg_super_fabio (cast `/Game/Super_Fabio/Blueprints/SG_SuperFabio` _returnvalue_2))
    (bind _output_get (set `self.As SG Super Fabio` _assg_super_fabio))
    (bind _asbp_sf_player_paper_character (cast `/Game/Super_Fabio/Blueprints/BP_SF_Player_Paper_Character` (`GameplayStatics.GetPlayerCharacter` 0)))
    (set `/Game/Super_Fabio/Blueprints/BP_SF_Player_Paper_Character.Player Health` (`/Game/Super_Fabio/Blueprints/SG_SuperFabio.LivesLeft` _output_get) _asbp_sf_player_paper_character)
    (else
      ; Create Save Game
      (bind _returnvalue_3 (`GameplayStatics.CreateSaveGameObject` "/Game/Super_Fabio/Blueprints/SG_SuperFabio.SG_SuperFabio_C"))
      (`GameplayStatics.SaveGameToSlot` _returnvalue_3 (`self.SaveGameName`))
      (bind _output_get_2 (set `self.As SG Super Fabio` _returnvalue_3))
      (bind _asbp_sf_player_paper_character_2 (cast `/Game/Super_Fabio/Blueprints/BP_SF_Player_Paper_Character` (`GameplayStatics.GetPlayerCharacter` 0)))
      (set `/Game/Super_Fabio/Blueprints/BP_SF_Player_Paper_Character.Player Health` (`/Game/Super_Fabio/Blueprints/SG_SuperFabio.LivesLeft` _output_get_2) _asbp_sf_player_paper_character_2))))

(event `SaveNewLives`
  (params (CurrentLives :type Integer))
  (bind _as_sg_super_fabio (`self.As SG Super Fabio`))
  ; Save New Lives
  (set `/Game/Super_Fabio/Blueprints/SG_SuperFabio.LivesLeft` CurrentLives _as_sg_super_fabio)
  (`GameplayStatics.SaveGameToSlot` _as_sg_super_fabio "SG_SuperFabio"))

(fn `UserConstructionScript`)