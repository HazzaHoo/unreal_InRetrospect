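; Player character Blueprint for the Super Fabio game, handling input setup, pausing and key-based progression.
; BeginPlay adds the game and global Enhanced Input mapping contexts, though the move, jump and interact events are empty.
; The pause action toggles a pause menu widget, game pause, input mode and cursor.
; Overlaps set HasKey on key pickup, while the progression portal calls LoadLevelInstance only when HasKey is false, with no level specified.
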(event `self.ReceiveBeginPlay`
  ; Player Control
  (set `self.SuperFabio_Game` true)
  (bind _asplayer_controller (cast `PlayerController` (`self.GetController`)))
  (bind _returnvalue (pcsubsystem `EnhancedInputLocalPlayerSubsystem` _asplayer_controller))
  (`/Engine/EditorBlueprintResources/StandardMacros.IsValid` _returnvalue
    (:`Is Valid`
      (`EnhancedInputSubsystemInterface.AddMappingContext` _returnvalue "/Game/Super_Fabio/IMC/IMC_SuperFabio.IMC_SuperFabio" 0 (struct))
      (`EnhancedInputSubsystemInterface.AddMappingContext` _returnvalue "/Game/Global_IMC/IMC_Global.IMC_Global" 0 (struct)))))

(event `EnhancedInput|/Game/Super_Fabio/IMC/IA_SF_Interact`
  (params (ActionValue :type Boolean) (ElapsedSeconds :type "Float (double-precision)") (TriggeredSeconds :type "Float (double-precision)") (InputAction :type "InputAction Object Reference" :default "/Game/Super_Fabio/IMC/IA_SF_Interact.IA_SF_Interact"))
  ; Player Control
)

(event `EnhancedInput|/Game/Super_Fabio/IMC/IA_SF_Jump`
  (params (ActionValue :type Boolean) (ElapsedSeconds :type "Float (double-precision)") (TriggeredSeconds :type "Float (double-precision)") (InputAction :type "InputAction Object Reference" :default "/Game/Super_Fabio/IMC/IA_SF_Jump.IA_SF_Jump"))
  ; Player Control
)

(event `EnhancedInput|/Game/Super_Fabio/IMC/IA_SF_Move`
  (params (ActionValue :type "Vector2D Structure") (ElapsedSeconds :type "Float (double-precision)") (TriggeredSeconds :type "Float (double-precision)") (InputAction :type "InputAction Object Reference" :default "/Game/Super_Fabio/IMC/IA_SF_Move.IA_SF_Move"))
  ; Player Control
)

(event `EnhancedInput|/Game/Global_IMC/IA_Pause`
  (params (ActionValue :type Boolean) (ElapsedSeconds :type "Float (double-precision)") (TriggeredSeconds :type "Float (double-precision)") (InputAction :type "InputAction Object Reference" :default "/Game/Global_IMC/IA_Pause.IA_Pause"))
  (bind _returnvalue (`GameplayStatics.GetPlayerController` 0))
  ;[0.15 0 0 0.5] Call Pause Menu
  (:`Completed`
    (if (not (`self.IsPauseMenuOpen`))
      (set `self.IsPauseMenuOpen` true)
      (bind _returnvalue_2 (`|CreateWidget` "/Game/Global_Userinterface/Pause/WBP_PauseMenu.WBP_PauseMenu_C" _returnvalue false false false false (`self.SuperFabio_Game`)))
      (bind _output_get (set `self.UnpauseMenuWidget` _returnvalue_2))
      (`UserWidget.AddToViewport` _output_get 0)
      (`WidgetBlueprintLibrary.SetInputMode_GameAndUIEx` _returnvalue null)
      (set `PlayerController.bShowMouseCursor` true (`GameplayStatics.GetPlayerController` 0))
      (`GameplayStatics.SetGamePaused` true)
      (else
        (set `self.IsPauseMenuOpen` false)
        (`Widget.RemoveFromParent` (`self.UnpauseMenuWidget`))
        (`GameplayStatics.SetGamePaused` false)
        (`WidgetBlueprintLibrary.SetInputMode_GameOnly` _returnvalue)
        (set `PlayerController.bShowMouseCursor` false (`GameplayStatics.GetPlayerController` 0))))))

(event `self.ReceiveActorBeginOverlap`
  (params (OtherActor :type "Actor Object Reference"))
  ; Progression Logic
  (`|ExecutionSequence`
    (:`then_0`
      ; Pick up Key
      (cast `/Game/Super_Fabio/Blueprints/BP_SF_Key` OtherActor)
      (set `self.hasKey` true))
    (:`then_1`
      (cast `/Game/Ping/Blueprints/BP_Ping_Progression_Portal` OtherActor)
      (if (not (`self.hasKey`))
        (`LevelStreamingDynamic.LoadLevelInstance` "" (0.0 0.0 0.0) (struct) "" null)))))

(fn `UserConstructionScript`)