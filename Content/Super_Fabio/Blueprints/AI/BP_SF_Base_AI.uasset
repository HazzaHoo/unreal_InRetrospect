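; Base enemy for the Super Fabio 2D platformer that patrols horizontally, kills the player on contact and can be stomped.
; Tick drives movement; side detectors reverse direction and rotate the sprite on obstacles not tagged Player, AI or Pickup, with DoOnce gates halting momentum.
; SquashDetector sets Stomped, calls the empty OnStomped hook and bounces the player, while KillBox shows game over unless stomped.
; Construction applies the SpriteChar flipbook; destroy-on-hit logic is disconnected.
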(event `self.KillBox.OnComponentBeginOverlap`
  (params (OverlappedComponent :type "PrimitiveComponent Object Reference") (OtherActor :type "Actor Object Reference") (OtherComp :type "PrimitiveComponent Object Reference") (OtherBodyIndex :type Integer) (bFromSweep :type Boolean) (SweepResult :type "HitResult Structure (by ref)"))
  (if (`self.Stomped?`)
    _
    (elif (`self.ActorHasTag` OtherActor "Player")
      (`/Engine/EditorBlueprintResources/StandardMacros.DoOnce` false
        (:`Completed`
          (bind _returnvalue (`|CreateWidget` "/Game/Super_Fabio/UserInterface/WB_GameOver_SuperFabio.WB_GameOver_SuperFabio_C"))
          (`UserWidget.AddToViewport` _returnvalue 0))))))

(event `self.Squash Detector.OnComponentBeginOverlap`
  (params (OverlappedComponent :type "PrimitiveComponent Object Reference") (OtherActor :type "Actor Object Reference") (OtherComp :type "PrimitiveComponent Object Reference") (OtherBodyIndex :type Integer) (bFromSweep :type Boolean) (SweepResult :type "HitResult Structure (by ref)"))
  ; Squash Detector
  (if (`self.ActorHasTag` OtherActor "Player")
    (set `self.Stomped?` true)
    (`self.OnStomped`)
    ; Launch Character if Stomped On
    (bind _asbp_sf_player_paper_character (cast `/Game/Super_Fabio/Blueprints/BP_SF_Player_Paper_Character` OtherActor))
    (`self.LaunchCharacter` _asbp_sf_player_paper_character (0.0 0.0 750.0) false true)))

(event `OnStomped`
  ; Squash Detector
)

(event `self.Left Detector.OnComponentBeginOverlap`
  (params (OverlappedComponent :type "PrimitiveComponent Object Reference") (OtherActor :type "Actor Object Reference") (OtherComp :type "PrimitiveComponent Object Reference") (OtherBodyIndex :type Integer) (bFromSweep :type Boolean) (SweepResult :type "HitResult Structure (by ref)"))
  ; Dead
  (if (not (or (`self.ActorHasTag` OtherActor "Player") (`self.ActorHasTag` OtherActor "AI") (`self.ActorHasTag` OtherActor "Pickup")))
    (set `self.ShouldGoLeftSide` false)
    (`SceneComponent.K2_SetWorldRotation` :`self` (`self.Sprite`))))

(event `self.Right Detector.OnComponentBeginOverlap`
  (params (OverlappedComponent :type "PrimitiveComponent Object Reference") (OtherActor :type "Actor Object Reference") (OtherComp :type "PrimitiveComponent Object Reference") (OtherBodyIndex :type Integer) (bFromSweep :type Boolean) (SweepResult :type "HitResult Structure (by ref)"))
  ; Dead
  (if (not (or (`self.ActorHasTag` OtherActor "Player") (`self.ActorHasTag` OtherActor "AI") (`self.ActorHasTag` OtherActor "Pickup")))
    (set `self.ShouldGoLeftSide` true)
    (`SceneComponent.K2_SetWorldRotation` (`self.Sprite`) (struct :`Yaw` 180.0) false false)))

(event `self.ReceiveHit`
  (params (MyComp :type "PrimitiveComponent Object Reference") (Other :type "Actor Object Reference") (OtherComp :type "PrimitiveComponent Object Reference") (bSelfMoved :type Boolean) (HitLocation :type "Vector Structure") (HitNormal :type "Vector Structure") (NormalImpulse :type "Vector Structure") (Hit :type "HitResult Structure (by ref)"))
  ;[0.15 0 0 0.5] Kills Enemy
)

(event `self.ReceiveTick`
  (params (DeltaSeconds :type "Float (single-precision)"))
  ; Move Left or Right
  (if (`self.ShouldGoLeftSide`)
    (`self.AddMovementInput` (-1.0 0.0 0.0) 1.0 true)
    (`|ExecutionSequence`
      (:`then_0`
        (`/Engine/EditorBlueprintResources/StandardMacros.DoOnce` false :!label _label
          (:`Completed`
            _)))
      (:`then_1`
        (goto _label_2 :!via `Reset`)))
    (else
      (`self.AddMovementInput` (1.0 0.0 0.0) 1.0 true)
      (`|ExecutionSequence`
        (:`then_0`
          (goto _label :!via `Reset`))
        (:`then_1`
          (`/Engine/EditorBlueprintResources/StandardMacros.DoOnce` false :!label _label_2
            (:`Completed`
              _))))))
  (`MovementComponent.StopMovementImmediately` (`self.CharacterMovement`)))

(fn `UserConstructionScript`
  (`PaperFlipbookComponent.SetFlipbook` (`self.Sprite`) (`self.SpriteChar`)))