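; BP_SF_Roomba_AI is a stompable Roomba enemy in Super Fabio, whose own graph only handles its death.
; OnStomped plays a hit sound and kill VFX, hides the sprite, disables the squash, side and kill-box collisions, and stops the hoover sound.
; It destroys the actor after a short delay.
; No movement or detection logic appears here, and the construction script only calls the parent.
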(event `self.OnStomped`
  (`GameplayStatics.PlaySound2D` "/Game/Super_Fabio/Audio/EnemyHit.EnemyHit" 1.0 1.0 0.0 null null)
  (`ActorComponent.Activate` (`self.Kill_VFX`) false)
  (`SceneComponent.SetHiddenInGame` (`self.Sprite`) true false)
  (`PrimitiveComponent.SetCollisionEnabled` (`self.Squash Detector`) "NoCollision")
  (`PrimitiveComponent.SetCollisionEnabled` (`self.Right Detector`) "NoCollision")
  (`PrimitiveComponent.SetCollisionEnabled` (`self.Left Detector`) "NoCollision")
  (`PrimitiveComponent.SetCollisionEnabled` (`self.KillBox`) "NoCollision")
  (`AudioComponent.Stop` (`self.RoombaHoover_Cue`))
  (`KismetSystemLibrary.Delay` 1.0)
  (`self.K2_DestroyActor`))

(fn `UserConstructionScript`
  (`parent.UserConstructionScript`))