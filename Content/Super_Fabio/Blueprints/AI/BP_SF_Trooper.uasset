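; BP_SF_Trooper is a hovering enemy in Super Fabio that the player can bounce on or be killed by.
; Overlapping its squash detector launches the player upward with a helmet-jump sound.
; A one-shot OnStomped event swaps the sprite for a helmet, disables hit boxes, switches hover audio to Niagara effects and changes walk speed.
; Kill box overlaps with the Player tag show the game-over widget once, after a brief delay.
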(event `self.Squash Detector1.OnComponentBeginOverlap`
  (params (OverlappedComponent :type "PrimitiveComponent Object Reference") (OtherActor :type "Actor Object Reference") (OtherComp :type "PrimitiveComponent Object Reference") (OtherBodyIndex :type Integer) (bFromSweep :type Boolean) (SweepResult :type "HitResult Structure (by ref)"))
  (bind _asbp_sf_player_paper_character (cast `/Game/Super_Fabio/Blueprints/BP_SF_Player_Paper_Character` OtherActor))
  (`self.LaunchCharacter` _asbp_sf_player_paper_character (0.0 0.0 750.0) false true)
  (`GameplayStatics.PlaySound2D` "/Game/Super_Fabio/Audio/HelmetJump.HelmetJump" 1.0 1.0 0.0 null null))

(event `self.OnStomped`
  (`/Engine/EditorBlueprintResources/StandardMacros.DoOnce` false
    (:`Completed`
      (`SceneComponent.SetVisibility` (`self.Helmet`) true false)
      (`SceneComponent.SetVisibility` (`self.Sprite`) false false)
      (`PrimitiveComponent.SetCollisionEnabled` (`self.Squash Detector`) "NoCollision")
      (`PrimitiveComponent.SetCollisionEnabled` (`self.KillBox`) "NoCollision")
      (`ActorComponent.Activate` (`self.Niagara`) false)
      (`AudioComponent.Stop` (`self.TrooperHoover_Cue`))
      (set `CharacterMovementComponent.MaxWalkSpeed` 600.0 (`self.CharacterMovement`))
      (`GameplayStatics.PlaySound2D` "/Game/Super_Fabio/Audio/EnemyHit.EnemyHit" 1.0 1.0 0.0 null null))))

(event `self.KillBox1.OnComponentBeginOverlap`
  (params (OverlappedComponent :type "PrimitiveComponent Object Reference") (OtherActor :type "Actor Object Reference") (OtherComp :type "PrimitiveComponent Object Reference") (OtherBodyIndex :type Integer) (bFromSweep :type Boolean) (SweepResult :type "HitResult Structure (by ref)"))
  (`KismetSystemLibrary.Delay` 0.05)
  (if (`self.ActorHasTag` OtherActor "Player")
    (`/Engine/EditorBlueprintResources/StandardMacros.DoOnce` false
      (:`Completed`
        (bind _returnvalue (`|CreateWidget` "/Game/Super_Fabio/UserInterface/WB_GameOver_SuperFabio.WB_GameOver_SuperFabio_C"))
        (`UserWidget.AddToViewport` _returnvalue 0)))))

(fn `UserConstructionScript`
  (`parent.UserConstructionScript`))