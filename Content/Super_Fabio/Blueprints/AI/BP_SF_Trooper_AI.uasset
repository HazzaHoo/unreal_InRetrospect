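; BP_SF_Trooper_AI is a simple patrolling trooper AI in the Super Fabio game.
; Every tick it feeds movement input along its forward vector, so it walks continuously.
; An overlap beginning on WalkDetector or ending on LedgeDetector calls TurnChar, which applies a 180-degree rotation to reverse it at obstacles and ledges.
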(event `self.ReceiveTick`
  (params (DeltaSeconds :type "Float (single-precision)"))
  (`self.Move Forward`))

(event `Move Forward`
  ;[0.01581 0.15 0 0.5] Start
  ;; AC Function
  (`self.AddMovementInput` (`self.GetActorForwardVector`)))

(event `self.WalkDetector.OnComponentBeginOverlap`
  (params (OverlappedComponent :type "PrimitiveComponent Object Reference") (OtherActor :type "Actor Object Reference") (OtherComp :type "PrimitiveComponent Object Reference") (OtherBodyIndex :type Integer) (bFromSweep :type Boolean) (SweepResult :type "HitResult Structure (by ref)"))
  ;[0.15 0 0 0.5] Functionality
  (`self.TurnChar`))

(event `self.LedgeDetector.OnComponentEndOverlap`
  (params (OverlappedComponent :type "PrimitiveComponent Object Reference") (OtherActor :type "Actor Object Reference") (OtherComp :type "PrimitiveComponent Object Reference") (OtherBodyIndex :type Integer))
  ;[0.15 0 0 0.5] Functionality
  (`self.TurnChar`))

(fn `TurnChar`
  (`self.K2_SetActorRotation` (`KismetMathLibrary.ComposeRotators` (`self.K2_GetActorRotation`) (struct :`Yaw` -180.0))))

(fn `UserConstructionScript`)