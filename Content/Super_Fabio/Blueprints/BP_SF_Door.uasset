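; BP_SF_Door is a locked door in the Super Fabio game that opens when the player character arrives carrying a key.
; On overlap of its key check collision, it clears the player's HasKey flag and calls DestroyKey on the first BP_KeyPickup found in the level.
; It then swaps the closed door component for the open one and disables the blocking collision so the way is clear.
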(event `self.KeyCheckCollision.OnComponentBeginOverlap`
  (params (OverlappedComponent :type "PrimitiveComponent Object Reference") (OtherActor :type "Actor Object Reference") (OtherComp :type "PrimitiveComponent Object Reference") (OtherBodyIndex :type Integer) (bFromSweep :type Boolean) (SweepResult :type "HitResult Structure (by ref)"))
  (bind _asbp_sf_player_paper_character (cast `/Game/Super_Fabio/Blueprints/BP_SF_Player_Paper_Character` OtherActor))
  (if (`/Game/Super_Fabio/Blueprints/BP_SF_Player_Paper_Character.hasKey` _asbp_sf_player_paper_character)
    (set `/Game/Super_Fabio/Blueprints/BP_SF_Player_Paper_Character.hasKey` false _asbp_sf_player_paper_character)
    (bind _outactors (`GameplayStatics.GetAllActorsOfClass` "/Game/Super_Fabio/Blueprints/BP_KeyPickup.BP_KeyPickup_C"))
    (`/Game/Super_Fabio/Blueprints/BP_KeyPickup.DestroyKey` (`|GetArrayItem` _outactors))
    (`SceneComponent.SetHiddenInGame` (`self.DoorOpen`) false false)
    (`SceneComponent.SetHiddenInGame` (`self.DoorClosed`) true false)
    (`PrimitiveComponent.SetCollisionEnabled` (`self.BlockingVolumeCollision`) "NoCollision")))

(fn `UserConstructionScript`)