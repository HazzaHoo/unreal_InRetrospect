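; Key pickup for Super Fabio that, once touched by the player's Paper character, trails that player until DestroyKey removes it.
; Timelines started on BeginPlay animate the key sprite's idle movement and rocking.
; Capsule overlap stores the player and, once only, shows a bubble sprite, plays a sound and rescales the key.
; Tick then lerps the actor toward a point above the player's capsule, scaled by FollowSpeed.
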(event `DestroyKey`
  ; Destroy Key
  (`self.K2_DestroyActor`))

(event `self.ReceiveTick`
  (params (DeltaSeconds :type "Float (single-precision)"))
  ; Move Key to Player
  (if (`self.GotKey`)
    (`self.K2_SetActorLocation` (`KismetMathLibrary.VLerp` (`self.K2_GetActorLocation`) (+ (`SceneComponent.K2_GetComponentLocation` (`Character.CapsuleComponent` (`self.Player Ref`))) (0.0 1.0 50.0)) (* DeltaSeconds (`self.FollowSpeed`))))))

(event `self.Capsule.OnComponentBeginOverlap`
  (params (OverlappedComponent :type "PrimitiveComponent Object Reference") (OtherActor :type "Actor Object Reference") (OtherComp :type "PrimitiveComponent Object Reference") (OtherBodyIndex :type Integer) (bFromSweep :type Boolean) (SweepResult :type "HitResult Structure (by ref)"))
  (bind _key_sprite (`self.Key_Sprite`))
  (bind _asbp_sf_player_paper_character (cast `/Game/Super_Fabio/Blueprints/BP_SF_Player_Paper_Character` OtherActor))
  ; Pick Up Key (Player)
  (set `self.Player Ref` _asbp_sf_player_paper_character)
  (`/Engine/EditorBlueprintResources/StandardMacros.DoOnce` false
    (:`Completed`
      (set `self.GotKey` true)
      (`SceneComponent.SetHiddenInGame` (`self.Bubble_Sprite`) false false)
      (`GameplayStatics.PlaySound2D` "/Game/Super_Fabio/Audio/KeyPickup.KeyPickup" 1.0 1.0 0.0 null null)
      (bind (_direction _lerp) (`Timeline|Scale Lerp`)
        (:`Update`
          (`SceneComponent.SetRelativeScale3D` _key_sprite (`KismetMathLibrary.VLerp` (`SceneComponent.RelativeScale3D` _key_sprite) (0.2 0.2 0.2) _lerp)))))))

(event `self.ReceiveBeginPlay`
  (bind _key_sprite (`self.Key_Sprite`))
  (bind _returnvalue (`SceneComponent.GetRelativeTransform` (`self.Key_Sprite`)))
  ; Idle Animations
  (set `self.StartPos(Relative)` _returnvalue)
  (set `self.EndPos(Relactive)` (`KismetMathLibrary.MakeTransform` (.location (`self.EndPos(Relactive)`)) (.rotation (`self.EndPos(Relactive)`)) (.scale _returnvalue)))
  (`|ExecutionSequence`
    (:`then_0`
      (bind (_direction _lerp) (`Timeline|IdleAnimation`)
        (:`Update`
          (`SceneComponent.K2_SetRelativeLocation` _key_sprite (.location (`KismetMathLibrary.TLerp` (`self.StartPos(Relative)`) (`self.EndPos(Relactive)`) _lerp)) false false))))
    (:`then_1`
      (bind (_direction_2 _lerp_2) (`Timeline|Timeline`)
        (:`Update`
          (`SceneComponent.K2_SetRelativeRotation` _key_sprite (`KismetMathLibrary.RLerp` (struct :`Pitch` 15.0) (struct :`Pitch` -15.0) _lerp_2) false false))))))

(fn `UserConstructionScript`)