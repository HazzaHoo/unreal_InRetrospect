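; End-of-level portal for Super Fabio that moves the player on to the next game, with its sprite animated by two idle timelines for position and rotation.
; The first player overlap either loads out to the modern arcade if the game is finished, or shows the end-game widget and disables movement.
; OpenNewGame records the 50-coin secret in the game instance, pauses, fades music and starts the era transition to Crash Capybara.
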(event `self.Portal Trigger.OnComponentBeginOverlap`
  (params (OverlappedComponent :type "PrimitiveComponent Object Reference") (OtherActor :type "Actor Object Reference") (OtherComp :type "PrimitiveComponent Object Reference") (OtherBodyIndex :type Integer) (bFromSweep :type Boolean) (SweepResult :type "HitResult Structure (by ref)"))
  (bind _asbp_sf_player_paper_character (cast `/Game/Super_Fabio/Blueprints/BP_SF_Player_Paper_Character` OtherActor))
  (`/Engine/EditorBlueprintResources/StandardMacros.DoOnce` false
    (:`Completed`
      (`ActorComponent.SetActive` (`self.Portal Trigger`) true false)
      (bind _asglobal_instance (cast `/Game/Global_IMC/Global_Instance` (`GameplayStatics.GetGameInstance`)))
      (if (`/Game/Global_IMC/Global_Instance.IsGameFinished?` _asglobal_instance)
        (bind _returnvalue (`|CreateWidget` "/Game/Global_Userinterface/WB_LoadInOrOut.WB_LoadInOrOut_C"))
        (`/Game/Global_Userinterface/WB_LoadInOrOut.Load Out` _returnvalue)
        (`UserWidget.AddToViewport` _returnvalue 0)
        (`KismetSystemLibrary.Delay` 0.5)
        (`GameplayStatics.OpenLevel` "L_Modern_Arcade")
        (else
          (bind _returnvalue_2 (`|CreateWidget` "/Game/Super_Fabio/UserInterface/WB_SF_EndGame.WB_SF_EndGame_C"))
          (`UserWidget.AddToViewport` _returnvalue_2 0)
          (`CharacterMovementComponent.DisableMovement` (`Character.CharacterMovement` _asbp_sf_player_paper_character)))))))

(event `self.ReceiveBeginPlay`
  ;[0 0.15 0.002719 0.5] Hide at the start of the level
  (`self.Idle Animations`)
  (`ActorComponent.SetActive` (`self.Portal Trigger`) false false))

(event `SetEndGameSecret`
  (bind _asbp_sf_player_paper_character (cast `/Game/Super_Fabio/Blueprints/BP_SF_Player_Paper_Character` (`GameplayStatics.GetPlayerCharacter` 0)))
  (if (>= (`/Game/Super_Fabio/Blueprints/BP_SF_Player_Paper_Character.Coins` _asbp_sf_player_paper_character) 50)
    (bind _asglobal_instance (cast `/Game/Global_IMC/Global_Instance` (`GameplayStatics.GetGameInstance`)))
    (set `/Game/Global_IMC/Global_Instance.SuperFabio50+Coins` true _asglobal_instance)))

(event `OpenNewGame`
  ;[0.005771 0.15 0 0.5] activate
  (`self.SetEndGameSecret`)
  (`GameplayStatics.SetGamePaused` true)
  (bind _returnvalue (`|CreateWidget` "/Game/Global_Userinterface/WB_Transition.WB_Transition_C"))
  (`/Game/Global_Userinterface/WB_Transition.WhatEra?` _returnvalue "1" "9" "9" "L_Crash_Capybara")
  (`UserWidget.AddToViewport` _returnvalue 0)
  (bind _outactors (`GameplayStatics.GetAllActorsOfClass` "/Game/Super_Fabio/Blueprints/BP_SF_Player_Paper_Character.BP_SF_Player_Paper_Character_C"))
  (`/Game/Super_Fabio/Blueprints/BP_SF_Player_Paper_Character.FadeMusicOut` (`|GetArrayItem` _outactors) 1.0))

(event `Idle Animations`
  (bind _papersprite (`self.PaperSprite`))
  (bind _returnvalue (`SceneComponent.GetRelativeTransform` (`self.PaperSprite`)))
  ; Idle Animations
  (set `self.StartPos(Relative)` _returnvalue)
  (set `self.EndPos(Relactive)` (`KismetMathLibrary.MakeTransform` (.location (`self.EndPos(Relactive)`)) (.rotation (`self.EndPos(Relactive)`)) (.scale _returnvalue)))
  (`|ExecutionSequence`
    (:`then_0`
      (bind (_direction _lerp) (`Timeline|Timeline`)
        (:`Update`
          (`SceneComponent.K2_SetRelativeLocation` _papersprite (.location (`KismetMathLibrary.TLerp` (`self.StartPos(Relative)`) (`self.EndPos(Relactive)`) _lerp)) false false))))
    (:`then_1`
      (bind (_direction_2 _lerp_2) (`Timeline|Timeline_0`)
        (:`Update`
          (`SceneComponent.K2_SetRelativeRotation` _papersprite (`KismetMathLibrary.RLerp` (struct :`Pitch` 75.0) (struct :`Pitch` 105.0) _lerp_2) false false))))))

(fn `UserConstructionScript`)