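; Placeholder player character Blueprint for Super Fabio, with logic meant to be moved to the actual character Blueprint.
; Enhanced Input events drive jumping with an IsJumping flag, and pass move input to AddMovementInput with a zero world direction.
; An unfinished overlap handler, flagged as a mess, checks for pipe entrances and the interact input, or another placeholder character, to set that character's location to world origin.
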(event `EnhancedInput|/Game/Super_Fabio/IMC/IA_SF_Jump`
  (params (ActionValue :type Boolean) (ElapsedSeconds :type "Float (double-precision)") (TriggeredSeconds :type "Float (double-precision)") (InputAction :type "InputAction Object Reference" :default "/Game/Super_Fabio/IMC/IA_SF_Jump.IA_SF_Jump"))
  ;[0 0 0.981 0.5] Transfer this over to the actual character blueprint
  ;;[0 0.15 0.006247 0.5] Jumping
  (:`Started`
    (`self.Jump`)
    (set `self.isJumping` true))
  (:`Canceled`
    (`self.StopJumping`)
    (set `self.isJumping` false)))

(event `EnhancedInput|/Game/Super_Fabio/IMC/IA_SF_Move`
  (params (ActionValue :type "Float (double-precision)") (ElapsedSeconds :type "Float (double-precision)") (TriggeredSeconds :type "Float (double-precision)") (InputAction :type "InputAction Object Reference" :default "/Game/Super_Fabio/IMC/IA_SF_Move.IA_SF_Move"))
  ;[0 0 0.981 0.5] Transfer this over to the actual character blueprint
  ;;[0 0.15 0.006247 0.5] Movement
  (:`Triggered`
    (`self.AddMovementInput` (0.0 0.0 0.0) ActionValue)))

(event `self.ReceiveActorBeginOverlap`
  (params (OtherActor :type "Actor Object Reference"))
  ;[0 0 0.981 0.5] Transfer this over to the actual character blueprint
  ;;[0.15 0 0 0.5] dm: This is a complete Mess. I'm fairly certain I have done this wrong. I'm gong to find a tutorial do this properly
  (`|ExecutionSequence`
    (:`then_0`
      (cast `/Game/Super_Fabio/Blueprints/BP_SF_Pipe_In` OtherActor)
      (if (not (`|GetInputActionValue`))
        (`SceneComponent.K2_SetWorldLocation` (`Actor.RootComponent` (stale _asplace_holder_bp_sf_player_character)) (0.0 0.0 0.0) false false :!label _label)))
    (:`then_1`
      (bind _asplace_holder_bp_sf_player_character (cast `/Game/Super_Fabio/Blueprints/PlaceHolder_BP_SF_Player_Character` OtherActor))
      (goto _label))))

(fn `UserConstructionScript`)