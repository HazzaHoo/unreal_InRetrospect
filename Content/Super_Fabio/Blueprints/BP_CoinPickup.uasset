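; Collectible coin pickup for Super Fabio that adds one to the player character's Coins.
; After a short overlap delay, a player cast and DoOnce gate the award, which hides the sprite, sets PickedUp, activates VFX and plays a sound.
; Two timelines animate the idle sprite, moving it between relative positions and rocking its rotation.
; A SpawnCoin event applies an up-and-sideways force, then a delayed downward one.
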(event `self.Capsule.OnComponentBeginOverlap`
  (params (OverlappedComponent :type "PrimitiveComponent Object Reference") (OtherActor :type "Actor Object Reference") (OtherComp :type "PrimitiveComponent Object Reference") (OtherBodyIndex :type Integer) (bFromSweep :type Boolean) (SweepResult :type "HitResult Structure (by ref)"))
  (`KismetSystemLibrary.Delay` 0.2)
  (bind _asbp_sf_player_paper_character (cast `/Game/Super_Fabio/Blueprints/BP_SF_Player_Paper_Character` OtherActor))
  (`/Engine/EditorBlueprintResources/StandardMacros.DoOnce` false
    (:`Completed`
      (set `/Game/Super_Fabio/Blueprints/BP_SF_Player_Paper_Character.Coins` (+ (`/Game/Super_Fabio/Blueprints/BP_SF_Player_Paper_Character.Coins` _asbp_sf_player_paper_character) 1) _asbp_sf_player_paper_character)
      (`SceneComponent.SetHiddenInGame` (`self.Coin_Sprite`) true true)
      (set `self.PickedUp?` true)
      (`ActorComponent.Activate` (`self.SF_CoinPickup_VFX`) true)
      (`GameplayStatics.PlaySound2D` "/Game/Super_Fabio/Audio/Pickup.Pickup" 1.0 1.0 0.0 null null))))

(event `self.ReceiveBeginPlay`
  (bind _coin_sprite (`self.Coin_Sprite`))
  ; Idle Animations
  (`KismetSystemLibrary.Delay` 0.2)
  (set `self.Start Pos(Relative)` (`self.Start Pos(Relative)`))
  (set `self.EndPos(Relactive)` (`KismetMathLibrary.MakeTransform` (.location (`self.EndPos(Relactive)`)) (.rotation (`self.EndPos(Relactive)`)) (.scale (`SceneComponent.GetRelativeTransform` (`self.Coin_Sprite`)))))
  (`|ExecutionSequence`
    (:`then_0`
      (bind (_direction _lerp) (`Timeline|Timeline`)
        (:`Update`
          (`SceneComponent.K2_SetRelativeLocation` _coin_sprite (.location (`KismetMathLibrary.TLerp` (`self.Start Pos(Relative)`) (`self.EndPos(Relactive)`) _lerp)) false false))))
    (:`then_1`
      (bind (_direction_2 _lerp_2) (`Timeline|Timeline_0`)
        (:`Update`
          (`SceneComponent.K2_SetRelativeRotation` _coin_sprite (`KismetMathLibrary.RLerp` (struct :`Pitch` 5.0) (struct :`Pitch` -5.0) _lerp_2) false false))))))

(event `SpawnCoin`
  (`PhysicsThreadLibrary.AddForce` (struct) (0.5 0.0 1.0))
  (`KismetSystemLibrary.Delay` 0.2)
  (`PhysicsThreadLibrary.AddForce` (struct) (0.0 0.0 -10.0)))

(fn `UserConstructionScript`)