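; Trooper enemy for the Super Fabio game that changes into a helmet form when stomped.
; On the first stomp only, it hides the sprite, shows the helmet and deactivates the squash detector.
; It also lowers and shrinks the left and right detectors and sets a new max walk speed.
; The graph holds only this stomp response, with no movement logic of its own.
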(event `self.OnStomped`
  (bind _right_detector (`self.Right Detector`))
  (bind _left_detector (`self.Left Detector`))
  (`/Engine/EditorBlueprintResources/StandardMacros.DoOnce` false
    (:`Completed`
      (`SceneComponent.SetVisibility` (`self.Helmet`) true false)
      (`SceneComponent.SetVisibility` (`self.Sprite`) false false)
      (`ActorComponent.SetActive` (`self.Squash Detector`) false false)
      (`SceneComponent.K2_SetRelativeTransform` _right_detector (`KismetMathLibrary.MakeTransform` (- (`SceneComponent.RelativeLocation` _right_detector) (0.0 0.0 40.0)) (struct) (0.75 1.0 0.85)) false false)
      (`SceneComponent.K2_SetRelativeTransform` _left_detector (`KismetMathLibrary.MakeTransform` (- (`SceneComponent.RelativeLocation` _left_detector) (0.0 0.0 40.0)) (struct) (0.75 1.0 0.85)) false false)
      (set `CharacterMovementComponent.MaxWalkSpeed` 300.0 (`self.CharacterMovement`)))))

(fn `UserConstructionScript`
  (`parent.UserConstructionScript`))