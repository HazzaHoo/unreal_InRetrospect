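; BP_SF_Base_AI is the base side-scrolling enemy for Super Fabio, walking horizontally every tick with a flipbook set at construction.
; Left and right detectors reverse its direction on non-player overlaps, or show the game-over widget once after a brief delay when touching the player.
; A squash detector calls the empty OnStomped event when the player overlaps it.
; The destroy-on-player-hit logic is disconnected.
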(event `OnStomped`)

(event `self.Squash Detector.OnComponentBeginOverlap`
  (params (OverlappedComponent :type "PrimitiveComponent Object Reference") (OtherActor :type "Actor Object Reference") (OtherComp :type "PrimitiveComponent Object Reference") (OtherBodyIndex :type Integer) (bFromSweep :type Boolean) (SweepResult :type "HitResult Structure (by ref)"))
  ; Squash Detector
  (if (`self.ActorHasTag` OtherActor "Player")
    (`self.OnStomped`)))

(event `self.Left Detector.OnComponentBeginOverlap`
  (params (OverlappedComponent :type "PrimitiveComponent Object Reference") (OtherActor :type "Actor Object Reference") (OtherComp :type "PrimitiveComponent Object Reference") (OtherBodyIndex :type Integer) (bFromSweep :type Boolean) (SweepResult :type "HitResult Structure (by ref)"))
  ; Dead
  (if (`self.ActorHasTag` OtherActor "Player")
    (`KismetSystemLibrary.Delay` 0.05)
    (`/Engine/EditorBlueprintResources/StandardMacros.DoOnce` false :!label _label
      (:`Completed`
        (bind _returnvalue (`|CreateWidget` "/Game/Super_Fabio/UserInterface/WB_GameOver_SuperFabio.WB_GameOver_SuperFabio_C"))
        (`UserWidget.AddToViewport` _returnvalue 0)))
    (else
      (set `self.ShouldGoLeftSide` false))))

(event `self.ReceiveHit`
  (params (MyComp :type "PrimitiveComponent Object Reference") (Other :type "Actor Object Reference") (OtherComp :type "PrimitiveComponent Object Reference") (bSelfMoved :type Boolean) (HitLocation :type "Vector Structure") (HitNormal :type "Vector Structure") (NormalImpulse :type "Vector Structure") (Hit :type "HitResult Structure (by ref)"))
  ;[0.15 0 0 0.5] Kills Enemy
)

(event `self.Right Detector.OnComponentBeginOverlap`
  (params (OverlappedComponent :type "PrimitiveComponent Object Reference") (OtherActor :type "Actor Object Reference") (OtherComp :type "PrimitiveComponent Object Reference") (OtherBodyIndex :type Integer) (bFromSweep :type Boolean) (SweepResult :type "HitResult Structure (by ref)"))
  ; Dead
  (if (`self.ActorHasTag` OtherActor "Player")
    (`KismetSystemLibrary.Delay` 0.05)
    (goto _label)
    (else
      (set `self.ShouldGoLeftSide` true))))

(event `self.ReceiveTick`
  (params (DeltaSeconds :type "Float (single-precision)"))
  ; Move Left or Right
  (if (`self.ShouldGoLeftSide`)
    (`self.AddMovementInput` (-1.0 0.0 0.0) 1.0 true)
    (else
      (`self.AddMovementInput` (1.0 0.0 0.0) 1.0 true))))

(fn `UserConstructionScript`
  (`PaperFlipbookComponent.SetFlipbook` (`self.Sprite`) (`self.SpriteChar`)))