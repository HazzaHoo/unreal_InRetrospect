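; BP_SF_LuckyBlock is a lucky block in Super Fabio that bumps and pops out coins when its trigger box is overlapped.
; Every overlap replays a timeline that moves the block vertically, while a DoOnce limits the sound and coin payout to the first hit.
; The payout is one to three coin pickups with VFX, spawned at slightly randomised positions by a self-calling event with a short delay between each.
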(event `Spawn Again`
  (bind _returnvalue (`SceneComponent.K2_GetComponentToWorld` (`self.WallColision`)))
  (bind (_returnvalue_x _returnvalue_y _returnvalue_z) (`KismetMathLibrary.BreakVector` (`SceneComponent.K2_GetComponentLocation` (`self.SpawnPoint`))))
  (`KismetSystemLibrary.Delay` 0.2)
  (bind _returnvalue_2 (`|SpawnActorFromClass` "/Game/Super_Fabio/Blueprints/BP_CoinPickup.BP_CoinPickup_C" (`KismetMathLibrary.MakeTransform` (`KismetMathLibrary.MakeVector` (+ (.x (.location _returnvalue)) (`KismetMathLibrary.RandomFloatInRange` -25.0 25.0)) (+ (.y (.location _returnvalue)) (`KismetMathLibrary.RandomFloatInRange` -5.0 5.0)) (+ _returnvalue_z (`self.ItemSpawnLocationOffset`))) (.rotation _returnvalue) (0.5 0.5 0.5)) "Undefined" "MultiplyWithRoot" null null :!label _label))
  (`NiagaraFunctionLibrary.SpawnSystemAtLocation` "/Game/Super_Fabio/VFX/SF_CoinPickup_VFX.SF_CoinPickup_VFX" (`SceneComponent.K2_GetComponentLocation` (`/Game/Super_Fabio/Blueprints/BP_CoinPickup.Coin_Sprite` _returnvalue_2)))
  (bind _result (`/Engine/EditorBlueprintResources/StandardMacros.IncrementInt` (`self.AmtSpawned`))
    (:`  `
      (if (not (>= _result (`self.AmtToSpawn`)))
        (`self.Spawn Again`)))))

(event `self.TriggerBox.OnComponentBeginOverlap`
  (params (OverlappedComponent :type "PrimitiveComponent Object Reference") (OtherActor :type "Actor Object Reference") (OtherComp :type "PrimitiveComponent Object Reference") (OtherBodyIndex :type Integer) (bFromSweep :type Boolean) (SweepResult :type "HitResult Structure (by ref)"))
  (`|ExecutionSequence`
    (:`then_0`
      (`/Engine/EditorBlueprintResources/StandardMacros.DoOnce` false
        (:`Completed`
          (`GameplayStatics.PlaySound2D` "/Game/Arcade(Both)/Audio/Coin_Pickup.Coin_Pickup" 1.0 1.0 0.0 null null)
          (set `self.AmtToSpawn` (`KismetMathLibrary.RandomIntegerInRange` 1 3))
          (`KismetSystemLibrary.Delay` 0.05)
          (goto _label))))
    (:`then_1`
      (bind (_direction _lerp) (`Timeline|T_Move` :!via `PlayFromStart`)
        (:`Update`
          (`SceneComponent.K2_SetRelativeLocation` (`self.LuckyBlock`) (`KismetMathLibrary.VLerp` (0.0 0.0 0.0) (0.0 0.0 25.0) _lerp) false false))))))

(fn `UserConstructionScript`)