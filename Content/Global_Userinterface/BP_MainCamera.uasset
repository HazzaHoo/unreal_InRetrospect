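; BP_MainCamera is a 3D menu camera actor that moves the player's view between linked menus.
; On BeginPlay it binds to the transition event of its WB_Menu3D widget and disables its own collision.
; The event's index selects an entry in LinkedMenus; the actor then turns its collision off, enables the target's, and blends the view target to it with ease-in-out.
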(event `self.ReceiveBeginPlay`
  (bind _aswb_menu_3d (cast `/Game/Global_Userinterface/WB_Menu3D` (`WidgetComponent.GetUserWidgetObject` (`self.Widget`))))
  (add `/Game/Global_Userinterface/WB_Menu3D.TransitionToLinkedMenu` _aswb_menu_3d (delegate `OnTransitionBetweenMenus`))
  (`self.SetActorEnableCollision` false))

(event `OnTransitionBetweenMenus`
  (params (MenuIndex :type Integer))
  (if (`KismetArrayLibrary.Array_IsValidIndex` (`self.LinkedMenus`) MenuIndex)
    (`self.TransitionTo` (`|GetArrayItem` (`self.LinkedMenus`) MenuIndex))))

(event `TransitionTo`
  (params (NewMenu :type "/Game/Global_Userinterface/BP_MainCamera Object Reference"))
  ; Transition to New Camera
  (`self.SetActorEnableCollision` false)
  (`self.SetActorEnableCollision` NewMenu true)
  (`PlayerController.SetViewTargetWithBlend` (`GameplayStatics.GetPlayerController` 0) NewMenu 1.0 "VTBlend_EaseInOut" 1.0 false))

(fn `UserConstructionScript`)