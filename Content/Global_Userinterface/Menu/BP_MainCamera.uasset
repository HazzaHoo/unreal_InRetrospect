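; Menu camera actor with a 3D widget menu that moves the view between linked menus and plays the menu music.
; The widget's transition event passes an index into LinkedMenus, and the camera eases the view target to that actor over a second, switching collision from itself to the target.
; Music fades in an intro, starts the main part after a timed delay, and has an event to fade out.
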(event `self.ReceiveBeginPlay`
  ; Transition To Event
  (bind _aswb_menu_3d (cast `/Game/Global_Userinterface/Menu/WB_Menu3D` (`WidgetComponent.GetUserWidgetObject` (`self.Widget`))))
  (add `/Game/Global_Userinterface/Menu/WB_Menu3D.TransitionToLinkedMenu` _aswb_menu_3d (delegate `OnTransitionBetweenMenus`))
  (`self.SetActorEnableCollision` false)
  (`self.Fade Menu Music In`))

(event `OnTransitionBetweenMenus`
  (params (MenuIndex :type Integer))
  ; Transition To Event
  (if (`KismetArrayLibrary.Array_IsValidIndex` (`self.LinkedMenus`) MenuIndex)
    (`self.TransitionTo` (`|GetArrayItem` (`self.LinkedMenus`) MenuIndex))))

(event `TransitionTo`
  (params (NewMenu :type "/Game/Global_Userinterface/Menu/BP_MainCamera Object Reference"))
  ; Transition to New Camera
  (`self.SetActorEnableCollision` false)
  (`self.SetActorEnableCollision` NewMenu true)
  (`PlayerController.SetViewTargetWithBlend` (`GameplayStatics.GetPlayerController` 0) NewMenu 1.0 "VTBlend_EaseInOut" 1.0 false))

(event `Fade Menu Music In`
  ; Fade Music In or Out
  (bind _returnvalue (`GameplayStatics.CreateSound2D` "/Game/Global_Userinterface/Intro.Intro" 1.0 1.0 0.0 null))
  (`AudioComponent.FadeIn` _returnvalue 2.0 1.0 0.0 "Linear")
  (`KismetSystemLibrary.Delay` 16.25)
  (bind _returnvalue_2 (`GameplayStatics.CreateSound2D` "/Game/Global_Userinterface/Rest.Rest" 1.0 1.0 0.0 null))
  (`AudioComponent.Play` _returnvalue_2 0.0))

(event `Fade Menu Music Out`
  ; Fade Music In or Out
  (`/Engine/EditorBlueprintResources/StandardMacros.IsValid` (stale `Fade Menu Music In` _returnvalue)
    (:`Is Valid`
      (`AudioComponent.FadeOut` (stale `Fade Menu Music In` _returnvalue) 0.5 0.0 "Linear"))
    (:`Is Not Valid`
      (`/Engine/EditorBlueprintResources/StandardMacros.IsValid` (stale `Fade Menu Music In` _returnvalue_2)
        (:`Is Valid`
          (`AudioComponent.FadeOut` (stale `Fade Menu Music In` _returnvalue_2) 0.5 0.0 "Linear"))))))

(fn `UserConstructionScript`)