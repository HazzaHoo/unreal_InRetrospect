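; BP_DebugManager is a debug helper for jumping between the game's levels with number keys.
; On BeginPlay it adds the global Enhanced Input mapping context and enables input for the first player controller.
; While DebugMode is set, keys 1 to 8 open the arcade, minigame and main menu levels by name.
; Logic to toggle DebugMode and its WB_Debug overlay exists but is unconnected, so it never runs.
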(event `self.ReceiveBeginPlay`
  (bind _returnvalue (`GameplayStatics.GetPlayerController` 0))
  (bind _returnvalue_2 (pcsubsystem `EnhancedInputLocalPlayerSubsystem` _returnvalue))
  (`/Engine/EditorBlueprintResources/StandardMacros.IsValid` _returnvalue_2
    (:`Is Valid`
      (`EnhancedInputSubsystemInterface.AddMappingContext` _returnvalue_2 "/Game/Global_IMC/IMC_Global.IMC_Global" 0 (struct))
      (`self.EnableInput` _returnvalue))))

(event `Key|BackSpace`
  (params (Key :type "Key Structure")))

(event `Key|One`
  (params (Key :type "Key Structure"))
  (:`Pressed`
    (if (`self.DebugMode`)
      (`GameplayStatics.OpenLevel` "L_BrokenArcade"))))

(event `Key|Two`
  (params (Key :type "Key Structure"))
  (:`Pressed`
    (if (`self.DebugMode`)
      (`GameplayStatics.OpenLevel` "L_Ping"))))

(event `Key|Three`
  (params (Key :type "Key Structure"))
  (:`Pressed`
    (if (`self.DebugMode`)
      (`GameplayStatics.OpenLevel` "L_SuperFabio"))))

(event `Key|Four`
  (params (Key :type "Key Structure"))
  (:`Pressed`
    (if (`self.DebugMode`)
      (`GameplayStatics.OpenLevel` "L_Crash_Capybara"))))

(event `Key|Five`
  (params (Key :type "Key Structure"))
  (:`Pressed`
    (if (`self.DebugMode`)
      (`GameplayStatics.OpenLevel` "L_Acoustic_Vigilante"))))

(event `Key|Six`
  (params (Key :type "Key Structure"))
  (:`Pressed`
    (if (`self.DebugMode`)
      (`GameplayStatics.OpenLevel` "L_Chrono_Panic"))))

(event `Key|Seven`
  (params (Key :type "Key Structure"))
  (:`Pressed`
    (if (`self.DebugMode`)
      (`GameplayStatics.OpenLevel` "L_Modern_Arcade"))))

(event `Key|Eight`
  (params (Key :type "Key Structure"))
  (:`Pressed`
    (if (`self.DebugMode`)
      (`GameplayStatics.OpenLevel` "L_MainMenu"))))

(fn `UserConstructionScript`)