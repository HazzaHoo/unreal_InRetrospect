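; BP_AV_Life is a world-placed health gauge for Acoustic Vigilante that displays the player's health through the rotation of a cylinder.
; On BeginPlay it turns its root once toward BP_AV_Player and caches a reference to that player.
; Every Tick it sets the cylinder's relative rotation by interpolating between the NoLife and MaxLife rotators, using the player's Health normalized to a 100-point scale.
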(event `self.ReceiveBeginPlay`
  (`self.RotateToPlayer`)
  (bind _returnvalue (`GameplayStatics.GetActorOfClass` "/Game/Acoustic_Vigilante/Blueprints/BP_AV_Player.BP_AV_Player_C"))
  (set `self.Player Ref` _returnvalue))

(event `self.ReceiveTick`
  (params (DeltaSeconds :type "Float (single-precision)"))
  (`SceneComponent.K2_SetRelativeRotation` (`self.Cylinder`) (`KismetMathLibrary.RLerp` (`self.NoLife`) (`self.MaxLife`) (/ (`/Game/Acoustic_Vigilante/Blueprints/BP_AV_Player.Health` (`self.Player Ref`)) 100.0)) false false))

(fn `RotateToPlayer`
  (bind _returnvalue (`GameplayStatics.GetActorOfClass` "/Game/Acoustic_Vigilante/Blueprints/BP_AV_Player.BP_AV_Player_C"))
  (`SceneComponent.K2_SetWorldRotation` (`self.DefaultSceneRoot`) (`KismetMathLibrary.FindLookAtRotation` (`SceneComponent.K2_GetComponentLocation` (`self.Cube`)) (`self.K2_GetActorLocation` _returnvalue)) false false))

(fn `UserConstructionScript`)