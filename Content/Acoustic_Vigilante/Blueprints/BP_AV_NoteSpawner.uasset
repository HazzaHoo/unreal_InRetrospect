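; Rhythm-game note spawner that drops coloured notes into four lanes from a beat-map DataTable chosen by difficulty and song.
; After an intro delay it starts the music and a looping timer that compares each row's spawn time to Tick-accumulated SongTime.
; Once the player reaches the target score, a key periodically replaces a note.
; When the map runs out, it fails the player for insufficient score or time.
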(event `StartNoteSpawner`
  (`self.GetDifficulty`)
  (bind _returnvalue (`GameplayStatics.GetActorOfClass` "/Game/Acoustic_Vigilante/Blueprints/BP_AV_Player.BP_AV_Player_C"))
  (set `self.PlayerRef` _returnvalue)
  (`KismetSystemLibrary.Delay` (`self.TimeBeforeNoteSpawn`))
  (`/Game/Acoustic_Vigilante/Blueprints/BP_AV_Player.StartMusic(AfterIntro)` _returnvalue)
  (bind _outactors (`GameplayStatics.GetAllActorsOfClass` "/Game/Acoustic_Vigilante/Blueprints/BP_AV_HitZone.BP_AV_HitZone_C"))
  (for _array_element _outactors
    (`/Game/Acoustic_Vigilante/Blueprints/BP_AV_HitZone.RemoveWidgets` _array_element))
  (`KismetSystemLibrary.K2_SetTimerDelegate` (delegate `CheckSpawns`) 0.04 true))

(event `Set Note Colour`
  (switch `int` (stale `CheckSpawns` _output_get)
    (:`1`
      (bind _note (`/Game/Acoustic_Vigilante/Blueprints/BP_AV_Note.note` (stale `CheckSpawns` _returnvalue_4)))
      (`PrimitiveComponent.SetMaterial` _note 0 "/Game/Acoustic_Vigilante/Assets/Material/Notes/M_AV_Note_Green.M_AV_Note_Green"))
    (:`2`
      (`PrimitiveComponent.SetMaterial` _note 0 "/Game/Acoustic_Vigilante/Assets/Material/Notes/M_AV_Note_Red.M_AV_Note_Red"))
    (:`3`
      (`PrimitiveComponent.SetMaterial` _note 0 "/Game/Acoustic_Vigilante/Assets/Material/Notes/M_AV_Note_Yellow.M_AV_Note_Yellow"))
    (:`4`
      (`PrimitiveComponent.SetMaterial` _note 0 "/Game/Acoustic_Vigilante/Assets/Material/Notes/M_AV_Note_Blue.M_AV_Note_Blue"))))

(event `CheckSpawns`
  (bind _playerref (`self.PlayerRef`))
  (bind _playerref_2 (`self.PlayerRef`))
  (bind _playerref_3 (`self.PlayerRef`))
  (bind _currentindex (`self.CurrentIndex`))
  (`|ExecutionSequence`
    (:`then_0`
      (bind _outrownames (`DataTableFunctionLibrary.GetDataTableRowNames` (`self.BeatMapTable`)))
      (bind _returnvalue (`KismetArrayLibrary.Array_Length` _outrownames))
      (if (< _currentindex _returnvalue)
        (bind _returnvalue_2 (`|GetDataTableRow` (`self.BeatMapTable`) (`KismetStringLibrary.Conv_StringToName` (`KismetStringLibrary.Concat_StrStr` "note" (`KismetStringLibrary.Conv_IntToString` (`self.CurrentIndex`)))))
          (:`then`
            (bind (_spawntime _laneindex) (break `/Game/Acoustic_Vigilante/Assets/S_AV_NoteData` _returnvalue_2))
            (if (>= (`self.SongTime`) _spawntime)
              (if (>= (`/Game/Acoustic_Vigilante/Blueprints/BP_AV_Player.Score` _playerref_3) (`/Game/Acoustic_Vigilante/Blueprints/BP_AV_Player.TargetScore` _playerref_3))
                (if (>= (`self.NotesAfterWin`) 5)
                  (set `self.NotesAfterWin` 0)
                  (bind _returnvalue_3 (`|SpawnActorFromClass` "/Game/Acoustic_Vigilante/Blueprints/BP_AV_Key.BP_AV_Key_C" (`self.GetTransform` (`|GetArrayItem` (`self.SpawnPoints`) (- _laneindex 1))) "Undefined" "MultiplyWithRoot" null null))
                  (set `/Game/Acoustic_Vigilante/Blueprints/BP_AV_Key.LaneIndex` _laneindex _returnvalue_3)
                  (set `self.CurrentIndex` (+ (`self.CurrentIndex`) 1))
                  (else
                    (set `self.NotesAfterWin` (+ (`self.NotesAfterWin`) 1))
                    (bind _returnvalue_4 (`|SpawnActorFromClass` "/Game/Acoustic_Vigilante/Blueprints/BP_AV_Note.BP_AV_Note_C" (`self.GetTransform` (`|GetArrayItem` (`self.SpawnPoints`) (- _laneindex 1))) "Undefined" "MultiplyWithRoot" null null :!label _label))
                    (bind _output_get (set `/Game/Acoustic_Vigilante/Blueprints/BP_AV_Note.LaneIndex` _laneindex _returnvalue_4))
                    (set `self.CurrentIndex` (+ (`self.CurrentIndex`) 1))
                    (`self.Set Note Colour`)))
                (else
                  (goto _label))))))
        (elif (== _currentindex _returnvalue)
          (`/Engine/EditorBlueprintResources/StandardMacros.DoOnce` false
            (:`Completed`
              (if (< (`/Game/Acoustic_Vigilante/Blueprints/BP_AV_Player.Score` _playerref_2) (`/Game/Acoustic_Vigilante/Blueprints/BP_AV_Player.TargetScore` _playerref_2))
                (`KismetSystemLibrary.Delay` 5.0)
                (`/Game/Acoustic_Vigilante/Blueprints/BP_AV_Player.OnFail` _playerref false false true)
                (else
                  (`KismetSystemLibrary.Delay` 5.0)
                  (`/Game/Acoustic_Vigilante/Blueprints/BP_AV_Player.OnFail` _playerref false true false))))))))
    (:`then_1`
      (goto _label_2 :!via `Open`))))

(event `self.ReceiveTick`
  (params (DeltaSeconds :type "Float (single-precision)"))
  (`/Engine/EditorBlueprintResources/StandardMacros.Gate` true :!label _label_2
    (:`Exit`
      (set `self.SongTime` (+ (`self.SongTime`) DeltaSeconds)))))

(fn `GetDifficulty`
  (bind _asglobal_instance (cast `/Game/Global_IMC/Global_Instance` (`GameplayStatics.GetGameInstance`)))
  (switch `/Game/Ping/Blueprints/E_Difficulty` (`/Game/Global_IMC/Global_Instance.SelectedDifficulty` _asglobal_instance)
    (:`NewEnumerator0`
      (if (`self.YMCA?`)
        (set `self.BeatMapTable` "/Game/Acoustic_Vigilante/Blueprints/Beats/YMCA_EASY.YMCA_EASY")
        (else
          (set `self.BeatMapTable` "/Game/Acoustic_Vigilante/Blueprints/Beats/RidinSolo_easy.RidinSolo_easy"))))
    (:`NewEnumerator1`
      (if (`self.YMCA?`)
        (set `self.BeatMapTable` "/Game/Acoustic_Vigilante/Blueprints/Beats/YMCA_MEDIUM.YMCA_MEDIUM")
        (else
          (set `self.BeatMapTable` "/Game/Acoustic_Vigilante/Blueprints/Beats/RidinSolo_medium.RidinSolo_medium"))))
    (:`NewEnumerator2`
      (if (`self.YMCA?`)
        (set `self.BeatMapTable` "/Game/Acoustic_Vigilante/Blueprints/Beats/YMCA_HARD.YMCA_HARD")
        (else
          (set `self.BeatMapTable` "/Game/Acoustic_Vigilante/Blueprints/Beats/RidinSolo_hard.RidinSolo_hard"))))))

(fn `UserConstructionScript`)