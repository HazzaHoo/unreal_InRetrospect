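; BP_AV_BackgroundCamera is a background camera actor for Acoustic Vigilante that travels along a referenced spline once play begins.
; BeginPlay calls MoveCamera, which scales the timeline's play rate by the inverse of TimeToComplete and plays it.
; Each timeline update maps its alpha to a distance along the spline and sets the actor's world location there, leaving rotation untouched.
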(event `self.ReceiveBeginPlay`
  (`self.MoveCamera`))

(event `MoveCamera`
  (bind _spline (`/Game/Acoustic_Vigilante/Blueprints/BP_CameraSplinePath.Spline` (`self.Spline to Follow`)))
  (`TimelineComponent.SetPlayRate` (`self.T_Move`) (/ 1.0 (`self.Time To Complete`)))
  (bind (_direction _movecamera) (`Timeline|T_Move`)
    (:`Update`
      (`self.K2_SetActorLocation` (`SplineComponent.GetLocationAtDistanceAlongSpline` _spline (`KismetMathLibrary.Lerp` 0.0 (`SplineComponent.GetSplineLength` _spline) _movecamera) "World")))))

(fn `UserConstructionScript`)