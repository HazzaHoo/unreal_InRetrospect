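; Lane hit zone for a rhythm game, with a coloured bumper, lane label widget and hit-grade popup.
; A box overlap queues incoming notes and flags keys in the zone, reporting a miss to the player when an unhit note leaves.
; CheckHit plays a bumper bump, grades the oldest queued note by X distance from the hit line, then sends the score to the player, shows the grade and destroys the note.
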(event `RemoveWidgets`
  (`/Engine/EditorBlueprintResources/StandardMacros.IsValid` (stale `self.ReceiveBeginPlay` _aswb_av_controls)
    (:`Is Valid`
      (`/Game/Acoustic_Vigilante/UserInterface/WB_AV_Controls.FadeOutControls` (stale `self.ReceiveBeginPlay` _aswb_av_controls)))))

(event `self.ReceiveBeginPlay`
  (bind _returnvalue_x (`KismetMathLibrary.BreakVector` (`SceneComponent.K2_GetComponentLocation` (`self.Box`))))
  (set `self.HitLine` _returnvalue_x)
  (`self.RotateWidgetToCamera`)
  (set `self.CenterBumpNormal` (`SceneComponent.RelativeLocation` (`self.CenterBump`)))
  (bind _aswb_av_controls (cast `/Game/Acoustic_Vigilante/UserInterface/WB_AV_Controls` (`WidgetComponent.GetWidget` (`self.Widget`))))
  (`/Game/Acoustic_Vigilante/UserInterface/WB_AV_Controls.SetText` _aswb_av_controls (`self.LaneIndex`))
  (`self.SetColourLane`))

(event `self.Box.OnComponentBeginOverlap`
  (params (OverlappedComponent :type "PrimitiveComponent Object Reference") (OtherActor :type "Actor Object Reference") (OtherComp :type "PrimitiveComponent Object Reference") (OtherBodyIndex :type Integer) (bFromSweep :type Boolean) (SweepResult :type "HitResult Structure (by ref)"))
  (bind _asbp_av_note (cast `/Game/Acoustic_Vigilante/Blueprints/BP_AV_Note` OtherActor)
    (:`then`
      (`KismetArrayLibrary.Array_Add` (`self.NoteInZone`) _asbp_av_note))
    (:`CastFailed`
      (bind _asbp_av_key (cast `/Game/Acoustic_Vigilante/Blueprints/BP_AV_Key` OtherActor))
      (set `self.ActiveKey` _asbp_av_key)
      (set `self.IsKeyInZone` true))))

(event `self.Box.OnComponentEndOverlap`
  (params (OverlappedComponent :type "PrimitiveComponent Object Reference") (OtherActor :type "Actor Object Reference") (OtherComp :type "PrimitiveComponent Object Reference") (OtherBodyIndex :type Integer))
  (bind _asbp_av_note (cast `/Game/Acoustic_Vigilante/Blueprints/BP_AV_Note` OtherActor)
    (:`then`
      (if (`/Game/Acoustic_Vigilante/Blueprints/BP_AV_Note.IsHit` _asbp_av_note)
        (`KismetArrayLibrary.Array_RemoveItem` (`self.NoteInZone`) _asbp_av_note)
        (else
          (bind _asbp_av_player (cast `/Game/Acoustic_Vigilante/Blueprints/BP_AV_Player` (`GameplayStatics.GetPlayerPawn` 0)))
          (`/Game/Acoustic_Vigilante/Blueprints/BP_AV_Player.OnMiss` _asbp_av_player)
          (`KismetArrayLibrary.Array_RemoveItem` (`self.NoteInZone`) _asbp_av_note))))
    (:`CastFailed`
      (bind _asbp_av_key (cast `/Game/Acoustic_Vigilante/Blueprints/BP_AV_Key` OtherActor))
      (set `self.ActiveKey` _asbp_av_key)
      (set `self.IsKeyInZone` false))))

(event `CenterBumpAnimation`
  (bind (_direction _lerp) (`Timeline|Anim` :!via `PlayFromStart`)
    (:`Update`
      (`SceneComponent.K2_SetRelativeLocation` (`self.CenterBump`) (`KismetMathLibrary.VLerp` (`self.CenterBumpNormal`) (`self.CenterBumpHeight`) _lerp) false false))))

(event `CheckHit`
  (bind _hitgradewidget_ref (`self.HitGradeWidget Ref`))
  (bind _noteinzone (`self.NoteInZone`))
  (bind _hitgradewidget_ref_2 (`self.HitGradeWidget Ref`))
  (bind _returnvalue_x (`KismetMathLibrary.BreakVector` (`self.K2_GetActorLocation` (`|GetArrayItem` (`self.NoteInZone`)))))
  (bind _returnvalue (`KismetMathLibrary.Abs` (- _returnvalue_x (`self.HitLine`))))
  (`self.CenterBumpAnimation`)
  (if (> (`KismetArrayLibrary.Array_Length` (`self.NoteInZone`)) 0)
    (set `/Game/Acoustic_Vigilante/Blueprints/BP_AV_Note.IsHit` true (`|GetArrayItem` (`self.NoteInZone`)))
    (`ActorComponent.Activate` (`self.N_AV_HitNote`) true)
    (if (<= _returnvalue 20.0)
      (bind _asbp_av_player (cast `/Game/Acoustic_Vigilante/Blueprints/BP_AV_Player` (`GameplayStatics.GetPlayerPawn` 0)))
      (`/Game/Acoustic_Vigilante/Blueprints/BP_AV_Player.OnHit` _asbp_av_player 20)
      (`/Game/Acoustic_Vigilante/UserInterface/WB_AV_HitGrade.SetTextAnim` _hitgradewidget_ref "PERFECT!!!")
      (elif (<= _returnvalue 60.0)
        (bind _asbp_av_player_2 (cast `/Game/Acoustic_Vigilante/Blueprints/BP_AV_Player` (`GameplayStatics.GetPlayerPawn` 0)))
        (`/Game/Acoustic_Vigilante/Blueprints/BP_AV_Player.OnHit` _asbp_av_player_2 10)
        (`/Game/Acoustic_Vigilante/UserInterface/WB_AV_HitGrade.SetTextAnim` _hitgradewidget_ref "GREAT!!")
        (elif (<= _returnvalue 120.0)
          (bind _asbp_av_player_3 (cast `/Game/Acoustic_Vigilante/Blueprints/BP_AV_Player` (`GameplayStatics.GetPlayerPawn` 0)))
          (`/Game/Acoustic_Vigilante/Blueprints/BP_AV_Player.OnHit` _asbp_av_player_3 5)
          (`/Game/Acoustic_Vigilante/UserInterface/WB_AV_HitGrade.SetTextAnim` _hitgradewidget_ref_2 "GOOD!")
          (else
            (bind _asbp_av_player_4 (cast `/Game/Acoustic_Vigilante/Blueprints/BP_AV_Player` (`GameplayStatics.GetPlayerPawn` 0)))
            (`/Game/Acoustic_Vigilante/Blueprints/BP_AV_Player.OnBadHit` _asbp_av_player_4 1)
            (`/Game/Acoustic_Vigilante/UserInterface/WB_AV_HitGrade.SetTextAnim` _hitgradewidget_ref_2 "BAD")))))
    (`self.K2_DestroyActor` (`|GetArrayItem` _noteinzone))
    (`KismetArrayLibrary.Array_Remove` _noteinzone)))

(fn `RotateWidgetToCamera`
  (bind _returnvalue (`GameplayStatics.GetActorOfClass` "/Game/Acoustic_Vigilante/Blueprints/BP_AV_Player.BP_AV_Player_C"))
  (`SceneComponent.K2_SetWorldRotation` (`self.HitGradeUI`) (`KismetMathLibrary.FindLookAtRotation` (`SceneComponent.K2_GetComponentLocation` (`self.HitGradeUI`)) (`self.K2_GetActorLocation` _returnvalue)) false false)
  (bind _aswb_av_hit_grade (cast `/Game/Acoustic_Vigilante/UserInterface/WB_AV_HitGrade` (`WidgetComponent.GetWidget` (`self.HitGradeUI`))))
  (set `self.HitGradeWidget Ref` _aswb_av_hit_grade))

(fn `SetColourLane`
  (bind _center (`self.Center`))
  (switch `int` (`self.LaneIndex`)
    (:`1`
      (`PrimitiveComponent.SetMaterial` _center 0 "/Game/Acoustic_Vigilante/Assets/Material/Bumpers/M_Bumper_Green.M_Bumper_Green"))
    (:`2`
      (`PrimitiveComponent.SetMaterial` _center 0 "/Game/Acoustic_Vigilante/Assets/Material/Bumpers/M_Bumper_Red.M_Bumper_Red"))
    (:`3`
      (`PrimitiveComponent.SetMaterial` _center 0 "/Game/Acoustic_Vigilante/Assets/Material/Bumpers/M_Bumper_Yellow.M_Bumper_Yellow"))
    (:`4`
      (`PrimitiveComponent.SetMaterial` _center 0 "/Game/Acoustic_Vigilante/Assets/Material/Bumpers/M_Bumper_Blue.M_Bumper_Blue"))))

(fn `UserConstructionScript`)