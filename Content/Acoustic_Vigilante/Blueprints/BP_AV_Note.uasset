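; BP_AV_Note is a note actor for Acoustic Vigilante that travels along negative world X once spawned.
; On BeginPlay it records the current SongTime from BP_AV_NoteSpawner as its SpawnTime, then sets NoteSpeed from the Global_Instance's selected difficulty.
; Easy, Medium and Hard currently all give the same speed.
; Tick offsets the note by that speed scaled by delta time.
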(event `self.ReceiveBeginPlay`
  (bind _returnvalue (`GameplayStatics.GetActorOfClass` "/Game/Acoustic_Vigilante/Blueprints/BP_AV_NoteSpawner.BP_AV_NoteSpawner_C"))
  (set `self.SpawnTime` (`/Game/Acoustic_Vigilante/Blueprints/BP_AV_NoteSpawner.SongTime` _returnvalue))
  (`self.GetDifficutlySpeed`))

(event `self.ReceiveTick`
  (params (DeltaSeconds :type "Float (single-precision)"))
  (`self.K2_AddActorWorldOffset` (`KismetMathLibrary.MakeVector` (* DeltaSeconds (* (`self.NoteSpeed`) -1.0)))))

(fn `GetDifficutlySpeed`
  (bind _asglobal_instance (cast `/Game/Global_IMC/Global_Instance` (`GameplayStatics.GetGameInstance`)))
  (switch `/Game/Ping/Blueprints/E_Difficulty` (`/Game/Global_IMC/Global_Instance.SelectedDifficulty` _asglobal_instance)
    (:`NewEnumerator0`
      (set `self.NoteSpeed` 1750.0))
    (:`NewEnumerator1`
      (set `self.NoteSpeed` 1750.0))
    (:`NewEnumerator2`
      (set `self.NoteSpeed` 1750.0))))

(fn `UserConstructionScript`)