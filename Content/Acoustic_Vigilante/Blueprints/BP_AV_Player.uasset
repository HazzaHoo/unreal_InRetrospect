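; Player for the Acoustic Vigilante four-lane rhythm minigame, handling input, score, combo, health and song playback.
; Each lane input finds its BP_AV_HitZone and either checks a note hit or collects a key, which wins and transitions to L_Chrono_Panic.
; Hit and miss functions update the HUD, with misses triggering a record scratch.
; OnFail shows game over, but its zero-health call is disconnected.
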(event `OnFail`
  (params (`OutofLife?` :type Boolean) (`OutOfTime?` :type Boolean) (`NotEnoughScore?` :type Boolean))
  (bind _returnvalue (`GameplayStatics.GetPlayerController` 0))
  (if (not (`self.HasWon`))
    (`/Engine/EditorBlueprintResources/StandardMacros.DoOnce` false
      (:`Completed`
        (bind _returnvalue_2 (`|CreateWidget` "/Game/Acoustic_Vigilante/UserInterface/WBP_AV_GameOver.WBP_AV_GameOver_C"))
        (`UserWidget.AddToViewport` _returnvalue_2 0)
        (`/Game/Acoustic_Vigilante/UserInterface/WBP_AV_GameOver.Set Text` _returnvalue_2 `OutofLife?` `OutOfTime?` `NotEnoughScore?`)
        (set `PlayerController.bShowMouseCursor` true _returnvalue)
        (`WidgetBlueprintLibrary.SetInputMode_GameAndUIEx` _returnvalue _returnvalue_2 "DoNotLock" false))))
  (`self.FadeMusicOut` 1.0))

(event `RecordScratch`
  ; Record Scratch
  (`GameplayStatics.PlaySound2D` "/Game/Acoustic_Vigilante/Audio/RecordScratch.RecordScratch" 0.4 (`KismetMathLibrary.RandomFloatInRange` 0.75 1.25) 0.0 null null)
  (`AudioComponent.SetVolumeMultiplier` (`self.Song Ref`) 0.5)
  (`KismetSystemLibrary.Delay` 0.2)
  (`AudioComponent.SetVolumeMultiplier` (`self.Song Ref`) (`self.VolumeMulti`)))

(event `EnhancedInput|/Game/Acoustic_Vigilante/IMC/IA_AV_Pause`
  (params (ActionValue :type Boolean) (ElapsedSeconds :type "Float (double-precision)") (TriggeredSeconds :type "Float (double-precision)") (InputAction :type "InputAction Object Reference" :default "/Game/Acoustic_Vigilante/IMC/IA_AV_Pause.IA_AV_Pause"))
  (bind _pause_widget_ref (`self.Pause Widget Ref`))
  (:`Started`
    (if (not (`self.Failed?`))
      (switch `ESlateVisibility` (`Widget.Visibility` _pause_widget_ref)
        (:`Visible`
          (`/Game/Acoustic_Vigilante/UserInterface/WB_PauseScreen_AV.Close Pause Menu` _pause_widget_ref))
        (:`Hidden`
          (`/Game/Acoustic_Vigilante/UserInterface/WB_PauseScreen_AV.Open Pause Menu` _pause_widget_ref))))))

(event `FadeMusicOut`
  (params (FadeOutTime :type "Float (double-precision)"))
  (`/Engine/EditorBlueprintResources/StandardMacros.IsValid` (stale `StartMusic(AfterIntro)` _output_get)
    (:`Is Valid`
      (`AudioComponent.FadeOut` (stale `StartMusic(AfterIntro)` _output_get) FadeOutTime 0.0 "Linear"))))

(event `StartMusic(AfterIntro)`
  (if (`self.YMCA?`)
    (bind _returnvalue (`GameplayStatics.CreateSound2D` "/Game/Acoustic_Vigilante/Audio/YMCA_Trim.YMCA_Trim" 1.0 1.0 0.0 null))
    (bind _output_get (set `self.Song Ref` _returnvalue))
    (`/Engine/EditorBlueprintResources/StandardMacros.IsValid` _output_get
      (:`Is Valid`
        (`AudioComponent.FadeIn` _output_get 1.0 1.0 0.0 "Linear")
        (set `self.VolumeMulti` (`AudioComponent.VolumeMultiplier` (`self.Song Ref`)))))
    (else
      (bind _returnvalue_2 (`GameplayStatics.CreateSound2D` "/Game/Acoustic_Vigilante/Audio/Jason_Derulo__Ridin_Solo_Official_HD_Music_Videomp3.Jason_Derulo__Ridin_Solo_Official_HD_Music_Videomp3" 1.0 1.0 0.0 null))
      (bind _output_get_2 (set `self.Song Ref` _returnvalue_2))
      (`/Engine/EditorBlueprintResources/StandardMacros.IsValid` _output_get_2
        (:`Is Valid`
          (`AudioComponent.FadeIn` _output_get_2 1.0 1.0 0.0 "Linear")
          (set `self.VolumeMulti` (`AudioComponent.VolumeMultiplier` (`self.Song Ref`))))))))

(event `PauseMusic?`
  (params (`Pause?` :type Boolean))
  (`/Engine/EditorBlueprintResources/StandardMacros.IsValid` (stale `StartMusic(AfterIntro)` _output_get)
    (:`Is Valid`
      (`AudioComponent.SetPaused` (stale `StartMusic(AfterIntro)` _output_get) `Pause?`))))

(event `self.ReceiveBeginPlay`
  (bind _returnvalue (`GameplayStatics.GetPlayerController` 0))
  (`WidgetBlueprintLibrary.SetInputMode_UIOnlyEx` _returnvalue null)
  (set `PlayerController.bShowMouseCursor` true _returnvalue)
  (bind _returnvalue_2 (`|CreateWidget` "/Game/Acoustic_Vigilante/UserInterface/WBP_AV_ChooseSong.WBP_AV_ChooseSong_C"))
  (`UserWidget.AddToViewport` _returnvalue_2 0)
  ; PLayer Controler
  (`self.Set Target Score`)
  (set `self.AcousticVigilante_Game` true)
  (bind _asplayer_controller (cast `PlayerController` (`self.GetController`)))
  (bind _returnvalue_3 (pcsubsystem `EnhancedInputLocalPlayerSubsystem` _asplayer_controller))
  (`/Engine/EditorBlueprintResources/StandardMacros.IsValid` _returnvalue_3
    (:`Is Valid`
      (`EnhancedInputSubsystemInterface.AddMappingContext` _returnvalue_3 "/Game/Acoustic_Vigilante/IMC/IMC_AcousticVigilante.IMC_AcousticVigilante" 0 (struct))
      (bind _returnvalue_4 (`GameplayStatics.GetActorOfClass` "/Game/Acoustic_Vigilante/Blueprints/BP_AV_ScoreCount.BP_AV_ScoreCount_C"))
      (set `self.HUD` (`/Game/Acoustic_Vigilante/Blueprints/BP_AV_ScoreCount.ScoreWidget Ref` _returnvalue_4))
      (bind _returnvalue_5 (`|CreateWidget` "/Game/Acoustic_Vigilante/UserInterface/WB_PauseScreen_AV.WB_PauseScreen_AV_C"))
      (bind _output_get (set `self.Pause Widget Ref` _returnvalue_5))
      (`UserWidget.AddToViewport` _output_get 0)
      (`Widget.SetVisibility` _output_get "Hidden")
      (bind _returnvalue_6 (`GameplayStatics.GetActorOfClass` "/Game/Acoustic_Vigilante/Blueprints/BP_AV_NoteSpawner.BP_AV_NoteSpawner_C"))
      (set `self.NoteSpawnerRef` _returnvalue_6)
      (bind _returnvalue_7 (`GameplayStatics.GetActorOfClass` "/Game/Acoustic_Vigilante/Blueprints/BP_AV_HitZone.BP_AV_HitZone_C"))
      (set `self.HitZoneRef` _returnvalue_7))))

(event `EnhancedInput|/Game/Acoustic_Vigilante/IMC/IA_AV_Hit_Left`
  (params (ActionValue :type Boolean) (ElapsedSeconds :type "Float (double-precision)") (TriggeredSeconds :type "Float (double-precision)") (InputAction :type "InputAction Object Reference" :default "/Game/Acoustic_Vigilante/IMC/IA_AV_Hit_Left.IA_AV_Hit_Left"))
  ; PLayer Controler
  (:`Started`
    (`/Engine/EditorBlueprintResources/StandardMacros.DoOnce` false :!label _label
      (:`Completed`
        (bind _outactors (`GameplayStatics.GetAllActorsOfClass` "/Game/Acoustic_Vigilante/Blueprints/BP_AV_HitZone.BP_AV_HitZone_C"))
        (for _array_element _outactors
          (bind _asbp_av_hit_zone (cast `/Game/Acoustic_Vigilante/Blueprints/BP_AV_HitZone` _array_element))
          (if (== (`/Game/Acoustic_Vigilante/Blueprints/BP_AV_HitZone.LaneIndex` _asbp_av_hit_zone) 1)
            (if (`/Game/Acoustic_Vigilante/Blueprints/BP_AV_HitZone.IsKeyInZone` _asbp_av_hit_zone)
              (`self.OnKeyHit` _asbp_av_hit_zone)
              (else
                (`/Game/Acoustic_Vigilante/Blueprints/BP_AV_HitZone.CheckHit` _asbp_av_hit_zone))))))))
  (:`Completed`
    (goto _label :!via `Reset`)))

(event `Win`
  ;[0.142 0.4646 0.119 0.5] Win & Lose
)

(event `EnhancedInput|/Game/Acoustic_Vigilante/IMC/IA_AV_Hit_MidLeft`
  (params (ActionValue :type Boolean) (ElapsedSeconds :type "Float (double-precision)") (TriggeredSeconds :type "Float (double-precision)") (InputAction :type "InputAction Object Reference" :default "/Game/Acoustic_Vigilante/IMC/IA_AV_Hit_MidLeft.IA_AV_Hit_MidLeft"))
  ; PLayer Controler
  (:`Started`
    (`/Engine/EditorBlueprintResources/StandardMacros.DoOnce` false :!label _label_2
      (:`Completed`
        (bind _outactors (`GameplayStatics.GetAllActorsOfClass` "/Game/Acoustic_Vigilante/Blueprints/BP_AV_HitZone.BP_AV_HitZone_C"))
        (for _array_element _outactors
          (bind _asbp_av_hit_zone (cast `/Game/Acoustic_Vigilante/Blueprints/BP_AV_HitZone` _array_element))
          (if (== (`/Game/Acoustic_Vigilante/Blueprints/BP_AV_HitZone.LaneIndex` _asbp_av_hit_zone) 2)
            (if (`/Game/Acoustic_Vigilante/Blueprints/BP_AV_HitZone.IsKeyInZone` _asbp_av_hit_zone)
              (`self.OnKeyHit` _asbp_av_hit_zone)
              (else
                (`/Game/Acoustic_Vigilante/Blueprints/BP_AV_HitZone.CheckHit` _asbp_av_hit_zone))))))))
  (:`Completed`
    (goto _label_2 :!via `Reset`)))

(event `Loose`
  ;[0.142 0.4646 0.119 0.5] Win & Lose
)

(event `EnhancedInput|/Game/Acoustic_Vigilante/IMC/IA_AV_Hit_MidRight`
  (params (ActionValue :type Boolean) (ElapsedSeconds :type "Float (double-precision)") (TriggeredSeconds :type "Float (double-precision)") (InputAction :type "InputAction Object Reference" :default "/Game/Acoustic_Vigilante/IMC/IA_AV_Hit_MidRight.IA_AV_Hit_MidRight"))
  ; PLayer Controler
  (:`Started`
    (`/Engine/EditorBlueprintResources/StandardMacros.DoOnce` false :!label _label_3
      (:`Completed`
        (bind _outactors (`GameplayStatics.GetAllActorsOfClass` "/Game/Acoustic_Vigilante/Blueprints/BP_AV_HitZone.BP_AV_HitZone_C"))
        (for _array_element _outactors
          (bind _asbp_av_hit_zone (cast `/Game/Acoustic_Vigilante/Blueprints/BP_AV_HitZone` _array_element))
          (if (== (`/Game/Acoustic_Vigilante/Blueprints/BP_AV_HitZone.LaneIndex` _asbp_av_hit_zone) 3)
            (if (`/Game/Acoustic_Vigilante/Blueprints/BP_AV_HitZone.IsKeyInZone` _asbp_av_hit_zone)
              (`self.OnKeyHit` _asbp_av_hit_zone)
              (else
                (`/Game/Acoustic_Vigilante/Blueprints/BP_AV_HitZone.CheckHit` _asbp_av_hit_zone))))))))
  (:`Completed`
    (goto _label_3 :!via `Reset`)))

(event `EnhancedInput|/Game/Acoustic_Vigilante/IMC/IA_AV_Hit_Right`
  (params (ActionValue :type Boolean) (ElapsedSeconds :type "Float (double-precision)") (TriggeredSeconds :type "Float (double-precision)") (InputAction :type "InputAction Object Reference" :default "/Game/Acoustic_Vigilante/IMC/IA_AV_Hit_Right.IA_AV_Hit_Right"))
  ; PLayer Controler
  (:`Started`
    (`/Engine/EditorBlueprintResources/StandardMacros.DoOnce` false :!label _label_4
      (:`Completed`
        (bind _outactors (`GameplayStatics.GetAllActorsOfClass` "/Game/Acoustic_Vigilante/Blueprints/BP_AV_HitZone.BP_AV_HitZone_C"))
        (for _array_element _outactors
          (bind _asbp_av_hit_zone (cast `/Game/Acoustic_Vigilante/Blueprints/BP_AV_HitZone` _array_element))
          (if (== (`/Game/Acoustic_Vigilante/Blueprints/BP_AV_HitZone.LaneIndex` _asbp_av_hit_zone) 4)
            (if (`/Game/Acoustic_Vigilante/Blueprints/BP_AV_HitZone.IsKeyInZone` _asbp_av_hit_zone)
              (`self.OnKeyHit` _asbp_av_hit_zone)
              (else
                (`/Game/Acoustic_Vigilante/Blueprints/BP_AV_HitZone.CheckHit` _asbp_av_hit_zone))))))))
  (:`Completed`
    (goto _label_4 :!via `Reset`)))

(event `EnhancedInput|/Game/Global_IMC/IA_Pause`
  (params (ActionValue :type Boolean) (ElapsedSeconds :type "Float (double-precision)") (TriggeredSeconds :type "Float (double-precision)") (InputAction :type "InputAction Object Reference" :default "/Game/Global_IMC/IA_Pause.IA_Pause"))
  ;[0.15 0 0 0.5] Call Pause Menu
)

(fn `CameraShake`
  (`GameplayStatics.PlayWorldCameraShake` "/Game/Acoustic_Vigilante/UserInterface/BP_AV_FailedNoteShake.BP_AV_FailedNoteShake_C" (`self.K2_GetActorLocation`) 0.0 1000.0))

(fn `OnBadHit`
  (params (PointsToAdd :type Integer))
  (bind _output_get (set `self.Score` (+ (`self.Score`) PointsToAdd)))
  (bind _output_get_2 (set `self.Combo` 0))
  (`/Game/Acoustic_Vigilante/UserInterface/WBP_AV_HUD.UpdateHUD` (`self.HUD`) _output_get _output_get_2 (`self.Health`)))

(fn `OnHit`
  (params (PointsToAdd :type Integer))
  (bind _output_get (set `self.Combo` (`KismetMathLibrary.Min` (+ (`self.Combo`) 1) 5)))
  (bind _output_get_2 (set `self.Score` (+ (`self.Score`) (* PointsToAdd _output_get))))
  (bind _output_get_3 (set `self.Health` (`KismetMathLibrary.FClamp` (+ (`self.Health`) (`self.NoteHealthPerHit`)) 0.0 100.0)))
  (`/Game/Acoustic_Vigilante/UserInterface/WBP_AV_HUD.UpdateHUD` (`self.HUD`) _output_get_2 _output_get _output_get_3))

(fn `OnKeyHit`
  (params (HitZoneRef :type "/Game/Acoustic_Vigilante/Blueprints/BP_AV_HitZone Object Reference"))
  (`self.K2_DestroyActor` (`/Game/Acoustic_Vigilante/Blueprints/BP_AV_HitZone.ActiveKey` HitZoneRef))
  (`GameplayStatics.PlaySound2D` "/Game/Crash_Capybara/Audio/CC_KeyPickup.CC_KeyPickup" 1.0 1.0 0.0 null null)
  (set `self.HasWon` true)
  (if (> (`self.TargetScore`) (`self.Endgame Secret Value`))
    (bind _asglobal_instance (cast `/Game/Global_IMC/Global_Instance` (`GameplayStatics.GetGameInstance`)))
    (set `/Game/Global_IMC/Global_Instance.AcousticHighScore` true _asglobal_instance))
  (bind _returnvalue (`|CreateWidget` "/Game/Global_Userinterface/WB_Transition.WB_Transition_C"))
  (`self.FadeMusicOut` 1.0)
  (`/Game/Global_Userinterface/WB_Transition.WhatEra?` _returnvalue "2" "0" "1" "L_Chrono_Panic")
  (`UserWidget.AddToViewport` _returnvalue 0))

(fn `OnMiss`
  (if (not (`self.HasWon`))
    (bind _output_get (set `self.Combo` 0))
    (bind _output_get_2 (set `self.Health` (`KismetMathLibrary.FMax` (- (`self.Health`) 10.0))))
    (`/Game/Acoustic_Vigilante/UserInterface/WBP_AV_HUD.UpdateHUD` (`self.HUD`) (`self.Score`) _output_get _output_get_2)
    (`self.RecordScratch`)
    (if (<= (`self.Health`) 0.0)
      _)))

(fn `Set Target Score`
  (bind _asglobal_instance (cast `/Game/Global_IMC/Global_Instance` (`GameplayStatics.GetGameInstance`)))
  (switch `/Game/Ping/Blueprints/E_Difficulty` (`/Game/Global_IMC/Global_Instance.SelectedDifficulty` _asglobal_instance)
    (:`NewEnumerator0`
      (if (`self.YMCA?`)
        (set `self.TargetScore` 17000.0)
        (set `self.Endgame Secret Value` 19000.0)
        (else
          (set `self.TargetScore` 20000.0)
          (set `self.Endgame Secret Value` 22000.0))))
    (:`NewEnumerator1`
      (if (`self.YMCA?`)
        (set `self.TargetScore` 28000.0)
        (set `self.Endgame Secret Value` 30000.0)
        (else
          (set `self.TargetScore` 25000.0)
          (set `self.Endgame Secret Value` 27000.0))))
    (:`NewEnumerator2`
      (if (`self.YMCA?`)
        (set `self.TargetScore` 38000.0)
        (set `self.Endgame Secret Value` 40000.0)
        (else
          (set `self.TargetScore` 40000.0)
          (set `self.Endgame Secret Value` 43000.0))))))

(fn `UserConstructionScript`)