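; BP_AV_ScoreCount is an Acoustic Vigilante actor that presents the HUD widget in the world through its ScoreCount widget component.
; On BeginPlay it rotates its Cube component once to face the BP_AV_Player actor, with no later tracking.
; It then caches the component's WBP_AV_HUD widget in ScoreWidgetRef; no score logic lives in this Blueprint.
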(event `self.ReceiveBeginPlay`
  (`self.RotateToPlayer`)
  (bind _aswbp_av_hud (cast `/Game/Acoustic_Vigilante/UserInterface/WBP_AV_HUD` (`WidgetComponent.GetWidget` (`self.ScoreCount`))))
  (set `self.ScoreWidget Ref` _aswbp_av_hud))

(fn `RotateToPlayer`
  (bind _returnvalue (`GameplayStatics.GetActorOfClass` "/Game/Acoustic_Vigilante/Blueprints/BP_AV_Player.BP_AV_Player_C"))
  (`SceneComponent.K2_SetWorldRotation` (`self.Cube`) (`KismetMathLibrary.FindLookAtRotation` (`SceneComponent.K2_GetComponentLocation` (`self.Cube`)) (`self.K2_GetActorLocation` _returnvalue)) false false))

(fn `UserConstructionScript`)