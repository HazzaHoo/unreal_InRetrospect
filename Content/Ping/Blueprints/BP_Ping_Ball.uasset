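; Pong-style physics ball for the Ping minigame that bounces between player and AI paddles and asks its spawner for a replacement when destroyed.
; Debounced paddle hits reverse and grow the X impulse, add a fixed Y kick by contact side, and play a sound.
; Game-instance difficulty sets speed gain and trace length.
; Each tick it traces along its velocity, sending any AI paddle impact point to that AI.
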(event `GetPlayerLocationRotationForBall`
  (params (ActorHit :type "Actor Object Reference") (HitLocation :type "Vector Structure"))
  (bind _y (.y HitLocation))
  ;[0.02287 0.15 0.01302 0.5] Add Y Axis Impluse to Hit Angle of Paddles
  (bind _asbp_ping_player (cast `/Game/Ping/Blueprints/BP_Ping_Player` ActorHit)
    (:`then`
      (if (not (>= (`self.ballspeed`) (`self.MaxSpeedBall`)))
        (set `self.ballspeed` (+ (* (`self.ballspeed`) -1.0) (`self.Speed+`))))
      (if (> _y (.y (`SceneComponent.K2_GetComponentLocation` (`/Game/Ping/Blueprints/BP_Ping_Player.Arrow` _asbp_ping_player))))
        (set `self.AngleImpluse` 125.0 :!label _label)
        (else
          (set `self.AngleImpluse` -125.0 :!label _label_2)))
      (`PrimitiveComponent.AddImpulse` (`self.Sphere`) (`KismetMathLibrary.MakeVector` (`self.ballspeed`) (`self.AngleImpluse`)) "None" true)
      (`GameplayStatics.PlaySound2D` "/Game/Ping/Audio/Hit_SFX.Hit_SFX" 1.0 1.0 0.0 null null)
      (`KismetSystemLibrary.Delay` 0.2)
      (`self.ResetHit`))
    (:`CastFailed`
      (bind _asbp_ping_ai (cast `/Game/Ping/Blueprints/BP_Ping_AI` ActorHit)
        (:`then`
          (set `self.ballspeed` (* (+ (`self.ballspeed`) (`self.Speed+`)) -1.0))
          (if (> _y (.y (`SceneComponent.K2_GetComponentLocation` (`/Game/Ping/Blueprints/BP_Ping_AI.Arrow` _asbp_ping_ai))))
            (goto _label)
            (else
              (goto _label_2))))
        (:`CastFailed`
          (`self.ResetHit`))))))

(event `self.ReceiveHit`
  (params (MyComp :type "PrimitiveComponent Object Reference") (Other :type "Actor Object Reference") (OtherComp :type "PrimitiveComponent Object Reference") (bSelfMoved :type Boolean) (HitLocation :type "Vector Structure") (HitNormal :type "Vector Structure") (NormalImpulse :type "Vector Structure") (Hit :type "HitResult Structure (by ref)"))
  ;[0.0141 0.15 0.04702 0.5] Event Hit
  (`/Engine/EditorBlueprintResources/StandardMacros.DoOnce` false :!label _label_3
    (:`Completed`
      (`self.GetPlayerLocationRotationForBall` Other HitLocation))))

(event `ResetHit`
  ;[0.0141 0.15 0.04702 0.5] Event Hit
  (goto _label_3 :!via `Reset`))

(event `self.ReceiveBeginPlay`
  ;[0.15 0 0 0.5] Impulse the ball
  (bind _returnvalue (`GameplayStatics.GetActorOfClass` "/Game/Ping/Blueprints/BP_Ping_AI.BP_Ping_AI_C"))
  (bind _output_get (set `self.AI_ref` _returnvalue))
  (set `/Game/Ping/Blueprints/BP_Ping_AI.Ballrefs` self _output_get)
  (`PrimitiveComponent.AddImpulse` (`self.Sphere`) (500.0 0.0 0.0) "None" true)
  (bind _asglobal_instance (cast `/Game/Global_IMC/Global_Instance` (`GameplayStatics.GetGameInstance`)))
  (switch `/Game/Ping/Blueprints/E_Difficulty` (`/Game/Global_IMC/Global_Instance.SelectedDifficulty` _asglobal_instance)
    (:`NewEnumerator0`
      (set `self.Speed+` 5.0)
      (set `self.DefDifficulty` 1000.0))
    (:`NewEnumerator1`
      (set `self.Speed+` 10.0)
      (set `self.DefDifficulty` 1250.0))
    (:`NewEnumerator2`
      (set `self.Speed+` 15.0)
      (set `self.DefDifficulty` 1500.0))))

(event `self.ReceiveActorBeginOverlap`
  (params (OtherActor :type "Actor Object Reference"))
  (bind _returnvalue_x (`KismetMathLibrary.BreakVector` (`self.GetVelocity`)))
  ; Progression Logic
  (cast `/Game/Ping/Blueprints/BP_Ping_Progression_Portal` OtherActor)
  (if (> _returnvalue_x 0.0)
    _))

(event `self.ReceiveDestroyed`
  ;[0.15 0 0 0.5] Spawn a ball
  (`/Game/Ping/Blueprints/BP_Ping_BallSpawner.SpawnBall` (`self.BallSpawnerRef`)))

(event `self.ReceiveTick`
  (params (DeltaSeconds :type "Float (single-precision)"))
  (bind _returnvalue (`SceneComponent.K2_GetComponentLocation` (`self.Sphere`)))
  (bind _returnvalue_2 (`PrimitiveComponent.GetPhysicsLinearVelocity` (`self.Sphere`) "None"))
  (bind (_outhit _returnvalue_3) (`KismetSystemLibrary.LineTraceSingle` :`Start` _returnvalue :`End` (+ _returnvalue (* (`KismetMathLibrary.Normal` _returnvalue_2) (`self.DefDifficulty`))) :`TraceChannel` "TraceTypeQuery1" :`DrawTime` 0.2))
  (if _returnvalue_3
    (bind (_bblockinghit _binitialoverlap _time _distance _location _impactpoint _normal _impactnormal _physmat _hitactor) (`GameplayStatics.BreakHitResult` _outhit))
    (bind _asbp_ping_ai (cast `/Game/Ping/Blueprints/BP_Ping_AI` _hitactor)
      (:`then`
        (`/Game/Ping/Blueprints/BP_Ping_AI.EventHit` _asbp_ping_ai _impactpoint))
      (:`CastFailed`
        (`self.NEwStart` :!label _label_4)))
    (else
      (goto _label_4))))

(event `NEwStart`)

(fn `UserConstructionScript`)