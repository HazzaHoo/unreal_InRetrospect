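; AI-controlled actor for the Ping game, apparently the opponent paddle, that slides along Y to track the ball.
; EventHit stores the Y of the location it receives as the target.
; Tick moves toward that target at constant speed with a swept move, clamped to fixed Y limits.
; BeginPlay sets that speed from the difficulty selected in Global_Instance and records the start location.
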(event `EventHit`
  (params (Location :type "Vector Structure"))
  (set `self.TargetLocationY` Location_Y))

(event `self.ReceiveTick`
  (params (DeltaSeconds :type "Float (single-precision)"))
  (bind (_returnvalue_x _returnvalue_y _returnvalue_z) (`KismetMathLibrary.BreakVector` (`self.K2_GetActorLocation`)))
  ;[0.15 0 0 0.5] Search for the ball
  (`self.K2_SetActorLocation` (`KismetMathLibrary.VInterpTo_Constant` (`self.K2_GetActorLocation`) (`KismetMathLibrary.MakeVector` _returnvalue_x (`KismetMathLibrary.FClamp` (`self.TargetLocationY`) -1690.0 -413.0) _returnvalue_z) DeltaSeconds (`self.AI_Speed`)) true))

(event `self.ReceiveBeginPlay`
  ;[0.15 0 0 0.5] Set difficulty
  (set `self.StartLocation` (`self.K2_GetActorLocation`))
  (bind _asglobal_instance (cast `/Game/Global_IMC/Global_Instance` (`GameplayStatics.GetGameInstance`)))
  (switch `/Game/Ping/Blueprints/E_Difficulty` (`/Game/Global_IMC/Global_Instance.SelectedDifficulty` _asglobal_instance)
    (:`NewEnumerator0`
      (set `self.AI_Speed` 400.0))
    (:`NewEnumerator1`
      (set `self.AI_Speed` 600.0))
    (:`NewEnumerator2`
      (set `self.AI_Speed` 800.0))))

(fn `UserConstructionScript`)