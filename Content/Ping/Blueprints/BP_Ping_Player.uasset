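; Player pawn for the Ping minigame, sliding a paddle cube along local Y with swept Enhanced Input movement.
; BeginPlay sets the key score threshold from Global_Instance difficulty, spawns the progression portal at a random key spawn point, and starts input, UI and music.
; The pause action first dismisses the start screen, adding the score HUD and launching the ball, then toggles the pause widget.
; An older pause-menu branch is left unconnected.
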(event `SetKeySpawnPoint`
  ; Spawn Key in Key Points In level
  (bind _outactors (`GameplayStatics.GetAllActorsOfClass` "/Game/Ping/Blueprints/BP_KeySpawnLocation.BP_KeySpawnLocation_C"))
  (`|SpawnActorFromClass` "/Game/Ping/Blueprints/BP_Ping_Progression_Portal.BP_Ping_Progression_Portal_C" (`KismetMathLibrary.MakeTransform` (`SceneComponent.K2_GetComponentLocation` (`/Game/Ping/Blueprints/BP_KeySpawnLocation.DefaultSceneRoot` (`|GetArrayItem` _outactors (`KismetMathLibrary.RandomIntegerInRange` 0 (`KismetArrayLibrary.Array_LastIndex` _outactors)))))) "Undefined" "MultiplyWithRoot" null null))

(event `EnhancedInput|/Game/Global_IMC/IA_Pause`
  (params (ActionValue :type Boolean) (ElapsedSeconds :type "Float (double-precision)") (TriggeredSeconds :type "Float (double-precision)") (InputAction :type "InputAction Object Reference" :default "/Game/Global_IMC/IA_Pause.IA_Pause"))
  (bind _pause_widget (`self.Pause Widget`))
  (bind _pause_widget_2 (`self.Pause Widget`))
  ;[0.15 0.15 0.15 0.5 74] User-interface
  ;; Input and Check Start Screen Open
  (:`Completed`
    ;; Open or Close Pause Menu
    (if (`self.StartScreenOpen?`)
      ;; Start Screen Remove and Spawn Score
      (`Widget.RemoveFromParent` (`self.Start Screen Widget`))
      (bind _returnvalue (`|CreateWidget` "/Game/Ping/UserInterface/WB_Score_Ping.WB_Score_Ping_C"))
      (bind _output_get (set `self.ScoreHUD` _returnvalue))
      (`UserWidget.AddToViewport` _output_get 2)
      (set `self.StartScreenOpen?` false)
      ;; Spawn Ball
      (bind _outactors (`GameplayStatics.GetAllActorsOfClass` "/Game/Ping/Blueprints/BP_Ping_BallSpawner.BP_Ping_BallSpawner_C"))
      (`/Game/Ping/Blueprints/BP_Ping_BallSpawner.SpawnBall` (`|GetArrayItem` _outactors))
      ;; Button Tutorial
      (bind _outactors_2 (`GameplayStatics.GetAllActorsOfClass` "/Game/Ping/Blueprints/BP_Buttons.BP_Buttons_C"))
      (`SceneComponent.SetHiddenInGame` (`/Game/Ping/Blueprints/BP_Buttons.DefaultSceneRoot` (`|GetArrayItem` _outactors_2)) true true)
      (else
        (`/Engine/EditorBlueprintResources/StandardMacros.IsValid` _pause_widget_2
          (:`Is Valid`
            (switch `ESlateVisibility` (`Widget.Visibility` _pause_widget_2)
              (:`Visible`
                (`/Game/Ping/UserInterface/WB_PauseScreen_Ping.Close Pause Menu` _pause_widget))
              (:`Hidden`
                (`/Game/Ping/UserInterface/WB_PauseScreen_Ping.Open Pause Menu` _pause_widget))))
          (:`Is Not Valid`
            (`KismetSystemLibrary.PrintString` "No Pause Menu Found")))))))

(event `Spawn Start Screen`
  ;[0.15 0.15 0.15 0.5 74] User-interface
  ;; Spawn Start Screen
  (bind _returnvalue (`|CreateWidget` "/Game/Ping/UserInterface/WB_StartScreen_Ping.WB_StartScreen_Ping_C"))
  (bind _output_get (set `self.Start Screen Widget` _returnvalue))
  (`UserWidget.AddToViewport` _output_get 0)
  (set `self.StartScreenOpen?` true)
  (bind _returnvalue_2 (`|CreateWidget` "/Game/Ping/UserInterface/WB_PauseScreen_Ping.WB_PauseScreen_Ping_C"))
  (bind _output_get_2 (set `self.Pause Widget` _returnvalue_2))
  (`UserWidget.AddToViewport` _output_get_2 0)
  (`Widget.SetVisibility` _output_get_2 "Hidden"))

(event `self.ReceiveBeginPlay`
  ;[0.15 0 0 0.5] Player Control
  (`self.Get Difficulty`)
  (`self.SetKeySpawnPoint`)
  (set `self.PingGame` true)
  (bind _asplayer_controller (cast `PlayerController` (`self.GetController`)))
  (bind _returnvalue (pcsubsystem `EnhancedInputLocalPlayerSubsystem` _asplayer_controller))
  (`/Engine/EditorBlueprintResources/StandardMacros.IsValid` _returnvalue
    (:`Is Valid`
      (`EnhancedInputSubsystemInterface.AddMappingContext` _returnvalue "/Game/Ping/IMC/IMC_Ping.IMC_Ping" 0 (struct))
      (`EnhancedInputSubsystemInterface.AddMappingContext` _returnvalue "/Game/Global_IMC/IMC_Global.IMC_Global" 0 (struct))
      (`self.Spawn Start Screen`)
      (bind _returnvalue_2 (`GameplayStatics.CreateSound2D` "/Game/Ping/Audio/Ping_Music.Ping_Music" 1.0 1.0 0.0 null))
      (`AudioComponent.FadeIn` _returnvalue_2 2.0 1.0 0.0 "Linear"))))

(event `EnhancedInput|/Game/Global_IMC/IA_Pause`
  (params (ActionValue :type Boolean) (ElapsedSeconds :type "Float (double-precision)") (TriggeredSeconds :type "Float (double-precision)") (InputAction :type "InputAction Object Reference" :default "/Game/Global_IMC/IA_Pause.IA_Pause"))
  ;[0 0 0 0.5] Call Pause Menu
)

(event `EnhancedInput|/Game/Ping/IMC/IA_Ping_Move`
  (params (ActionValue :type "Float (double-precision)") (ElapsedSeconds :type "Float (double-precision)") (TriggeredSeconds :type "Float (double-precision)") (InputAction :type "InputAction Object Reference" :default "/Game/Ping/IMC/IA_Ping_Move.IA_Ping_Move"))
  ;[0.15 0 0 0.5] Player Control
  (:`Triggered`
    (`KismetSystemLibrary.Delay` 0.001)
    (if (not (`self.StartScreenOpen?`))
      (`SceneComponent.K2_AddLocalOffset` (`self.Cube`) (`KismetMathLibrary.MakeVector` 0.0 (* ActionValue (`self.Speed`))) true false))))

(event `Fade Music Out`
  ;[0.15 0 0 0.5] Player Control
  (`/Engine/EditorBlueprintResources/StandardMacros.IsValid` (stale `self.ReceiveBeginPlay` _returnvalue_2)
    (:`Is Valid`
      (`AudioComponent.FadeOut` (stale `self.ReceiveBeginPlay` _returnvalue_2) 0.5 0.0 "Linear"))))

(fn `Get Difficulty`
  (bind _asglobal_instance (cast `/Game/Global_IMC/Global_Instance` (`GameplayStatics.GetGameInstance`)))
  (switch `/Game/Ping/Blueprints/E_Difficulty` (`/Game/Global_IMC/Global_Instance.SelectedDifficulty` _asglobal_instance)
    (:`NewEnumerator0`
      (set `self.ScoreToSpawnKey` 3))
    (:`NewEnumerator1`
      (set `self.ScoreToSpawnKey` 4))
    (:`NewEnumerator2`
      (set `self.ScoreToSpawnKey` 5))))

(fn `UserConstructionScript`)