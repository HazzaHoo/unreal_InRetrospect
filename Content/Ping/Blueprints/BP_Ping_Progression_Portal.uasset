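; Progression portal for the Ping level, shown as a flashing key that sends the game on to L_SuperFabio.
; It starts hidden with collision off and a self-recalling blink loop running, until SpawnKey enables it with Niagara and sound.
; The first overlap by a "Ball"-tagged actor fades music, shows the era transition widget and pauses.
; If the enemy has not scored, it flags PingFlawless in the GameInstance and any existing settings save.
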(event `FlashKey`
  (bind _placeholder_portalrender (`self.PlaceHolder_PortalRender`))
  ; Flash Key
  (`SceneComponent.SetVisibility` _placeholder_portalrender true false)
  (`KismetSystemLibrary.Delay` 0.5)
  (`SceneComponent.SetVisibility` _placeholder_portalrender false false)
  (`KismetSystemLibrary.Delay` 0.5)
  (`self.FlashKey`))

(event `self.ReceiveBeginPlay`
  ; Set's the Trigger to inactive at the start of the game
  (`ActorComponent.SetActive` (`self.Portal_Trigger`) false false)
  (`SceneComponent.SetHiddenInGame` (`self.PlaceHolder_PortalRender`) true false)
  (`PrimitiveComponent.SetCollisionEnabled` (`self.Portal_Trigger`) "NoCollision")
  (`self.FlashKey`))

(event `SpawnKey`
  ; Trigger Portal activation
  (`ActorComponent.SetActive` (`self.Portal_Trigger`) true false)
  (`SceneComponent.SetHiddenInGame` (`self.PlaceHolder_PortalRender`) false false)
  (`PrimitiveComponent.SetCollisionEnabled` (`self.Portal_Trigger`) "QueryAndPhysics")
  (`ActorComponent.Activate` (`self.Niagara`) false)
  (`GameplayStatics.PlaySound2D` "/Game/Ping/Audio/KeySpawn_SFX.KeySpawn_SFX" 1.0 1.0 0.0 null null))

(event `self.Portal_Trigger.OnComponentBeginOverlap`
  (params (OverlappedComponent :type "PrimitiveComponent Object Reference") (OtherActor :type "Actor Object Reference") (OtherComp :type "PrimitiveComponent Object Reference") (OtherBodyIndex :type Integer) (bFromSweep :type Boolean) (SweepResult :type "HitResult Structure (by ref)"))
  ; Trigger and Load Next Level
  (if (`self.ActorHasTag` OtherActor "Ball")
    (`/Engine/EditorBlueprintResources/StandardMacros.DoOnce` false
      (:`Completed`
        (bind _outactors (`GameplayStatics.GetAllActorsOfClass` "/Game/Ping/Blueprints/BP_Ping_Player.BP_Ping_Player_C"))
        (`/Game/Ping/Blueprints/BP_Ping_Player.Fade Music Out` (`|GetArrayItem` _outactors))
        (`self.Set EndGame Item`)
        (`GameplayStatics.PlaySound2D` "/Game/Ping/Audio/PickupKey_SFX.PickupKey_SFX" 1.0 1.0 0.0 null null)
        (bind _returnvalue (`|CreateWidget` "/Game/Global_Userinterface/WB_Transition.WB_Transition_C"))
        (`/Game/Global_Userinterface/WB_Transition.PlayerEraSound` _returnvalue)
        (`/Game/Global_Userinterface/WB_Transition.WhatEra?` _returnvalue "1" "9" "8" "L_SuperFabio")
        (`UserWidget.AddToViewport` _returnvalue 3)
        (`GameplayStatics.SetGamePaused` true)))))

(event `Set EndGame Item`
  (bind _foundwidgets (`WidgetBlueprintLibrary.GetAllWidgetsOfClass` "/Game/Ping/UserInterface/WB_Score_Ping.WB_Score_Ping_C"))
  (if (<= (`/Game/Ping/UserInterface/WB_Score_Ping.EnemyScore` (`|GetArrayItem` _foundwidgets)) 0)
    (bind _asglobal_instance (cast `/Game/Global_IMC/Global_Instance` (`GameplayStatics.GetGameInstance`)))
    (set `/Game/Global_IMC/Global_Instance.PingFlawless` true _asglobal_instance)
    (bind _returnvalue (`GameplayStatics.DoesSaveGameExist` "settings"))
    (if _returnvalue
      (bind _returnvalue_2 (`GameplayStatics.LoadGameFromSlot` "settings"))
      (bind _assettings_save_game (cast `/Game/SettingsSaveGame` _returnvalue_2))
      (set `/Game/SettingsSaveGame.PingFlawless` true _assettings_save_game)
      (`GameplayStatics.SaveGameToSlot` _assettings_save_game "settings"))))

(fn `UserConstructionScript`)