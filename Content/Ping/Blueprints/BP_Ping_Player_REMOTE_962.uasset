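; Player pawn for the Ping minigame, sliding its Cube sideways with swept local offsets through Enhanced Input once the start screen closes.
; BeginPlay spawns a progression portal at a random key spawn location, adds input mappings and shows the start screen.
; The pause input first dismisses that screen, creates the score HUD, spawns the ball and hides button hints.
; Later presses toggle a cached, animated pause widget with game pause and cursor.
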(event `SetKeySpawnPoint`
  ; Spawn Key in Key Points In level
  (bind _outactors (`GameplayStatics.GetAllActorsOfClass` "/Game/Ping/Blueprints/BP_KeySpawnLocation.BP_KeySpawnLocation_C"))
  (`|SpawnActorFromClass` "/Game/Ping/Blueprints/BP_Ping_Progression_Portal.BP_Ping_Progression_Portal_C" (`KismetMathLibrary.MakeTransform` (`SceneComponent.K2_GetComponentLocation` (`/Game/Ping/Blueprints/BP_KeySpawnLocation.DefaultSceneRoot` (`|GetArrayItem` _outactors (`KismetMathLibrary.RandomIntegerInRange` 0 (`KismetArrayLibrary.Array_LastIndex` _outactors)))))) "Undefined" "MultiplyWithRoot" null null))

(event `Close Pause Menu`
  (bind _returnvalue (`GameplayStatics.GetPlayerController` 0))
  ;[0.15 0.15 0.15 0.5 74] User-interface
  ;; Open or Close Pause Menu
  (`/Game/Ping/UserInterface/WB_PauseScreen_Ping.Close Menu Animation` (`self.As WB Pause Screen Ping`) :!label _label)
  (`KismetSystemLibrary.Delay` 0.5)
  (`Widget.SetVisibility` (`self.PauseWidget`) "Hidden")
  (`/Game/Ping/UserInterface/WB_PauseScreen_Ping.Close Menu Animation` (`self.As WB Pause Screen Ping`))
  (set `self.IsPauseMenuOpen?` false)
  (`GameplayStatics.SetGamePaused` false)
  (`WidgetBlueprintLibrary.SetInputMode_GameOnly` _returnvalue)
  (set `PlayerController.bShowMouseCursor` false _returnvalue))

(event `EnhancedInput|/Game/Global_IMC/IA_Pause`
  (params (ActionValue :type Boolean) (ElapsedSeconds :type "Float (double-precision)") (TriggeredSeconds :type "Float (double-precision)") (InputAction :type "InputAction Object Reference" :default "/Game/Global_IMC/IA_Pause.IA_Pause"))
  (bind _returnvalue (`GameplayStatics.GetPlayerController` 0))
  ;[0.15 0.15 0.15 0.5 74] User-interface
  ;; Input and Check Start Screen Open
  (:`Completed`
    ;; Open or Close Pause Menu
    (if (`self.StartScreenOpen?`)
      ;; Start Screen Remove and Spawn Score
      (`Widget.RemoveFromParent` (`self.Start Screen Widget`))
      (bind _returnvalue_2 (`|CreateWidget` "/Game/Ping/UserInterface/WB_Score_Ping.WB_Score_Ping_C"))
      (bind _output_get (set `self.ScoreHUD` _returnvalue_2))
      (`UserWidget.AddToViewport` _output_get 2)
      (set `self.StartScreenOpen?` false)
      ;; Spawn Ball
      (bind _outactors (`GameplayStatics.GetAllActorsOfClass` "/Game/Ping/Blueprints/BP_Ping_BallSpawner.BP_Ping_BallSpawner_C"))
      (`/Game/Ping/Blueprints/BP_Ping_BallSpawner.SpawnBall` (`|GetArrayItem` _outactors))
      ;; Button Tutorial
      (bind _outactors_2 (`GameplayStatics.GetAllActorsOfClass` "/Game/Ping/Blueprints/BP_Buttons.BP_Buttons_C"))
      (`SceneComponent.SetHiddenInGame` (`/Game/Ping/Blueprints/BP_Buttons.DefaultSceneRoot` (`|GetArrayItem` _outactors_2)) true true)
      (else
        (`/Engine/EditorBlueprintResources/StandardMacros.IsValid` (`self.PauseWidget`)
          (:`Is Valid`
            (if (`self.IsPauseMenuOpen?`)
              (goto _label)
              (else
                (`Widget.SetVisibility` (`self.PauseWidget`) "Visible"))))
          (:`Is Not Valid`
            (bind _returnvalue_3 (`|CreateWidget` "/Game/Ping/UserInterface/WB_PauseScreen_Ping.WB_PauseScreen_Ping_C"))
            (bind _output_get_2 (set `self.PauseWidget` _returnvalue_3))
            (`UserWidget.AddToViewport` _output_get_2 0)
            (bind _aswb_pause_screen_ping (cast `/Game/Ping/UserInterface/WB_PauseScreen_Ping` _output_get_2))
            (set `self.As WB Pause Screen Ping` _aswb_pause_screen_ping)))
        (`/Game/Ping/UserInterface/WB_PauseScreen_Ping.Play Load Animation` (`self.As WB Pause Screen Ping`))
        (set `self.IsPauseMenuOpen?` true)
        (`GameplayStatics.SetGamePaused` true)
        (`WidgetBlueprintLibrary.SetInputMode_GameAndUIEx` _returnvalue (`self.PauseWidget`) "DoNotLock" false)
        (set `PlayerController.bShowMouseCursor` true _returnvalue)))))

(event `Spawn Start Screen`
  ;[0.15 0.15 0.15 0.5 74] User-interface
  ;; Spawn Start Screen
  (bind _returnvalue (`|CreateWidget` "/Game/Ping/UserInterface/WB_StartScreen_Ping.WB_StartScreen_Ping_C"))
  (bind _output_get (set `self.Start Screen Widget` _returnvalue))
  (`UserWidget.AddToViewport` _output_get 0)
  (set `self.StartScreenOpen?` true))

(event `self.ReceiveBeginPlay`
  ;[0.15 0 0 0.5] Player Control
  (`self.SetKeySpawnPoint`)
  (set `self.PingGame` true)
  (bind _asplayer_controller (cast `PlayerController` (`self.GetController`)))
  (bind _returnvalue (pcsubsystem `EnhancedInputLocalPlayerSubsystem` _asplayer_controller))
  (`/Engine/EditorBlueprintResources/StandardMacros.IsValid` _returnvalue
    (:`Is Valid`
      (`EnhancedInputSubsystemInterface.AddMappingContext` _returnvalue "/Game/Ping/IMC/IMC_Ping.IMC_Ping" 0 (struct))
      (`EnhancedInputSubsystemInterface.AddMappingContext` _returnvalue "/Game/Global_IMC/IMC_Global.IMC_Global" 0 (struct))
      (`self.Spawn Start Screen`))))

(event `EnhancedInput|/Game/Global_IMC/IA_Pause`
  (params (ActionValue :type Boolean) (ElapsedSeconds :type "Float (double-precision)") (TriggeredSeconds :type "Float (double-precision)") (InputAction :type "InputAction Object Reference" :default "/Game/Global_IMC/IA_Pause.IA_Pause"))
  ;[0 0 0 0.5] Call Pause Menu
)

(event `EnhancedInput|/Game/Ping/IMC/IA_Ping_Move`
  (params (ActionValue :type "Float (double-precision)") (ElapsedSeconds :type "Float (double-precision)") (TriggeredSeconds :type "Float (double-precision)") (InputAction :type "InputAction Object Reference" :default "/Game/Ping/IMC/IA_Ping_Move.IA_Ping_Move"))
  ;[0.15 0 0 0.5] Player Control
  (:`Triggered`
    (if (not (`self.StartScreenOpen?`))
      (`SceneComponent.K2_AddLocalOffset` (`self.Cube`) (`KismetMathLibrary.MakeVector` 0.0 (* ActionValue (`self.Speed`))) true false))))

(fn `UserConstructionScript`)