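; BP_GetScore is a goal trigger for the Ping game that awards a point when a ball enters its box.
; On ball overlap it moves a Niagara effect to the ball and activates it, destroys the ball and plays a score sound.
; The Player1goal flag selects which score updates on the cached player's ScoreHUD, crediting the opponent of the goal's owner.
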(event `self.ReceiveBeginPlay`
  ;[0.15 0 0 0.5] Take player ref
  (bind _asbp_ping_player (cast `/Game/Ping/Blueprints/BP_Ping_Player` (`GameplayStatics.GetPlayerPawn` 0)))
  (set `self.Player_ref` _asbp_ping_player))

(event `self.Box.OnComponentBeginOverlap`
  (params (OverlappedComponent :type "PrimitiveComponent Object Reference") (OtherActor :type "Actor Object Reference") (OtherComp :type "PrimitiveComponent Object Reference") (OtherBodyIndex :type Integer) (bFromSweep :type Boolean) (SweepResult :type "HitResult Structure (by ref)"))
  (bind _niagara (`self.Niagara`))
  ;[0.15 0 0 0.5] Transfer info from player/AI to Widget and gives score to AI/Player
  (bind _asbp_ping_ball (cast `/Game/Ping/Blueprints/BP_Ping_Ball` OtherActor))
  (`SceneComponent.K2_SetWorldLocation` _niagara (`SceneComponent.K2_GetComponentLocation` (`/Game/Ping/Blueprints/BP_Ping_Ball.Sphere` _asbp_ping_ball)) false false)
  (`ActorComponent.Activate` _niagara false)
  (`self.K2_DestroyActor` _asbp_ping_ball)
  (if (`self.Player1goal?`)
    (`/Game/Ping/UserInterface/WB_Score_Ping.UpdatePlayer_2_score` (`/Game/Ping/Blueprints/BP_Ping_Player.ScoreHUD` (`self.Player_ref`)))
    (else
      (`/Game/Ping/UserInterface/WB_Score_Ping.UpdatePlayer_1_score` (`/Game/Ping/Blueprints/BP_Ping_Player.ScoreHUD` (`self.Player_ref`)))))
  (`GameplayStatics.PlaySound2D` "/Game/Ping/Audio/Score_SFX.Score_SFX" 1.0 1.0 0.0 null null))

(fn `UserConstructionScript`)