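; Bullet projectile that damages the player on contact or ricochets visually off anything else.
; BeginPlay copies BulletSpeed into ProjectileMovement, then enables Sphere2 collision after a short delay.
; An overlap with a Player-tagged actor calls PlayerDamage on BP_CP_Player and destroys the bullet.
; Other overlaps stop movement, hide Sphere, disable Sphere2 collision and spawn ricochet VFX and sound before a delayed destroy, with leftover debug prints.
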(event `self.ReceiveBeginPlay`
  (bind _bulletspeed (`self.BulletSpeed`))
  (bind _projectilemovement (`self.ProjectileMovement`))
  (set `ProjectileMovementComponent.MaxSpeed` _bulletspeed _projectilemovement)
  (set `ProjectileMovementComponent.InitialSpeed` _bulletspeed _projectilemovement)
  (`KismetSystemLibrary.Delay` 0.5)
  (`PrimitiveComponent.SetCollisionEnabled` (`self.Sphere2`) "QueryAndPhysics"))

(event `self.Sphere2.OnComponentBeginOverlap`
  (params (OverlappedComponent :type "PrimitiveComponent Object Reference") (OtherActor :type "Actor Object Reference") (OtherComp :type "PrimitiveComponent Object Reference") (OtherBodyIndex :type Integer) (bFromSweep :type Boolean) (SweepResult :type "HitResult Structure (by ref)"))
  (bind _returnvalue (`self.K2_GetActorLocation`))
  (`KismetSystemLibrary.PrintString` "Hello")
  (if (== OtherActor self)
    _
    (elif (`self.ActorHasTag` OtherActor "Player")
      (bind _asbp_cp_player (cast `/Game/Chrono_Panic/Blueprints/BP_CP_Player` OtherActor))
      (`/Game/Chrono_Panic/Blueprints/BP_CP_Player.Player Damage` _asbp_cp_player)
      (`self.K2_DestroyActor`)
      (else
        (`KismetSystemLibrary.PrintString` "Hello")
        (`MovementComponent.StopMovementImmediately` (`self.ProjectileMovement`))
        (`SceneComponent.SetHiddenInGame` (`self.Sphere`) true false)
        (`PrimitiveComponent.SetCollisionEnabled` (`self.Sphere2`) "NoCollision")
        (`NiagaraFunctionLibrary.SpawnSystemAtLocation` "/Game/Chrono_Panic/VFX/CP_VFX_Ricochet.CP_VFX_Ricochet" _returnvalue)
        (`GameplayStatics.SpawnSoundAtLocation` "/Game/Chrono_Panic/Audio/Richochet_01_Cue.Richochet_01_Cue" _returnvalue (struct) 1.0 1.0 0.0 null null)
        (`KismetSystemLibrary.Delay` 1.0)
        (`self.K2_DestroyActor`)))))

(fn `UserConstructionScript`)