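; Enemy bullet projectile for Chrono Panic that damages the player or ricochets off anything else it hits.
; BeginPlay applies BulletSpeed to the projectile movement and caches the rifle of the owning BP_CP_Enemy2.
; Sphere overlaps ignore that rifle and itself, calling PlayerDamage and destroying the bullet on a Player-tagged actor.
; Other overlaps stop and hide the bullet, play ricochet effects and destroy it after a short delay.
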(event `self.ReceiveBeginPlay`
  (bind _bulletspeed (`self.BulletSpeed`))
  (bind _projectilemovement (`self.ProjectileMovement`))
  (set `ProjectileMovementComponent.MaxSpeed` _bulletspeed _projectilemovement)
  (set `ProjectileMovementComponent.InitialSpeed` _bulletspeed _projectilemovement)
  (bind _asbp_cp_enemy_2 (cast `/Game/Chrono_Panic/Blueprints/BP_CP_Enemy2` (`self.GetOwner`)))
  (set `self.RifleRef` (`/Game/Chrono_Panic/Blueprints/BP_CP_Enemy2.SM_Rifle` _asbp_cp_enemy_2)))

(event `self.Sphere.OnComponentBeginOverlap`
  (params (OverlappedComponent :type "PrimitiveComponent Object Reference") (OtherActor :type "Actor Object Reference") (OtherComp :type "PrimitiveComponent Object Reference") (OtherBodyIndex :type Integer) (bFromSweep :type Boolean) (SweepResult :type "HitResult Structure (by ref)"))
  (bind _returnvalue (`self.K2_GetActorLocation`))
  (if (or (== OtherComp (`self.RifleRef`)) (== OtherActor self))
    _
    (elif (`self.ActorHasTag` OtherActor "Player")
      ; Hit Player
      (bind _asbp_cp_player (cast `/Game/Chrono_Panic/Blueprints/BP_CP_Player` OtherActor))
      (`/Game/Chrono_Panic/Blueprints/BP_CP_Player.Player Damage` _asbp_cp_player)
      (`self.K2_DestroyActor`)
      (else
        ; Ricohet
        (`MovementComponent.StopMovementImmediately` (`self.ProjectileMovement`))
        (`SceneComponent.SetHiddenInGame` (`self.Cube`) true false)
        (`PrimitiveComponent.SetCollisionEnabled` (`self.Sphere`) "NoCollision")
        (`NiagaraFunctionLibrary.SpawnSystemAtLocation` "/Game/Chrono_Panic/VFX/CP_VFX_Ricochet.CP_VFX_Ricochet" _returnvalue)
        (`GameplayStatics.SpawnSoundAtLocation` "/Game/Chrono_Panic/Audio/Richochet_01_Cue.Richochet_01_Cue" _returnvalue (struct) 1.0 1.0 0.0 null null)
        (`KismetSystemLibrary.Delay` 1.0)
        (`self.K2_DestroyActor`)))))

(fn `UserConstructionScript`)