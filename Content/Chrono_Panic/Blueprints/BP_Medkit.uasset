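; BP_Medkit is a health pickup actor for Chrono Panic that heals the player.
; On BeginPlay, two timelines animate its Cube component, one driving rotation and the other vertical offset through lerps.
; HealPlayer, with no caller in this Blueprint, plays the heal animation on the first in-game HUD widget, calls PlayerHeal on the BP_CP_Player found by class lookup, then destroys the medkit.
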(event `self.ReceiveBeginPlay`
  (bind _cube (`self.Cube`))
  ; Animation
  (`|ExecutionSequence`
    (:`then_0`
      (bind (_direction _lerp) (`Timeline|Timeline`)
        (:`Update`
          (`SceneComponent.K2_SetRelativeRotation` _cube (`KismetMathLibrary.RLerp` (struct :`Pitch` -38.973944) (struct :`Pitch` -38.973944 :`Yaw` 360.0) _lerp) false false))))
    (:`then_1`
      (bind (_direction_2 _lerp_2) (`Timeline|T_Animate`)
        (:`Update`
          (`SceneComponent.K2_SetRelativeLocation` _cube (`KismetMathLibrary.VLerp` (0.0 0.0 0.0) (0.0 0.0 50.0) _lerp_2) false false))))))

(event `Heal Player`
  (bind _foundwidgets (`WidgetBlueprintLibrary.GetAllWidgetsOfClass` "/Game/Chrono_Panic/UserInterface/WB_In-GameHUD_ChronoPanic.WB_In-GameHUD_ChronoPanic_C"))
  (`/Game/Chrono_Panic/UserInterface/WB_In-GameHUD_ChronoPanic.Heal HUD Animation` (`|GetArrayItem` _foundwidgets))
  (bind _returnvalue (`GameplayStatics.GetActorOfClass` "/Game/Chrono_Panic/Blueprints/BP_CP_Player.BP_CP_Player_C"))
  (`/Game/Chrono_Panic/Blueprints/BP_CP_Player.PlayerHeal` _returnvalue)
  (`self.K2_DestroyActor`))

(fn `UserConstructionScript`)