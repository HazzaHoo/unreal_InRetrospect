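; Player for Chrono Panic, an on-rails cover shooter that moves along BP_CP_PlayerSpline and stops at checkpoints to fight enemies.
; Tick aims the pistol at the mouse and advances movement; shots trace under the cursor to hit enemies, boss, medkits or exit portal, with bullet-by-bullet reloading.
; Crouch and gated strafe timelines offset the camera and toggle invincibility.
; Also handles health, HUD, pause and game-over screens, and music.
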(event `FadeMusicOut`
  (params (FadeOutTime :type "Float (double-precision)"))
  ; Fade Music In or Out
  (`|ExecutionSequence`
    (:`then_0`
      (`/Engine/EditorBlueprintResources/StandardMacros.IsValid` (stale `FadeMusicIN` _returnvalue)
        (:`Is Valid`
          (`AudioComponent.FadeOut` (stale `FadeMusicIN` _returnvalue) FadeOutTime 0.0 "Linear"))))))

(event `Close Pause Menu`
  (bind _returnvalue (`GameplayStatics.GetPlayerController` 0))
  ;[0.15 0.15 0.15 0.5 74] User-interface
  ;; Open or Close Pause Menu
  (`GameplayStatics.SetGamePaused` false :!label _label)
  (`/Game/Chrono_Panic/UserInterface/WB_PauseScreen_ChronoPanic.Close Load Anim` (`self.As WB Pause Screen Chrono Panic`))
  (`KismetSystemLibrary.Delay` 1.0)
  (`Widget.SetVisibility` (`self.PauseWidget`) "Hidden")
  (set `self.IsPauseMenuOpen?` false)
  (`WidgetBlueprintLibrary.SetInputMode_GameOnly` _returnvalue)
  (set `PlayerController.bShowMouseCursor` false _returnvalue))

(event `FadeMusicIN`
  ; Fade Music In or Out
  (bind _returnvalue (`GameplayStatics.CreateSound2D` "/Game/Chrono_Panic/Audio/ChronoPanic_Music.ChronoPanic_Music" 1.0 1.0 0.0 null))
  (`AudioComponent.FadeIn` _returnvalue 2.0 1.0 0.0 "Linear"))

(event `EnhancedInput|/Game/Global_IMC/IA_Pause`
  (params (ActionValue :type Boolean) (ElapsedSeconds :type "Float (double-precision)") (TriggeredSeconds :type "Float (double-precision)") (InputAction :type "InputAction Object Reference" :default "/Game/Global_IMC/IA_Pause.IA_Pause"))
  (bind _returnvalue (`GameplayStatics.GetPlayerController` 0))
  ;[0.15 0.15 0.15 0.5 74] User-interface
  ;; Open or Close Pause Menu
  (:`Completed`
    (`/Engine/EditorBlueprintResources/StandardMacros.IsValid` (`self.PauseWidget`)
      (:`Is Valid`
        (if (`self.IsPauseMenuOpen?`)
          (goto _label)
          (else
            (`Widget.SetVisibility` (`self.PauseWidget`) "Visible"))))
      (:`Is Not Valid`
        (bind _returnvalue_2 (`|CreateWidget` "/Game/Chrono_Panic/UserInterface/WB_PauseScreen_ChronoPanic.WB_PauseScreen_ChronoPanic_C"))
        (bind _output_get (set `self.PauseWidget` _returnvalue_2))
        (`UserWidget.AddToViewport` _output_get 1)
        (bind _aswb_pause_screen_chrono_panic (cast `/Game/Chrono_Panic/UserInterface/WB_PauseScreen_ChronoPanic` _output_get))
        (bind _output_get_2 (set `self.As WB Pause Screen Chrono Panic` _aswb_pause_screen_chrono_panic))))
    (`/Game/Chrono_Panic/UserInterface/WB_PauseScreen_ChronoPanic.Play Load Anim` _output_get_2)
    (set `self.IsPauseMenuOpen?` true)
    (`GameplayStatics.SetGamePaused` true :!label _label_2)
    (`WidgetBlueprintLibrary.SetInputMode_GameAndUIEx` _returnvalue (`self.PauseWidget`) "DoNotLock" false)
    (set `PlayerController.bShowMouseCursor` true _returnvalue)))

(event `GameOverInput`
  ;[0.15 0.15 0.15 0.5 74] User-interface
  ;; Open or Close Pause Menu
  (goto _label_2))

(event `Spawn In-Game HUD`
  ;[0.15 0.15 0.15 0.5 74] User-interface
  ;; Spawn In Game HUD
  (bind _returnvalue (`|CreateWidget` "/Game/Chrono_Panic/UserInterface/WB_In-GameHUD_ChronoPanic.WB_In-GameHUD_ChronoPanic_C"))
  (bind _output_get (set `self.HUDWidget` _returnvalue))
  (`UserWidget.AddToViewport` _output_get 0)
  (bind _returnvalue_2 (`|CreateWidget` "/Game/Chrono_Panic/UserInterface/WB_Crosshair.WB_Crosshair_C"))
  (`UserWidget.AddToViewport` _returnvalue_2 0))

(event `EnhancedInput|/Game/Chrono_Panic/IMC/IA_CP_StrafeRight`
  (params (ActionValue :type Boolean) (ElapsedSeconds :type "Float (double-precision)") (TriggeredSeconds :type "Float (double-precision)") (InputAction :type "InputAction Object Reference" :default "/Game/Chrono_Panic/IMC/IA_CP_StrafeRight.IA_CP_StrafeRight"))
  (bind _cameradefaultlocation_relative_ (`self.CameraDefaultLocation(Relative)`))
  (bind _cameradefaultlocation_relative__2 (`self.CameraDefaultLocation(Relative)`))
  ; Strafe System
  (:`Triggered`
    (`/Engine/EditorBlueprintResources/StandardMacros.Gate` false :!label _label_3
      (:`Exit`
        (`/Engine/EditorBlueprintResources/StandardMacros.DoOnce` false :!label _label_4
          (:`Completed`
            (`|ExecutionSequence`
              (:`then_0`
                (`self.CloseRightStrafeGate`))
              (:`then_1`
                (`self.CloseLeftStrafeGate`))
              (:`then_2`
                (set `self.LeftStrafe?` false)
                (set `self.IsStrafing` true :!label _label_5)
                (set `self.isInvincible` false)
                (set `self.CameraDefaultLocation(Relative)` (`SceneComponent.RelativeLocation` (`self.Camera`)))
                (bind _returnvalue (`GameplayStatics.CreateSound2D` "/Game/Chrono_Panic/Audio/Strafe.Strafe" 1.0 1.0 0.0 null))
                (`AudioComponent.SetPitchMultiplier` _returnvalue (`KismetMathLibrary.RandomFloatInRange` 0.75 1.25))
                (`AudioComponent.Play` _returnvalue 0.0)
                (if (`self.isCrouching`)
                  (set `self.StrafeHeight` (`self.CrouchHeight`))
                  (bind (_direction _strafe) (`Timeline|TL_Strafe` :!label _label_6)
                    (:`Update`
                      (if (`self.LeftStrafe?`)
                        (`SceneComponent.K2_SetRelativeLocation` (`self.Camera`) (`KismetMathLibrary.VLerp` (`KismetMathLibrary.MakeVector` (.x _cameradefaultlocation_relative__2) (.y _cameradefaultlocation_relative__2) (`self.StrafeHeight`)) (`KismetMathLibrary.MakeVector` (.x _cameradefaultlocation_relative__2) (+ (.y _cameradefaultlocation_relative__2) (`self.StrafeLeftOffset`)) (`self.StrafeHeight`)) _strafe) false false)
                        (else
                          (`SceneComponent.K2_SetRelativeLocation` (`self.Camera`) (`KismetMathLibrary.VLerp` (`KismetMathLibrary.MakeVector` (.x _cameradefaultlocation_relative_) (.y _cameradefaultlocation_relative_) (`self.StrafeHeight`)) (`KismetMathLibrary.MakeVector` (.x _cameradefaultlocation_relative_) (+ (.y _cameradefaultlocation_relative_) (`self.StrafeRightOffset`)) (`self.StrafeHeight`)) _strafe) false false))))
                    (:`Finished`
                      (if (== _strafe 0.0)
                        (`|ExecutionSequence`
                          (:`then_0`
                            (`self.OpenLeftStrafeGate`))
                          (:`then_1`
                            (`self.OpenRightStrafeGate`))
                          (:`then_2`
                            (`self.ResetStrafeDoOnce`))))))
                  (else
                    (set `self.StrafeHeight` (`self.StandHeight`))
                    (goto _label_6))))))))))
  (:`Started`
    (goto _label_3))
  (:`Completed`
    (set `self.IsStrafing` false :!label _label_7)
    (set `self.isInvincible` true)
    (if (`self.isCrouching`)
      (set `self.StrafeHeight` (`self.CrouchHeight`))
      (goto _label_6 :!via `Reverse`)
      (else
        (set `self.StrafeHeight` (`self.StandHeight`))
        (goto _label_6 :!via `Reverse`)))))

(event `OpenRightStrafeGate`
  ; Strafe System
  (goto _label_3 :!via `Open`))

(event `ResetStrafeDoOnce`
  ; Strafe System
  (`|ExecutionSequence`
    (:`then_0`
      (goto _label_4 :!via `Reset`))
    (:`then_1`
      (goto _label_9 :!via `Reset`))))

(event `CloseRightStrafeGate`
  ; Strafe System
  (goto _label_3 :!via `Close`))

(event `EnhancedInput|/Game/Chrono_Panic/IMC/IA_CP_StrafeLeft`
  (params (ActionValue :type Boolean) (ElapsedSeconds :type "Float (double-precision)") (TriggeredSeconds :type "Float (double-precision)") (InputAction :type "InputAction Object Reference" :default "/Game/Chrono_Panic/IMC/IA_CP_StrafeLeft.IA_CP_StrafeLeft"))
  ; Strafe System
  (:`Triggered`
    (`/Engine/EditorBlueprintResources/StandardMacros.Gate` true :!label _label_8
      (:`Exit`
        (`/Engine/EditorBlueprintResources/StandardMacros.DoOnce` false :!label _label_9
          (:`Completed`
            (`|ExecutionSequence`
              (:`then_0`
                (set `self.LeftStrafe?` true)
                (goto _label_5))
              (:`then_1`
                (`self.CloseRightStrafeGate`))
              (:`then_2`
                (`self.CloseLeftStrafeGate`))))))))
  (:`Started`
    (goto _label_8))
  (:`Completed`
    (goto _label_7)))

(event `OpenLeftStrafeGate`
  ; Strafe System
  (goto _label_8 :!via `Open`))

(event `CloseLeftStrafeGate`
  ; Strafe System
  (goto _label_8 :!via `Close`))

(event `EnhancedInput|/Game/Chrono_Panic/IMC/IA_CP_ControlsMenu`
  (params (ActionValue :type Boolean) (ElapsedSeconds :type "Float (double-precision)") (TriggeredSeconds :type "Float (double-precision)") (InputAction :type "InputAction Object Reference" :default "/Game/Chrono_Panic/IMC/IA_CP_ControlsMenu.IA_CP_ControlsMenu"))
  ; Open Close Controls
  (:`Started`
    (`/Game/Chrono_Panic/UserInterface/WB_Controls_Chrono.OpenOrCloseControls` (`self.Controls Menu Widget Ref`))))

(event `self.ReceiveBeginPlay`
  (bind _strafeoffset (`self.StrafeOffset`))
  (bind (_relativelocation_x _relativelocation_y) (`KismetMathLibrary.BreakVector` (`SceneComponent.RelativeLocation` (`self.Camera`))))
  (set `PlayerController.bShowMouseCursor` false (`PlayerState.GetPlayerController` (`self.PlayerState`)))
  ; Update Default Location and Spawn Controls
  (bind _returnvalue (`|CreateWidget` "/Game/Chrono_Panic/UserInterface/WB_Controls_Chrono.WB_Controls_Chrono_C"))
  (`UserWidget.AddToViewport` _returnvalue 0)
  (set `self.Controls Menu Widget Ref` _returnvalue)
  (`self.IntroDoors`)
  (set `self.CameraDefaultLocation(Relative)` (`SceneComponent.RelativeLocation` (`self.Camera`)))
  (`SceneComponent.K2_SetRelativeLocation` (`self.Camera`) (`KismetMathLibrary.MakeVector` _relativelocation_x _relativelocation_y (`self.StandHeight`)) false false)
  ; Player Control
  (`self.FadeMusicIN`)
  (set `self.CP_Game` true)
  (bind _asplayer_controller (cast `PlayerController` (`self.GetController`)))
  (set `self.ControllerRef` _asplayer_controller)
  (bind _returnvalue_2 (pcsubsystem `EnhancedInputLocalPlayerSubsystem` _asplayer_controller))
  (`/Engine/EditorBlueprintResources/StandardMacros.IsValid` _returnvalue_2
    (:`Is Valid`
      (`EnhancedInputSubsystemInterface.AddMappingContext` _returnvalue_2 "/Game/Chrono_Panic/IMC/IMC_ChronoPanic.IMC_ChronoPanic" 0 (struct))
      (`EnhancedInputSubsystemInterface.AddMappingContext` _returnvalue_2 "/Game/Global_IMC/IMC_Global.IMC_Global" 0 (struct))
      (bind _returnvalue_3 (`GameplayStatics.GetActorOfClass` "/Game/Chrono_Panic/Blueprints/BP_CP_PlayerSpline.BP_CP_PlayerSpline_C"))
      (set `self.MovementSpline` _returnvalue_3)
      (`self.Spawn In-Game HUD`)
      (set `self.StrafeRightOffset` _strafeoffset)
      (set `self.StrafeLeftOffset` (* _strafeoffset -1.0)))))

(event `CalculateCrosshair`
  (bind _pistol_uv (`self.PISTOL_UV`))
  (bind (_worldlocation _worlddirection) (`PlayerController.DeprojectMousePositionToWorld` (`PlayerState.GetPlayerController` (`self.PlayerState`))))
  ; Move Gun to Mouse Position
  (bind _outhit (`KismetSystemLibrary.LineTraceSingle` _worldlocation (+ _worldlocation (* _worlddirection 10000.0)) "TraceTypeQuery1"))
  (`SceneComponent.K2_SetWorldRotation` _pistol_uv (`KismetMathLibrary.ComposeRotators` (`KismetMathLibrary.RLerp` (struct) (struct :`Pitch` 15.0) (stale `ShootGun` _lerp)) (`KismetMathLibrary.FindLookAtRotation` (`SceneComponent.K2_GetComponentLocation` _pistol_uv) (`.TraceEnd` (`GameplayStatics.BreakHitResult` _outhit)))) false false))

(event `EnemyKilled`
  ; Shoot Enemies
  (if (== (`self.CurentCheckpoint`) 2)
    (`KismetSystemLibrary.Delay` 0.75))
  (`/Game/Chrono_Panic/Blueprints/BP_CP_PlayerSpline.EnemyKilled` (`self.MovementSpline`) (stale `EnhancedInput|/Game/Chrono_Panic/IMC/IA_CP_Shoot` _asbp_cp_enemy_2)))

(event `EnhancedInput|/Game/Chrono_Panic/IMC/IA_CP_Reload`
  (params (ActionValue :type Boolean) (ElapsedSeconds :type "Float (double-precision)") (TriggeredSeconds :type "Float (double-precision)") (InputAction :type "InputAction Object Reference" :default "/Game/Chrono_Panic/IMC/IA_CP_Reload.IA_CP_Reload"))
  (bind _hudwidget (`self.HUDWidget`))
  ; Player Control
  ;; Reload
  (:`Completed`
    (if (`self.IsReloading?`)
      _
      (elif (not (== (`self.Current Ammo`) (`self.Max Ammo`)))
        (`GameplayStatics.PlaySound2D` "/Game/Chrono_Panic/Audio/StartReload.StartReload" 1.0 1.0 0.0 null null :!label _label_10)
        (set `self.IsReloading?` true :!label _label_11)
        (bind _result (`/Engine/EditorBlueprintResources/StandardMacros.IncrementInt` (`self.Current Ammo`))
          (:`  `
            (bind _output_get (set `self.Current Ammo` _result))
            (if (== _output_get (`self.Max Ammo`))
              (set `self.IsReloading?` false)
              (`/Game/Chrono_Panic/UserInterface/WB_In-GameHUD_ChronoPanic.Update Ammo` _hudwidget)
              (`GameplayStatics.PlaySound2D` "/Game/Chrono_Panic/Audio/EndReload.EndReload" 1.0 1.0 0.0 null null)
              (else
                (`KismetSystemLibrary.Delay` (`self.TimeBetweenEachBulletLoad`))
                (`/Game/Chrono_Panic/UserInterface/WB_In-GameHUD_ChronoPanic.Update Ammo` _hudwidget)
                (`self.LoopReload`)))))))))

(event `LoopReload`
  ; Player Control
  ;; Reload
  (goto _label_11))

(event `Reload`
  ; Player Control
  ;; Reload
  (goto _label_10))

(event `EnhancedInput|/Game/Chrono_Panic/IMC/IA_CP_Shoot`
  (params (ActionValue :type Boolean) (ElapsedSeconds :type "Float (double-precision)") (TriggeredSeconds :type "Float (double-precision)") (InputAction :type "InputAction Object Reference" :default "/Game/Chrono_Panic/IMC/IA_CP_Shoot.IA_CP_Shoot"))
  (bind _hitresult (`PlayerController.GetHitResultUnderCursorByChannel` (`self.ControllerRef`) "TraceTypeQuery1" true))
  ; Shoot Enemies
  (:`Started`
    (if (and (`self.CanShoot`) (> (`self.Current Ammo`) 0))
      (if (not (`self.IsReloading?`))
        (bind _returnvalue (`GameplayStatics.CreateSound2D` "/Game/Chrono_Panic/Audio/GunShot.GunShot" 1.0 1.0 0.0 null))
        (`AudioComponent.SetPitchMultiplier` _returnvalue (`KismetMathLibrary.RandomFloatInRange` 0.75 1.25))
        (`AudioComponent.Play` _returnvalue 0.0)
        (`self.ShootGun`)
        (`self.Ammo Count`)
        (`GameplayStatics.PlayWorldCameraShake` "/Game/Chrono_Panic/UserInterface/BP_CameraShake_Shooting.BP_CameraShake_Shooting_C" (`self.K2_GetActorLocation`) 0.0 1000.0)
        (`ActorComponent.Activate` (`self.CP_VFX_MuzzleFlash`) true)
        (bind _output_get (set `self.OutHitActorForShooting` (`.HitActor` (`GameplayStatics.BreakHitResult` _hitresult))))
        (bind _asbp_cp_enemy_2 (cast `/Game/Chrono_Panic/Blueprints/BP_CP_Enemy2` _output_get)
          (:`then`
            (`/Game/Chrono_Panic/Blueprints/BP_CP_Enemy2.Damage` _asbp_cp_enemy_2 (`self.Damage to Enemies`) self)
            (`NiagaraFunctionLibrary.SpawnSystemAtLocation` "/Game/Chrono_Panic/VFX/CP_VFX_Blood.CP_VFX_Blood" (`.Location` (`GameplayStatics.BreakHitResult` _hitresult)) :!label _label_12))
          (:`CastFailed`
            (bind _asbp_cp_progression_portal (cast `/Game/Chrono_Panic/Blueprints/BP_CP_Progression_Portal` (`self.OutHitActorForShooting`))
              (:`then`
                (`/Game/Chrono_Panic/Blueprints/BP_CP_Progression_Portal.EndLevel` _asbp_cp_progression_portal))
              (:`CastFailed`
                (bind _asbp_medkit (cast `/Game/Chrono_Panic/Blueprints/BP_Medkit` (`self.OutHitActorForShooting`))
                  (:`then`
                    (`/Game/Chrono_Panic/Blueprints/BP_Medkit.Heal Player` _asbp_medkit))
                  (:`CastFailed`
                    (bind _asbp_cc_boss (cast `/Game/Chrono_Panic/Blueprints/BP_CC_Boss` (`self.OutHitActorForShooting`))
                      (:`then`
                        (`/Game/Chrono_Panic/Blueprints/BP_CC_Boss.BossHit` _asbp_cc_boss)
                        (goto _label_12))
                      (:`CastFailed`
                        (`NiagaraFunctionLibrary.SpawnSystemAtLocation` "/Game/Chrono_Panic/VFX/CP_VFX_Ricochet.CP_VFX_Ricochet" (`.Location` (`GameplayStatics.BreakHitResult` _hitresult)))
                        (`GameplayStatics.SpawnSoundAtLocation` "/Game/Chrono_Panic/Audio/Richochet_01_Cue.Richochet_01_Cue" (`.Location` (`GameplayStatics.BreakHitResult` _hitresult)) (struct) 1.0 1.0 0.0 null null)))))))))))))

(event `ShootGun`
  ; Move Gun to Mouse Position
  ;; Recoil
  (bind (_direction _lerp) (`Timeline|T_ShootGun` :!via `PlayFromStart`)))

(event `EnhancedInput|/Game/Chrono_Panic/IMC/IA_CP_Crouch`
  (params (ActionValue :type Boolean) (ElapsedSeconds :type "Float (double-precision)") (TriggeredSeconds :type "Float (double-precision)") (InputAction :type "InputAction Object Reference" :default "/Game/Chrono_Panic/IMC/IA_CP_Crouch.IA_CP_Crouch"))
  (:`Started`
    ; Player Control
    ;; Crouching
    (if (not (`self.isMoving`))
      (set `self.isCrouching` true)
      (set `self.isInvincible` true)
      (`GameplayStatics.PlaySound2D` "/Game/Chrono_Panic/Audio/Crouch.Crouch" 1.0 1.0 0.0 null null)
      (bind (_direction _crouch) (`Timeline|TL_Crouch` :!label _label_13)
        (:`Update`
          (`SceneComponent.K2_SetRelativeLocation` (`self.Camera`) (`KismetMathLibrary.MakeVector` (.x (`SceneComponent.RelativeLocation` (`self.Camera`))) (.y (`SceneComponent.RelativeLocation` (`self.Camera`))) (`KismetMathLibrary.Lerp` (`self.StandHeight`) (`self.CrouchHeight`) _crouch)) false false)))))
  (:`Completed`
    (`GameplayStatics.PlaySound2D` "/Game/Chrono_Panic/Audio/Crouch.Crouch" 1.0 1.0 0.0 null null)
    (set `self.isCrouching` false :!label _label_14)
    (set `self.isInvincible` false)
    (goto _label_13 :!via `Reverse`)))

(event `ForceUnCrouch`
  ; Player Control
  ;; Crouching
  (goto _label_14))

(event `Enable Player Shooting`
  ; Player Control
  (set `self.CanShoot` true))

(event `Ammo Count`
  ; Ammo Count (Takes away one bullet and updates UI)
  (bind _result (`/Engine/EditorBlueprintResources/StandardMacros.DecrementInt` (`self.Current Ammo`))
    (:`  `
      (`/Engine/EditorBlueprintResources/StandardMacros.IncrementInt` (`self.ShotsFired`)
        (:`  `
          (bind _output_get (set `self.Current Ammo` (`KismetMathLibrary.Clamp` _result 0 (`self.Max Ammo`))))
          (`/Game/Chrono_Panic/UserInterface/WB_In-GameHUD_ChronoPanic.Update Ammo` (`self.HUDWidget`))
          (if (== _output_get 0)
            (`self.Reload`)))))))

(event `self.ReceiveTick`
  (params (DeltaSeconds :type "Float (single-precision)"))
  ; Player Control
  ;; Move player
  (`self.CalculateCrosshair`)
  (if (`self.isMoving`)
    (set `self.CheckpointTriggered` false)
    (set `PlayerController.bShowMouseCursor` false (`self.ControllerRef`))
    (bind _output_get (set `self.CurrentDistance` (+ (`self.CurrentDistance`) (* (`self.MoveSpeed`) (`GameplayStatics.GetWorldDeltaSeconds`)))))
    (`self.K2_SetActorLocation` (`SplineComponent.GetLocationAtDistanceAlongSpline` (`/Game/Chrono_Panic/Blueprints/BP_CP_PlayerSpline.Spline` (`self.MovementSpline`)) _output_get "World"))
    (`self.CameraRotationAlongSpline` (< (`KismetMathLibrary.Vector_DistanceSquared` (`SceneComponent.K2_GetComponentLocation` (`|GetArrayItem` (`/Game/Chrono_Panic/Blueprints/BP_CP_PlayerSpline.CheckpointArrows` (`self.MovementSpline`)) (`self.CurentCheckpoint`))) (`self.K2_GetActorLocation`)) 50000.0))
    (`KismetSystemLibrary.Delay` 0.5)
    (`GameplayStatics.PlayWorldCameraShake` "/Game/Chrono_Panic/UserInterface/BP_CameraShake_Move.BP_CameraShake_Move_C" (`self.K2_GetActorLocation`) 0.0 1000.0)
    (`GameplayStatics.PlaySound2D` "/Game/Chrono_Panic/Audio/Footstep_03_Cue.Footstep_03_Cue" 1.0 1.0 0.0 null null)
    (if (and (not (`self.CheckpointTriggered`)) (>= (`self.CurrentDistance`) (`|GetArrayItem` (`/Game/Chrono_Panic/Blueprints/BP_CP_PlayerSpline.CheckpointDistances` (`self.MovementSpline`)) (`self.CurentCheckpoint`))))
      (`self.ReachedCheckpoint`))))

(event `First Enemy Death`
  ; Player Control
  ;; Move player
  (`KismetSystemLibrary.Delay` 1.0)
  ;;; temp moving
  (if (not (`self.isMoving`)) :!label _label_15
    (set `self.CurentCheckpoint` (+ (`self.CurentCheckpoint`) 1))
    (set `self.isMoving` true)))

(event `IntroDoors`
  ; Player Control
  ;; Move player
  ;;; temp moving
  (`KismetSystemLibrary.Delay` (`self.TimeBeforeIntroDoors`))
  (goto _label_15))

(event `Player Damage`
  (bind _hudwidget (`self.HUDWidget`))
  ; Player Damage (Take away one life)
  (if (not (`self.isInvincible`))
    (`GameplayStatics.PlayWorldCameraShake` "/Game/Chrono_Panic/UserInterface/BP_CameraShake_Damage.BP_CameraShake_Damage_C" (`self.K2_GetActorLocation`) 0.0 1000.0)
    (set `self.Health` (- (`self.Health`) (`self.Bullet Damage`)))
    (`/Game/Chrono_Panic/UserInterface/WB_In-GameHUD_ChronoPanic.Update Lives` _hudwidget :!label _label_16)
    (`/Game/Chrono_Panic/UserInterface/WB_In-GameHUD_ChronoPanic.Damage HUD Animation` _hudwidget)
    (if (<= (`self.Health`) 0.0)
      (bind _returnvalue (`|CreateWidget` "/Game/Chrono_Panic/UserInterface/WB_GameOverScreen_ChronoPanic.WB_GameOverScreen_ChronoPanic_C"))
      (`UserWidget.AddToViewport` _returnvalue 2)
      (`self.GameOverInput`)
      (`/Game/Chrono_Panic/UserInterface/WB_GameOverScreen_ChronoPanic.UpdateText` _returnvalue false))))

(event `PlayerHeal`
  ; Player Damage (Take away one life)
  (set `self.Health` (`KismetMathLibrary.FClamp` (+ (`self.Health`) (`self.MedkitHealAmount`)) 0.0 100.0))
  (`GameplayStatics.PlaySound2D` "/Game/Chrono_Panic/Audio/HealthPickup.HealthPickup" 1.0 1.0 0.0 null null)
  (goto _label_16))

(event `ReachedCheckpoint`
  ; Player Control
  (set `self.CheckpointTriggered` true)
  (set `PlayerController.bShowMouseCursor` false (`self.ControllerRef`))
  (set `self.isMoving` false)
  (set `self.CanShoot` true)
  (bind _output_get (set `self.CurentCheckpoint` (+ (`self.CurentCheckpoint`) 1)))
  (`/Game/Chrono_Panic/Blueprints/BP_CP_PlayerSpline.ScanEnemys` (`self.MovementSpline`))
  (if (== _output_get 1)
    (`self.Enable Player Shooting`)))

(fn `CameraRotationAlongSpline`
  (params (`NearCheckpoint?` :type Boolean))
  (bind _returnvalue (`self.K2_GetActorRotation`))
  (bind _returnvalue_2 (`GameplayStatics.GetWorldDeltaSeconds`))
  (if `NearCheckpoint?`
    (`self.K2_SetActorRotation` (`KismetMathLibrary.RInterpTo` _returnvalue (`SceneComponent.K2_GetComponentRotation` (`|GetArrayItem` (`/Game/Chrono_Panic/Blueprints/BP_CP_PlayerSpline.CheckpointArrows` (`self.MovementSpline`)) (`self.CurentCheckpoint`))) _returnvalue_2 3.0))
    (else
      (`self.K2_SetActorRotation` (`KismetMathLibrary.RInterpTo` _returnvalue (.rotation (`SplineComponent.GetTransformAtDistanceAlongSpline` (`/Game/Chrono_Panic/Blueprints/BP_CP_PlayerSpline.Spline` (`self.MovementSpline`)) (`self.CurrentDistance`) "World" false)) _returnvalue_2 3.0)))))

(fn `UserConstructionScript`)