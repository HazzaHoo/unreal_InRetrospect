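; Rifle enemy for Chrono Panic that optionally runs to a preset position, then fires at the player, crouching at random intervals.
; Looping timers spawn bullets with randomized spread and trace player visibility; difficulty sets accuracy and reload time.
; Damage updates a player-facing health bar; death swaps in physics body and rifle props, sometimes dropping a medkit.
; IsDumb makes it a passive one-health target; material and voice are randomized.
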(event `Damage`
  (params (BulletDamage :type "Float (double-precision)") (PlayerRef :type "/Game/Chrono_Panic/Blueprints/BP_CP_Player Object Reference"))
  (bind _output_get (set `self.Health` (- (`self.Health`) BulletDamage)))
  (bind _aswb_enemy_health_bar (cast `/Game/Chrono_Panic/UserInterface/WB_EnemyHealthBar` (`WidgetComponent.GetWidget` (`self.Widget`))))
  (`/Game/Chrono_Panic/UserInterface/WB_EnemyHealthBar.UpdateHealth` _aswb_enemy_health_bar _output_get)
  (if (<= _output_get 0.0)
    (`self.Kill`)
    (`/Game/Chrono_Panic/Blueprints/BP_CP_Player.EnemyKilled` PlayerRef)))

(event `self.ReceiveTick`
  (params (DeltaSeconds :type "Float (single-precision)"))
  (if (not (`self.IsDumb?`))
    (`self.RotateHealthBartoPlayer`)
    (`self.RotateEnemyToPlayer`)))

(event `Kill`
  ;[0.15 0.15 0.15 0.5 42] Kill event
  (`/Engine/EditorBlueprintResources/StandardMacros.DoOnce` false
    (:`Completed`
      (`GameplayStatics.SpawnSoundAtLocation` (`self.DeathSound`) (`self.K2_GetActorLocation`) (struct) 1.0 1.0 0.0 null null)
      (bind _returnvalue (`|SpawnActorFromClass` "/Script/Engine.SkeletalMeshActor" (`SceneComponent.K2_GetComponentToWorld` (`self.Mesh`)) "AlwaysSpawn" "MultiplyWithRoot" null null))
      (`PrimitiveComponent.SetMaterial` (`SkeletalMeshActor.SkeletalMeshComponent` _returnvalue) 0 (`PrimitiveComponent.GetMaterial` (`self.Mesh`) 0))
      (`SkeletalMeshComponent.SetSkeletalMeshAsset` (`SkeletalMeshActor.SkeletalMeshComponent` _returnvalue) "/Game/Chrono_Panic/Assets/Enemies/Basic_Enemy/CP_BasicEnemy_T-Pose.CP_BasicEnemy_T-Pose")
      (bind _skeletalmeshcomponent (`SkeletalMeshActor.SkeletalMeshComponent` _returnvalue))
      (`SkeletalMeshComponent.SetAnimationMode` _skeletalmeshcomponent "AnimationSingleNode" true)
      (`SkeletalMeshComponent.SetAnimation` _skeletalmeshcomponent "/Game/Chrono_Panic/Assets/Enemies/Basic_Enemy/CP_BasicEnemy_Rifle_Idle.CP_BasicEnemy_Rifle_Idle")
      (`PrimitiveComponent.SetSimulatePhysics` _skeletalmeshcomponent true)
      (bind _returnvalue_2 (`|SpawnActorFromClass` "/Script/Engine.StaticMeshActor" (`SceneComponent.K2_GetComponentToWorld` (`self.SM_Rifle`)) "AlwaysSpawn" "MultiplyWithRoot" null null))
      (`SceneComponent.SetMobility` (`StaticMeshActor.StaticMeshComponent` _returnvalue_2) "Movable")
      (`StaticMeshComponent.SetStaticMesh` (`StaticMeshActor.StaticMeshComponent` _returnvalue_2) "/Game/Chrono_Panic/TempFolder/Weapons/Meshes/Rifle/SM_Rifle.SM_Rifle")
      (`PrimitiveComponent.SetSimulatePhysics` (`StaticMeshActor.StaticMeshComponent` _returnvalue_2) true)
      (if (== (`KismetMathLibrary.RandomIntegerInRange` 0 5) 0)
        (if (not (`self.DontSpawnMedkit`))
          (`|SpawnActorFromClass` "/Game/Chrono_Panic/Blueprints/BP_Medkit.BP_Medkit_C" (`KismetMathLibrary.MakeTransform` (`self.K2_GetActorLocation`)) "Undefined" "MultiplyWithRoot" null null)))
      (`self.K2_DestroyActor`))))

(event `Set Material`
  (bind _mesh (`self.Mesh`))
  (switch `int` (`KismetMathLibrary.RandomIntegerInRange` 0 1)
    (:`0`
      (`PrimitiveComponent.SetMaterial` _mesh 0 "/Game/Chrono_Panic/Assets/Material/M_BasicEnemy_01.M_BasicEnemy_01"))
    (:`1`
      (`PrimitiveComponent.SetMaterial` _mesh 0 "/Game/Chrono_Panic/Assets/Material/M_BasicEnemy_02.M_BasicEnemy_02"))))

(event `EnableCrouching`
  (bind (_x _y) (`KismetMathLibrary.BreakVector2D` (`self.CrouchRrandomRange`)))
  ;[0.15 0 0.01237 0.5 42] Beginplay
  ;;[0 0.06851 0.15 0.5 42] Crouch/Uncrouch Loop
  (if (`self.CanCrouch?`)
    (`KismetSystemLibrary.Delay` (`KismetMathLibrary.RandomFloatInRange` _x _y) :!label _label)
    (`/Engine/EditorBlueprintResources/StandardMacros.FlipFlop`
      (:`A`
        (`self.SetState` true :!label _label_2)
        (goto _label))
      (:`B`
        (`self.SetState` false)
        (goto _label)))))

(event `self.ReceiveBeginPlay`
  (`self.ChooseVoice`)
  (`self.Set Material`)
  ;[0.15 0 0.01237 0.5 42] Beginplay
  (if (`self.IsDumb?`)
    (set `self.Health` 1.0)
    (else
      (`self.Set Difficulty`)
      (`self.SetMovePositions`)
      (bind _returnvalue (`GameplayStatics.GetActorOfClass` "/Game/Chrono_Panic/Blueprints/BP_CP_Player.BP_CP_Player_C"))
      (set `self.Player Ref` _returnvalue)
      (bind _asabp_manny_ranged (cast `/Game/Chrono_Panic/TempFolder/Characters/Mannequins/Animations/ABP_Manny_Ranged` (`SkeletalMeshComponent.GetAnimInstance` (`self.Mesh`)))
        (:`then`
          (set `self.AnimBP` _asabp_manny_ranged))
        (:`CastFailed`
          _))
      (`KismetSystemLibrary.K2_SetTimer` null "PlayerVisibilityCheck" 0.5 true)
      (if (`self.StartCrouched?`)
        (goto _label_2)))))

(event `StopShooting`
  ;[0 0.15 0.1417 0.5 42] Stop shooting
  (`KismetSystemLibrary.K2_ClearAndInvalidateTimerHandle` (`self.TimerHandle`)))

(event `StartShooting`
  (if (`self.IsDumb?`)
    _
    (elif (`self.isDead?`)
      (`self.StopShooting`)
      (elif (not (`KismetSystemLibrary.K2_IsValidTimerHandle` (`self.TimerHandle`)))
        (bind _returnvalue (`KismetSystemLibrary.K2_SetTimerDelegate` (delegate `SpawnBullet`) (`KismetMathLibrary.RandomFloatInRange` 0.3 0.7) true))
        (set `self.TimerHandle` _returnvalue)))))

(event `Reload`
  (`/Engine/EditorBlueprintResources/StandardMacros.DoOnce` false
    (:`Completed`
      (`GameplayStatics.SpawnSoundAtLocation` (`self.ReloadSound`) (`self.K2_GetActorLocation`) (struct) 1.0 1.0 0.0 null null)
      (`GameplayStatics.SpawnSoundAtLocation` "/Game/Chrono_Panic/Audio/EnemyStartReload_Cue.EnemyStartReload_Cue" (`self.K2_GetActorLocation`) (struct) 1.0 1.0 0.0 null null)
      (set `self.IsReloading?` true)
      (`KismetSystemLibrary.Delay` (`self.Enemy Time to Reload`))
      (set `self.IsReloading?` false)
      (set `self.EnemyAmmoCount` (`self.MaxEnemyAmmoCount`))
      (`GameplayStatics.SpawnSoundAtLocation` "/Game/Chrono_Panic/Audio/EnemyEndReload_Cue.EnemyEndReload_Cue" (`self.K2_GetActorLocation`) (struct) 1.0 1.0 0.0 null null))))

(event `SpawnBullet`
  (bind _enemyammocount (`self.EnemyAmmoCount`))
  (bind _returnvalue_location (`KismetMathLibrary.BreakTransform` (`SceneComponent.K2_GetComponentToWorld` (`self.BulletStartPoint`))))
  (bind _returnvalue (`KismetMathLibrary.RandomFloatInRange` 0.0 (`KismetMathLibrary.MapRangeClamped` (`self.Accuracy`) 0.0 100.0 0.0 25.0)))
  ;[0.15 0 0.1107 0.5 42] Start shooting
  (if (`self.Crouched`)
    (`self.StopShooting`)
    (set `self.Shooting` false)
    (elif (<= _enemyammocount 0)
      (`self.Reload`)
      (else
        (`/Engine/EditorBlueprintResources/StandardMacros.DecrementInt` _enemyammocount
          (:`  `
            (bind _returnvalue_2 (`GameplayStatics.SpawnSoundAtLocation` "/Game/Chrono_Panic/Audio/EnemyGunShot_Cue.EnemyGunShot_Cue" (`self.K2_GetActorLocation`) (struct) 1.0 1.0 0.0 null null))
            (`AudioComponent.SetPitchMultiplier` _returnvalue_2 (`KismetMathLibrary.RandomFloatInRange` 0.75 1.25))
            (`|SpawnActorFromClass` "/Game/Chrono_Panic/Blueprints/BP_Bullets.BP_Bullets_C" (`KismetMathLibrary.MakeTransform` _returnvalue_location (`KismetMathLibrary.ComposeRotators` (`KismetMathLibrary.FindLookAtRotation` (`SceneComponent.K2_GetComponentLocation` (`self.BulletStartPoint`)) (`SceneComponent.K2_GetComponentLocation` (`/Game/Chrono_Panic/Blueprints/BP_CP_Player.PlayerHead` (`self.TargetPlayer`)))) (`KismetMathLibrary.MakeRotator` _returnvalue _returnvalue _returnvalue))) "Undefined" "MultiplyWithRoot" self null)
            (set `self.Shooting` true)))))))

(event `SetMovePositions`
  (if (not (`self.IsDumb?`))
    ; Get Positions to Move
    (set `self.MovePos_01` (`KismetMathLibrary.MakeVector` (.x (`SceneComponent.K2_GetComponentLocation` (`self.Pos_01`))) (.y (`SceneComponent.K2_GetComponentLocation` (`self.Pos_01`))) (.z (`SceneComponent.K2_GetComponentLocation` (`self.Pos_01`)))))
    (set `self.MovePos_02` (`KismetMathLibrary.MakeVector` (.x (`SceneComponent.K2_GetComponentLocation` (`self.Pos_02`))) (.y (`SceneComponent.K2_GetComponentLocation` (`self.Pos_02`))) (.z (`SceneComponent.K2_GetComponentLocation` (`self.Pos_02`)))))
    (`SceneComponent.K2_SetWorldLocation` (`self.CapsuleComponent`) (`self.MovePos_01`) false false)))

(event `ActivateEnemy`
  ; Move to Pos_02 when activate
  (if (`self.MakeRun`)
    (bind (_direction _lerp) (`Timeline|T_Running` :!via `PlayFromStart`)
      (:`Update`
        (`SceneComponent.K2_SetWorldLocationAndRotation` (`self.CapsuleComponent`) (`KismetMathLibrary.VLerp` (`self.MovePos_01`) (`self.MovePos_02`) _lerp) (`KismetMathLibrary.MakeRotator` (.roll (`KismetMathLibrary.FindLookAtRotation` (`SceneComponent.K2_GetComponentLocation` (`self.CapsuleComponent`)) (`self.MovePos_02`))) (.pitch (`KismetMathLibrary.FindLookAtRotation` (`SceneComponent.K2_GetComponentLocation` (`self.CapsuleComponent`)) (`self.MovePos_02`))) (.yaw (`KismetMathLibrary.FindLookAtRotation` (`SceneComponent.K2_GetComponentLocation` (`self.CapsuleComponent`)) (`self.MovePos_02`)))) false false)
        (set `self.Movement` true))
      (:`Finished`
        (set `self.Movement` false :!label _label_3)
        (`self.EnableCrouching`)
        (set `self.Crouched` false)
        ;[0 0.1257 0.15 0.5 42] Activate enemy
        (set `self.IsActive` true)
        (bind _asbp_cp_player (cast `/Game/Chrono_Panic/Blueprints/BP_CP_Player` (`GameplayStatics.GetPlayerPawn` 0))
          (:`then`
            (set `self.TargetPlayer` _asbp_cp_player)
            (if (`self.CanCrouch?`)
              (if (`self.Crouched`)
                (`self.StopShooting`)
                (else
                  ;;[0 0.07319 0.15 0.5 42] If its the first time seeing the player - Wait 2 seconds.
                  (if (`self.firstTimeSeen`) :!label _label_4
                    (`/Engine/EditorBlueprintResources/StandardMacros.DoOnce` false
                      (:`Completed`
                        (set `self.firstTimeSeen` false))))
                  (`self.StartShooting`)))
              (else
                (goto _label_4))))
          (:`CastFailed`
            (`self.StopShooting`)))))
    (else
      (goto _label_3))))

(event `PlayerVisibilityCheck`
  ;[0.15 0.05391 0.05391 0.5 42] Player visibility check
  (if (`self.isDead?`)
    _
    (elif (`self.IsActive`)
      (bind (_outhit _returnvalue) (`KismetSystemLibrary.LineTraceSingle` (`SceneComponent.K2_GetComponentLocation` (`self.BulletStartPoint`)) (`SceneComponent.K2_GetComponentLocation` (`/Game/Chrono_Panic/Blueprints/BP_CP_Player.PlayerHead` (`self.TargetPlayer`))) "TraceTypeQuery1"))
      (if _returnvalue
        (bind (_bblockinghit _binitialoverlap _time _distance _location _impactpoint _normal _impactnormal _physmat _hitactor _hitcomponent) (`GameplayStatics.BreakHitResult` _outhit))
        (bind _asbp_cp_player (cast `/Game/Chrono_Panic/Blueprints/BP_CP_Player` _hitactor))
        (set `self.canSeePlayer` (== (`/Game/Chrono_Panic/Blueprints/BP_CP_Player.PlayerHitBox` _asbp_cp_player) _hitcomponent))))))

(fn `ChooseVoice`
  (switch `int` (`KismetMathLibrary.RandomIntegerInRange` 0 3)
    (:`0`
      (set `self.DeathSound` "/Game/Chrono_Panic/Audio/Enemies/Harry/HarryDeath_Cue.HarryDeath_Cue")
      (set `self.ReloadSound` "/Game/Chrono_Panic/Audio/Enemies/Harry/HarryReload_Cue.HarryReload_Cue"))
    (:`1`
      (set `self.DeathSound` "/Game/Chrono_Panic/Audio/Enemies/Josh/JoshDeath_01_Cue.JoshDeath_01_Cue")
      (set `self.ReloadSound` "/Game/Chrono_Panic/Audio/Enemies/Josh/JoshReload_01_Cue.JoshReload_01_Cue"))
    (:`2`
      (set `self.DeathSound` "/Game/Chrono_Panic/Audio/Enemies/Elliot/ElliotDeath_01_Cue.ElliotDeath_01_Cue")
      (set `self.ReloadSound` "/Game/Chrono_Panic/Audio/Enemies/Elliot/ElliotReload_01_Cue.ElliotReload_01_Cue"))
    (:`3`
      (set `self.DeathSound` null)
      (set `self.ReloadSound` "/Game/Chrono_Panic/Audio/Enemies/Jack/JackReload_01_Cue.JackReload_01_Cue"))))

(fn `RotateEnemyToPlayer`
  (if (not (`self.Movement`))
    (`SceneComponent.K2_SetWorldRotation` (`self.Mesh`) (`KismetMathLibrary.MakeRotator` 0.0 0.0 (- (.yaw (`KismetMathLibrary.FindLookAtRotation` (`self.K2_GetActorLocation`) (`self.K2_GetActorLocation` (`self.Player Ref`)))) 90.0)) false false)))

(fn `RotateHealthBartoPlayer`
  (bind _widget (`self.Widget`))
  (`SceneComponent.K2_SetWorldRotation` _widget (`KismetMathLibrary.FindLookAtRotation` (`SceneComponent.K2_GetComponentLocation` _widget) (`self.K2_GetActorLocation` (`self.Player Ref`))) false false))

(fn `Set Difficulty`
  (bind _asglobal_instance (cast `/Game/Global_IMC/Global_Instance` (`GameplayStatics.GetGameInstance`)))
  (switch `/Game/Ping/Blueprints/E_Difficulty` (`/Game/Global_IMC/Global_Instance.SelectedDifficulty` _asglobal_instance)
    (:`NewEnumerator0`
      (set `self.Enemy Time to Reload` 5.0)
      (set `self.Accuracy` 80.0))
    (:`NewEnumerator1`
      (set `self.Enemy Time to Reload` 3.5)
      (set `self.Accuracy` 50.0))
    (:`NewEnumerator2`
      (set `self.Enemy Time to Reload` 2.5)
      (set `self.Accuracy` 25.0))))

(fn `SetState`
  (params (Crouched :type Boolean))
  (if (`self.isDead?`)
    (`self.StopShooting`)
    (elif Crouched
      (set `self.Crouched` true)
      (`self.StopShooting`)
      (else
        (set `self.Crouched` false)
        (if (`self.IsActive`)
          (`self.StartShooting`))))))

(fn `UserConstructionScript`)