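; BP_CP_WayPointManager manages the waypoints that the Chrono Panic player is teleported between.
; On BeginPlay it gathers every BP_CP_WayPoint, rebuilds an array ordered by each waypoint's Index whenever its max-index check passes, then snaps the player to the first entry.
; MoveToIndex bounds-checks a requested index, moves the player to that waypoint's location and rotation, and records it as CurrentIndex.
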(event `self.ReceiveBeginPlay`
  (bind _output (`|GetArrayItem` (`self.OrderedWaypoints`)))
  (bind _asbp_cp_player (cast `/Game/Chrono_Panic/Blueprints/BP_CP_Player` (`GameplayStatics.GetPlayerPawn` 0)))
  (set `self.PlayerRef` _asbp_cp_player)
  (bind _outactors (`GameplayStatics.GetAllActorsOfClass` "/Game/Chrono_Panic/Blueprints/BP_CP_WayPoint.BP_CP_WayPoint_C"))
  (bind _output_get (set `self.FoundWayPoints` _outactors))
  (for (_array_element _array_index) _output_get
    (if (> (`/Game/Chrono_Panic/Blueprints/BP_CP_WayPoint.Index` _array_element) (`self.MaxIndex`))
      (set `self.MaxIndex` _array_index)
      (`KismetArrayLibrary.Array_Clear` (`self.OrderedWaypoints`))
      (`KismetArrayLibrary.Array_Resize` (`self.OrderedWaypoints`) (+ (`self.MaxIndex`) 1))
      (for _array_element_2 (`self.FoundWayPoints`)
        (`KismetArrayLibrary.Array_Set` (`self.OrderedWaypoints`) (`/Game/Chrono_Panic/Blueprints/BP_CP_WayPoint.Index` _array_element_2) _array_element_2 true))
      (`self.K2_SetActorLocationAndRotation` (`self.PlayerRef`) (`self.K2_GetActorLocation` _output) (`self.K2_GetActorRotation` _output) false false)
      (set `self.CurrentIndex` 0))))

(fn `MoveToIndex`
  (params (NewIndex :type Integer))
  (bind _output (`|GetArrayItem` (`self.OrderedWaypoints`) NewIndex))
  (if (< NewIndex 0)
    _
    (elif (not (>= NewIndex (`KismetArrayLibrary.Array_Length` (`self.OrderedWaypoints`))))
      (`self.K2_SetActorLocationAndRotation` (`self.PlayerRef`) (`self.K2_GetActorLocation` _output) (`self.K2_GetActorRotation` _output) false false)
      (set `self.CurrentIndex` NewIndex))))

(fn `UserConstructionScript`)