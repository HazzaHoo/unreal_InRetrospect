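; BP_CP_Progression_Portal is the Chrono Panic end-of-level portal that returns the game to L_Modern_Arcade.
; On BeginPlay it stops the HUD timer and animates its placeholder render with rotation and position timelines.
; EndLevel plays sounds, fades music, then loads out to the arcade if the game is finished.
; Otherwise it records a shots-fired secret in the game instance and existing settings save, and shows an era transition widget.
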(event `self.ReceiveBeginPlay`
  (bind _placeholder_portalrender (`self.PlaceHolder_PortalRender`))
  (`KismetSystemLibrary.Delay` 0.2)
  (bind _foundwidgets (`WidgetBlueprintLibrary.GetAllWidgetsOfClass` "/Game/Chrono_Panic/UserInterface/WB_In-GameHUD_ChronoPanic.WB_In-GameHUD_ChronoPanic_C"))
  (set `/Game/Chrono_Panic/UserInterface/WB_In-GameHUD_ChronoPanic.StopTimer?` true (`|GetArrayItem` _foundwidgets))
  ; Animation
  (`|ExecutionSequence`
    (:`then_0`
      (bind (_direction _lerp) (`Timeline|Timeline_0`)
        (:`Update`
          (`SceneComponent.K2_SetRelativeRotation` _placeholder_portalrender (`KismetMathLibrary.RLerp` (struct :`Pitch` -74.0) (struct :`Pitch` -74.0 :`Yaw` 360.0) _lerp) false false))))
    (:`then_1`
      (bind (_direction_2 _lerp_2) (`Timeline|Timeline`)
        (:`Update`
          (`SceneComponent.K2_SetRelativeLocation` _placeholder_portalrender (`KismetMathLibrary.VLerp` (0.0 0.0 0.0) (0.0 0.0 50.0) _lerp_2) false false))))))

(event `EndLevel`
  (`GameplayStatics.PlaySound2D` "/Game/Global_Audio/New_Era.New_Era" 3.0 1.0 0.0 null null)
  (`GameplayStatics.PlaySound2D` "/Game/Crash_Capybara/Audio/CC_KeyPickup.CC_KeyPickup" 1.0 1.0 0.0 null null)
  (bind _returnvalue (`GameplayStatics.GetActorOfClass` "/Game/Chrono_Panic/Blueprints/BP_CP_Player.BP_CP_Player_C"))
  (`/Game/Chrono_Panic/Blueprints/BP_CP_Player.FadeMusicOut` _returnvalue 1.0)
  (`WidgetBlueprintLibrary.SetInputMode_GameOnly` (`GameplayStatics.GetPlayerController` 0))
  (bind _asglobal_instance (cast `/Game/Global_IMC/Global_Instance` (`GameplayStatics.GetGameInstance`)))
  (if (`/Game/Global_IMC/Global_Instance.IsGameFinished?` _asglobal_instance)
    (bind _returnvalue_2 (`|CreateWidget` "/Game/Global_Userinterface/WB_LoadInOrOut.WB_LoadInOrOut_C"))
    (`/Game/Global_Userinterface/WB_LoadInOrOut.Load Out` _returnvalue_2)
    (`UserWidget.AddToViewport` _returnvalue_2 0)
    (`KismetSystemLibrary.Delay` 0.5)
    (`GameplayStatics.OpenLevel` "L_Modern_Arcade")
    (elif (> (`/Game/Chrono_Panic/Blueprints/BP_CP_Player.ShotsFired` _returnvalue) (`self.ShotsFiredForSecret`))
      (set `/Game/Global_IMC/Global_Instance.ChronoShotsFired` true _asglobal_instance)
      (bind _returnvalue_3 (`GameplayStatics.DoesSaveGameExist` "settings"))
      (if _returnvalue_3
        (bind _returnvalue_4 (`GameplayStatics.LoadGameFromSlot` "settings"))
        (bind _assettings_save_game (cast `/Game/SettingsSaveGame` _returnvalue_4))
        (set `/Game/SettingsSaveGame.ChronoShots` true _assettings_save_game)
        (`GameplayStatics.SaveGameToSlot` _assettings_save_game "settings")
        (bind _returnvalue_5 (`|CreateWidget` "/Game/Global_Userinterface/WB_TransitionFirst.WB_TransitionFirst_C" :!label _label))
        (`/Game/Global_Userinterface/WB_TransitionFirst.WhatEra?` _returnvalue_5 "" "" "" "L_Modern_Arcade" true)
        (`UserWidget.AddToViewport` _returnvalue_5 0))
      (else
        (goto _label)))))

(fn `UserConstructionScript`)