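; BP_CP_PlayerSpline defines the player's spline path in Chrono Panic and manages enemy encounters at checkpoints along it.
; On BeginPlay it converts eleven arrow markers into distances along the spline.
; ScanEnemys activates and tracks enemies matching the current checkpoint, advances the index, and starts the boss shooting after a delay if none match.
; EnemyKilled counts down the tracked enemies and resumes player movement when all are dead.
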(event `self.ReceiveBeginPlay`
  (bind _spline (`self.Spline`))
  (bind _asbp_cp_player (cast `/Game/Chrono_Panic/Blueprints/BP_CP_Player` (`GameplayStatics.GetPlayerPawn` 0)))
  (set `self.PlayerRef` _asbp_cp_player)
  (bind _output_get (set `self.CheckpointArrows` (`|MakeArray` (`self.Arrow1`) (`self.Arrow2`) (`self.Arrow3`) (`self.Arrow4`) (`self.Arrow5`) (`self.Arrow6`) (`self.Arrow7`) (`self.Arrow8`) (`self.Arrow9`) (`self.Arrow10`) (`self.Arrow11`))))
  (for _array_element _output_get
    (`KismetArrayLibrary.Array_Add` (`self.CheckpointDistances`) (`SplineComponent.GetDistanceAlongSplineAtSplineInputKey` _spline (`SplineComponent.FindInputKeyClosestToWorldLocation` _spline (`SceneComponent.K2_GetComponentLocation` _array_element))))))

(event `ScanEnemys`
  (`KismetArrayLibrary.Array_Clear` (`self.CurrentCheckpointEnemys`))
  (bind _outactors (`GameplayStatics.GetAllActorsOfClass` "/Game/Chrono_Panic/Blueprints/BP_CP_Enemy2.BP_CP_Enemy2_C"))
  (for _array_element _outactors
    (if (== (`/Game/Chrono_Panic/Blueprints/BP_CP_Enemy2.CheckPointIndex` _array_element) (`self.CurrentCheckpoint`))
      (`/Game/Chrono_Panic/Blueprints/BP_CP_Enemy2.ActivateEnemy` _array_element)
      (`KismetArrayLibrary.Array_Add` (`self.CurrentCheckpointEnemys`) _array_element)
      (`KismetSystemLibrary.PrintString` (`KismetSystemLibrary.GetDisplayName` _array_element) true true (struct :`R` 0.193832 :`G` 1.0 :`A` 1.0) 12.0)))
  (set `self.EnemysRemaining` (`KismetArrayLibrary.Array_Length` (`self.CurrentCheckpointEnemys`)))
  (set `self.CurrentCheckpoint` (+ (`self.CurrentCheckpoint`) 1))
  (if (== (`KismetArrayLibrary.Array_Length` (`self.CurrentCheckpointEnemys`)) 0)
    (bind _returnvalue (`GameplayStatics.GetActorOfClass` "/Game/Chrono_Panic/Blueprints/BP_CC_Boss.BP_CC_Boss_C"))
    (`KismetSystemLibrary.Delay` 2.0)
    (`/Game/Chrono_Panic/Blueprints/BP_CC_Boss.StartShooting` _returnvalue)))

(event `EnemyKilled`
  (params (EnemyRef :type "/Game/Chrono_Panic/Blueprints/BP_CP_Enemy2 Object Reference"))
  (if (`KismetArrayLibrary.Array_Contains` (`self.CurrentCheckpointEnemys`) EnemyRef)
    (set `self.EnemysRemaining` (- (`self.EnemysRemaining`) 1))
    (if (<= (`self.EnemysRemaining`) 0)
      (set `/Game/Chrono_Panic/Blueprints/BP_CP_Player.isMoving` true (`self.PlayerRef`)))))

(fn `UserConstructionScript`)