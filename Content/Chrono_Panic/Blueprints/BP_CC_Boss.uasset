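; Chrono Panic boss enemy that shoots at the player and spawns a progression portal when killed.
; On activation it optionally runs between two points via a Timeline, then a looping timer fires bullets at the player's head with random spread, pausing to reload.
; Game instance difficulty sets reload time and accuracy.
; Hits update a player-facing health bar; death swaps the actor for physics-simulated body and rifle props.
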(event `Kill`
  (bind (_returnvalue_x _returnvalue_y _returnvalue_z) (`KismetMathLibrary.BreakVector` (`self.K2_GetActorLocation`)))
  ;[0.15 0.15 0.15 0.5 42] Kill Event
  (bind _returnvalue (`|SpawnActorFromClass` "/Script/Engine.SkeletalMeshActor" (`SceneComponent.K2_GetComponentToWorld` (`self.BossMesh`)) "AlwaysSpawn" "MultiplyWithRoot" null null))
  (`SkeletalMeshComponent.SetSkeletalMeshAsset` (`SkeletalMeshActor.SkeletalMeshComponent` _returnvalue) "/Game/Chrono_Panic/Assets/Enemies/Heavy_Enemy/CP_HeavyEnemy_T-Pose.CP_HeavyEnemy_T-Pose")
  (bind _skeletalmeshcomponent (`SkeletalMeshActor.SkeletalMeshComponent` _returnvalue))
  (`SkeletalMeshComponent.SetAnimationMode` _skeletalmeshcomponent "AnimationSingleNode" false)
  (`SkeletalMeshComponent.SetAnimation` _skeletalmeshcomponent "/Game/Chrono_Panic/Assets/Enemies/Basic_Enemy/CP_BasicEnemy_Rifle_Idle.CP_BasicEnemy_Rifle_Idle")
  (`PrimitiveComponent.SetSimulatePhysics` _skeletalmeshcomponent true)
  (bind _returnvalue_2 (`|SpawnActorFromClass` "/Script/Engine.StaticMeshActor" (`SceneComponent.K2_GetComponentToWorld` (`self.SM_Rifle`)) "AlwaysSpawn" "MultiplyWithRoot" null null))
  (`SceneComponent.SetMobility` (`StaticMeshActor.StaticMeshComponent` _returnvalue_2) "Movable")
  (`StaticMeshComponent.SetStaticMesh` (`StaticMeshActor.StaticMeshComponent` _returnvalue_2) "/Game/Chrono_Panic/TempFolder/Weapons/Meshes/Rifle/SM_Rifle.SM_Rifle")
  (`PrimitiveComponent.SetSimulatePhysics` (`StaticMeshActor.StaticMeshComponent` _returnvalue_2) true)
  (`|SpawnActorFromClass` "/Game/Chrono_Panic/Blueprints/BP_CP_Progression_Portal.BP_CP_Progression_Portal_C" (`KismetMathLibrary.MakeTransform` (`KismetMathLibrary.MakeVector` _returnvalue_x _returnvalue_y (+ _returnvalue_z 50.0))) "Undefined" "MultiplyWithRoot" null null)
  (`self.K2_DestroyActor`))

(event `SetMovePositions`
  ; Get Positions to Move
  (set `self.MovePos_01` (`KismetMathLibrary.MakeVector` (.x (`SceneComponent.K2_GetComponentLocation` (`self.Pos_01`))) (.y (`SceneComponent.K2_GetComponentLocation` (`self.Pos_01`))) (.z (`SceneComponent.K2_GetComponentLocation` (`self.BossMesh`)))))
  (set `self.MovePos_02` (`KismetMathLibrary.MakeVector` (.x (`SceneComponent.K2_GetComponentLocation` (`self.Pos_02`))) (.y (`SceneComponent.K2_GetComponentLocation` (`self.Pos_02`))) (.z (`SceneComponent.K2_GetComponentLocation` (`self.BossMesh`)))))
  (`SceneComponent.K2_SetWorldLocation` (`self.BossMesh`) (`self.MovePos_01`) false false))

(event `BossHit`
  ;[0.15 0.15 0.15 0.5 42] Hitpoints decrease
  (bind _output_get (set `self.Health` (- (`self.Health`) (`self.DamagePerShot(Player)`))))
  (bind _aswb_enemy_health_bar (cast `/Game/Chrono_Panic/UserInterface/WB_EnemyHealthBar` (`WidgetComponent.GetWidget` (`self.Widget`))))
  (`/Game/Chrono_Panic/UserInterface/WB_EnemyHealthBar.UpdateHealth` _aswb_enemy_health_bar _output_get)
  (if (<= _output_get 0.0)
    (`self.Kill`)))

(event `self.ReceiveBeginPlay`
  ;[0.15 0.15 0.15 0.5 42] Beginplay
  (`self.Set Difficulty`)
  (bind _asbp_cp_player (cast `/Game/Chrono_Panic/Blueprints/BP_CP_Player` (`GameplayStatics.GetPlayerPawn` 0))
    (:`then`
      (set `self.TargetPlayer` _asbp_cp_player))
    (:`CastFailed`
      _))
  (`self.SetMovePositions`))

(event `StartShooting`
  (if (not (`KismetSystemLibrary.K2_IsValidTimerHandle` (`self.TimerHandle`)))
    (bind _returnvalue (`KismetSystemLibrary.K2_SetTimerDelegate` (delegate `SpawnBullet`) (`self.ShootingInterval`) true))
    (set `self.TimerHandle` _returnvalue)))

(event `self.ReceiveTick`
  (params (DeltaSeconds :type "Float (single-precision)"))
  ;[0.15 0.15 0.15 0.5 42] Beginplay
  (`self.RotateHealthBartoPlayer`)
  (if (not (`self.Movement`))
    (`self.RotateEnemyToPlayer`)))

(event `ActivateEnemy`
  ; Move to Pos_02 when activate
  (if (`self.MakeRun`)
    (bind (_direction _lerp) (`Timeline|Timeline` :!via `PlayFromStart`)
      (:`Update`
        (`SceneComponent.K2_SetWorldLocationAndRotation` (`self.BossMesh`) (`KismetMathLibrary.VLerp` (`self.MovePos_01`) (`self.MovePos_02`) _lerp) (`KismetMathLibrary.MakeRotator` (.roll (`KismetMathLibrary.FindLookAtRotation` (`SceneComponent.K2_GetComponentLocation` (`self.BossMesh`)) (`self.MovePos_02`))) (.pitch (`KismetMathLibrary.FindLookAtRotation` (`SceneComponent.K2_GetComponentLocation` (`self.BossMesh`)) (`self.MovePos_02`))) (- (.yaw (`KismetMathLibrary.FindLookAtRotation` (`SceneComponent.K2_GetComponentLocation` (`self.BossMesh`)) (`self.MovePos_02`))) 90.0)) false false)
        (set `self.Movement` true))
      (:`Finished`
        (set `self.Movement` false :!label _label)
        (`self.StartShooting`)))
    (else
      (goto _label))))

(event `Reload`
  (`/Engine/EditorBlueprintResources/StandardMacros.DoOnce` false :!label _label_2
    (:`Completed`
      (set `self.IsReloading?` true)
      (`GameplayStatics.SpawnSoundAtLocation` "/Game/Chrono_Panic/Audio/EnemyStartReload_Cue.EnemyStartReload_Cue" (`self.K2_GetActorLocation`) (struct) 1.0 1.0 0.0 null null)
      (`KismetSystemLibrary.Delay` (`self.Enemy Time to Reload`))
      (`GameplayStatics.SpawnSoundAtLocation` "/Game/Chrono_Panic/Audio/EnemyEndReload_Cue.EnemyEndReload_Cue" (`self.K2_GetActorLocation`) (struct) 1.0 1.0 0.0 null null)
      (`KismetSystemLibrary.Delay` 0.3)
      (set `self.IsReloading?` false)
      (set `self.EnemyAmmoCount` (`self.MaxEnemyAmmoCount`))
      (goto _label_2 :!via `Reset`))))

(event `SpawnBullet`
  (bind _enemyammocount (`self.EnemyAmmoCount`))
  (bind _returnvalue_location (`KismetMathLibrary.BreakTransform` (`SceneComponent.K2_GetComponentToWorld` (`self.BulletStartPoint`))))
  (bind _returnvalue (`KismetMathLibrary.RandomFloatInRange` 0.0 (`KismetMathLibrary.MapRangeClamped` (`self.Accuracy`) 0.0 100.0 5.0)))
  ;[0.15 0 0.1107 0.5 36] Start shooting
  (if (<= _enemyammocount 0)
    (`self.Reload`)
    (set `self.Shooting` false :!label _label_3)
    (`/Engine/EditorBlueprintResources/StandardMacros.IsValid` (stale _returnvalue_2)
      (:`Is Valid`
        (`AudioComponent.Stop` (stale _returnvalue_2))
        (goto _label_4 :!via `Reset`))
      (:`Is Not Valid`
        (goto _label_4 :!via `Reset`)))
    (elif (`self.IsReloading?`)
      (goto _label_3)
      (else
        (`/Engine/EditorBlueprintResources/StandardMacros.DecrementInt` _enemyammocount
          (:`  `
            (`|ExecutionSequence`
              (:`then_0`
                (`/Engine/EditorBlueprintResources/StandardMacros.DoOnce` false :!label _label_4
                  (:`Completed`
                    (bind _returnvalue_2 (`GameplayStatics.SpawnSoundAtLocation` "/Game/Chrono_Panic/Audio/BossShoot.BossShoot" (`self.K2_GetActorLocation`) (struct) 1.0 1.0 0.0 null null)))))
              (:`then_1`
                (set `self.Shooting` true)
                (`|SpawnActorFromClass` "/Game/Chrono_Panic/Blueprints/BP_Bullets.BP_Bullets_C" (`KismetMathLibrary.MakeTransform` _returnvalue_location (`KismetMathLibrary.ComposeRotators` (`KismetMathLibrary.FindLookAtRotation` (`SceneComponent.K2_GetComponentLocation` (`self.BulletStartPoint`)) (`SceneComponent.K2_GetComponentLocation` (`/Game/Chrono_Panic/Blueprints/BP_CP_Player.PlayerHead` (`self.TargetPlayer`)))) (`KismetMathLibrary.MakeRotator` _returnvalue _returnvalue _returnvalue))) "AlwaysSpawn" "MultiplyWithRoot" null null)))))))))

(fn `RotateEnemyToPlayer`
  (bind _bossmesh (`self.BossMesh`))
  (bind _yaw (.yaw (`KismetMathLibrary.FindLookAtRotation` (`self.K2_GetActorLocation`) (`self.K2_GetActorLocation` (`self.TargetPlayer`)))))
  (if (`self.Movement`)
    _
    (elif (`self.Shooting`)
      (`SceneComponent.K2_SetWorldRotation` _bossmesh (`KismetMathLibrary.MakeRotator` 0.0 0.0 (- _yaw 50.0)) false false)
      (else
        (`SceneComponent.K2_SetWorldRotation` _bossmesh (`KismetMathLibrary.MakeRotator` 0.0 0.0 (- _yaw 90.0)) false false)))))

(fn `RotateHealthBartoPlayer`
  (bind _widget (`self.Widget`))
  (`SceneComponent.K2_SetWorldRotation` _widget (`KismetMathLibrary.FindLookAtRotation` (`SceneComponent.K2_GetComponentLocation` _widget) (`self.K2_GetActorLocation` (`self.TargetPlayer`))) false false))

(fn `Set Difficulty`
  (bind _asglobal_instance (cast `/Game/Global_IMC/Global_Instance` (`GameplayStatics.GetGameInstance`)))
  (switch `/Game/Ping/Blueprints/E_Difficulty` (`/Game/Global_IMC/Global_Instance.SelectedDifficulty` _asglobal_instance)
    (:`NewEnumerator0`
      (set `self.Enemy Time to Reload` 3.0)
      (set `self.Accuracy` 30.0))
    (:`NewEnumerator1`
      (set `self.Enemy Time to Reload` 2.0)
      (set `self.Accuracy` 20.0))
    (:`NewEnumerator2`
      (set `self.Enemy Time to Reload` 1.0)
      (set `self.Accuracy` 10.0))))

(fn `StopShooting`)

(fn `UserConstructionScript`)