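; Crab enemy for Crash Capybara that patrols between two locally defined points via looping AI Move To, with walk speed set by the game instance's difficulty.
; Touching its bottom hitbox kills it if the player is attacking; otherwise a box trace damages the nearest hit actor, with a cooldown.
; Falling onto its top hitbox bounces the player and kills it, as does any damage, disabling collision and playing sound and fizzle before destruction.
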(event `self.ReceiveBeginPlay`
  ;[0 0.05098 0.003697] Movements
  ;;[0 0.05098 0.003697] Location for movement
  (set `self.Point A` (`KismetMathLibrary.TransformLocation` (`self.GetTransform`) (`self.Point A`)))
  (set `self.Point B` (`KismetMathLibrary.TransformLocation` (`self.GetTransform`) (`self.Point B`)))
  (`self.Move To Point`)
  (`self.Get Difficulty`))

(event `Move To Point`
  ;[0 0.05098 0.003697] Movements
  ;;[0 0.05098 0.003697] Movements Input
  (if (not (`self.Dead?`))
    (`|AIMoveTo` self (`KismetMathLibrary.SelectVector` (`self.Point B`) (`self.Point A`) (`self.Is A to B`)) null
      (:`OnSuccess`
        (set `self.Is A to B` (not (`self.Is A to B`)))
        (`self.Move To Point`)))))

(event `self.Bottom Hitbox.OnComponentBeginOverlap`
  (params (OverlappedComponent :type "PrimitiveComponent Object Reference") (OtherActor :type "Actor Object Reference") (OtherComp :type "PrimitiveComponent Object Reference") (OtherBodyIndex :type Integer) (bFromSweep :type Boolean) (SweepResult :type "HitResult Structure (by ref)"))
  (bind _returnvalue (`SceneComponent.K2_GetComponentLocation` (`self.Bottom Hitbox`)))
  ;[0 0.05098 0.003697] Death
  (bind _asbp_cc_player_characher (cast `/Game/Crash_Capybara/Blueprints/BP_CC_PlayerCharacher` OtherActor))
  (if (`/Game/Crash_Capybara/Blueprints/BP_CC_PlayerCharacher.isAttacking(anim)` _asbp_cc_player_characher)
    (`self.On Stomped`)
    (else
      (bind _outhits (`KismetSystemLibrary.BoxTraceMulti` _returnvalue _returnvalue (`BoxComponent.GetScaledBoxExtent` (`self.Bottom Hitbox`)) (struct) "TraceTypeQuery1"))
      (for _array_element _outhits
        (bind (_bblockinghit _binitialoverlap _time _distance _location _impactpoint _normal _impactnormal _physmat _hitactor) (`GameplayStatics.BreakHitResult` _array_element))
        (`KismetArrayLibrary.Array_Add` (`self.Array of hit actors`) _hitactor)
        (`KismetArrayLibrary.Array_Add` (`self.Array of hit Distances`) (`KismetMathLibrary.Vector_Distance` (`SceneComponent.K2_GetComponentLocation` (`self.Bottom Hitbox`)) _location)))
      (`/Engine/EditorBlueprintResources/StandardMacros.DoOnce` false :!label _label
        (:`Completed`
          (`GameplayStatics.ApplyDamage` (`|GetArrayItem` (`self.Array of hit actors`) (`KismetMathLibrary.MinOfFloatArray` (`self.Array of hit Distances`))) 10.0 null null "/Script/Engine.DamageType")
          (`KismetArrayLibrary.Array_Clear` (`self.Array of hit actors`))
          (`KismetSystemLibrary.Delay` 3.0)
          (goto _label :!via `Reset`))))))

(event `self.Top Hitbox.OnComponentBeginOverlap`
  (params (OverlappedComponent :type "PrimitiveComponent Object Reference") (OtherActor :type "Actor Object Reference") (OtherComp :type "PrimitiveComponent Object Reference") (OtherBodyIndex :type Integer) (bFromSweep :type Boolean) (SweepResult :type "HitResult Structure (by ref)"))
  ;[0 0.05098 0.003697] Enemy stomped
  (bind _asbp_cc_player_characher (cast `/Game/Crash_Capybara/Blueprints/BP_CC_PlayerCharacher` OtherActor))
  (if (`self.Dead?`)
    _
    (elif (< (.z (`self.GetVelocity` _asbp_cc_player_characher)) 0.0)
      (`/Game/Crash_Capybara/Blueprints/BP_CC_PlayerCharacher.Bounce Off Enemy` _asbp_cc_player_characher)
      (`self.On Stomped` :!label _label_2))))

(event `self.ReceiveAnyDamage`
  (params (Damage :type "Float (single-precision)") (DamageType :type "DamageType Object Reference") (InstigatedBy :type "Controller Object Reference") (DamageCauser :type "Actor Object Reference"))
  (goto _label_2))

(event `On Stomped`
  ; On Stomped
  (`MovementComponent.StopMovementImmediately` (`self.CharacterMovement`))
  (set `self.Dead?` true)
  (`PrimitiveComponent.SetCollisionEnabled` (`self.Bottom Hitbox`) "NoCollision")
  (`PrimitiveComponent.SetCollisionEnabled` (`self.Top Hitbox`) "NoCollision")
  (`PrimitiveComponent.SetCollisionEnabled` (`self.BodyBox`) "NoCollision")
  (`AudioComponent.Play` (`self.CC_Crab_Cue`) 0.0)
  (`KismetSystemLibrary.Delay` 0.2)
  (`ActorComponent.Activate` (`self.CC_N_Fizzle`) false)
  (`SceneComponent.SetHiddenInGame` (`self.Mesh`) true false)
  (`KismetSystemLibrary.Delay` 1.5)
  (`self.K2_DestroyActor`))

(fn `Get Difficulty`
  (bind _charactermovement (`self.CharacterMovement`))
  (bind _asglobal_instance (cast `/Game/Global_IMC/Global_Instance` (`GameplayStatics.GetGameInstance`)))
  (switch `/Game/Ping/Blueprints/E_Difficulty` (`/Game/Global_IMC/Global_Instance.SelectedDifficulty` _asglobal_instance)
    (:`NewEnumerator0`
      (set `CharacterMovementComponent.MaxWalkSpeed` 100.0 _charactermovement))
    (:`NewEnumerator1`
      (set `CharacterMovementComponent.MaxWalkSpeed` 200.0 _charactermovement))
    (:`NewEnumerator2`
      (set `CharacterMovementComponent.MaxWalkSpeed` 3e+17 _charactermovement))))

(fn `UserConstructionScript`)