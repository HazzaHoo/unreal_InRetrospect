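; Turtle enemy for Crash Capybara that roams to random reachable points, with walk speed set by the game instance's difficulty.
; Top hitbox overlaps bounce the player and, like any damage taken, flip and halt the turtle first, then destroy it.
; Bottom hitbox overlaps destroy it if the player is spin-attacking; otherwise a box trace picks the nearest actor to damage, gated by a DoOnce cooldown.
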(event `self.ReceiveBeginPlay`
  ;[0 0.05098 0.003697] Movements
  (`self.MoveToRandomLocation`)
  (`self.Get Difficulty`))

(event `MoveToRandomLocation`
  ;[0 0.05098 0.003697] Movements
  ;;[0 0.05098 0.003697] Movements Input
  (if (not (`self.stopMovement`))
    (`|AIMoveTo` self (`NavigationSystemV1.K2_GetRandomReachablePointInRadius` (`self.K2_GetActorLocation`) (`KismetMathLibrary.RandomFloatInRange` (`self.minRoamRadius`) (`self.maxRoamRadius`)) null null) null
      (:`OnSuccess`
        _)
      (:`OnFail`
        _))
    (`KismetSystemLibrary.Delay` (`self.IdleDelay`))
    (`self.MoveToRandomLocation`)))

(event `self.Bottom Hitbox.OnComponentBeginOverlap`
  (params (OverlappedComponent :type "PrimitiveComponent Object Reference") (OtherActor :type "Actor Object Reference") (OtherComp :type "PrimitiveComponent Object Reference") (OtherBodyIndex :type Integer) (bFromSweep :type Boolean) (SweepResult :type "HitResult Structure (by ref)"))
  (bind _returnvalue (`SceneComponent.K2_GetComponentLocation` (`self.Bottom Hitbox`)))
  ;[0 0.05098 0.003697] Death
  (bind _asbp_cc_player_characher (cast `/Game/Crash_Capybara/Blueprints/BP_CC_PlayerCharacher` OtherActor))
  (if (`/Game/Crash_Capybara/Blueprints/BP_CC_PlayerCharacher.isAttacking(anim)` _asbp_cc_player_characher)
    (`self.OnSpinAttack`)
    (else
      (bind _outhits (`KismetSystemLibrary.BoxTraceMulti` _returnvalue _returnvalue (`BoxComponent.GetScaledBoxExtent` (`self.Bottom Hitbox`)) (struct) "TraceTypeQuery1"))
      (for _array_element _outhits
        (bind (_bblockinghit _binitialoverlap _time _distance _location _impactpoint _normal _impactnormal _physmat _hitactor) (`GameplayStatics.BreakHitResult` _array_element))
        (`KismetArrayLibrary.Array_Add` (`self.Array of hit actors`) _hitactor)
        (`KismetArrayLibrary.Array_Add` (`self.Array of hit Distances`) (`KismetMathLibrary.Vector_Distance` (`SceneComponent.K2_GetComponentLocation` (`self.Bottom Hitbox`)) _location)))
      (`/Engine/EditorBlueprintResources/StandardMacros.DoOnce` false :!label _label
        (:`Completed`
          (`GameplayStatics.ApplyDamage` (`|GetArrayItem` (`self.Array of hit actors`) (`KismetMathLibrary.MinOfFloatArray` (`self.Array of hit Distances`))) 10.0 null null "/Script/Engine.DamageType")
          (`KismetArrayLibrary.Array_Clear` (`self.Array of hit actors`))
          (`KismetSystemLibrary.Delay` 3.0)
          (goto _label :!via `Reset`))))))

(event `OnSpinAttack`
  ;[0 0.05098 0.003697] Stomp Logic
  ;;[0.15 0.1288 0 0.5] Stomped Second Time
  (`/Engine/EditorBlueprintResources/StandardMacros.DoOnce` false :!label _label_2
    (:`Completed`
      (`SceneComponent.SetHiddenInGame` (`self.Mesh`) true false)
      (`PrimitiveComponent.SetCollisionEnabled` (`self.Bottom Hitbox`) "NoCollision")
      (`PrimitiveComponent.SetCollisionEnabled` (`self.Top Hitbox`) "NoCollision")
      (`AudioComponent.Play` (`self.CC_Turtle_Cue`) 0.0)
      (`ActorComponent.Activate` (`self.CC_N_Fizzle`) false)
      (`KismetSystemLibrary.Delay` 1.0)
      (`self.K2_DestroyActor`))))

(event `On Stomped`
  ;[0 0.05098 0.003697] Stomp Logic
  (if (`self.itsFlipped`)
    (goto _label_2)
    (else
      ;;[0.15 0.05936 0.06085 0.5] First Time Stomped
      (`MovementComponent.StopMovementImmediately` (`self.CharacterMovement`))
      (set `self.stopMovement` true)
      (set `self.itsFlipped` true)
      (bind (_direction _alpha) (`Timeline|RotateTurtle` :!via `PlayFromStart`)
        (:`Update`
          (`SceneComponent.K2_SetRelativeRotation` (`self.Mesh`) (`KismetMathLibrary.MakeRotator` (`KismetMathLibrary.Lerp` 0.0 180.0 _alpha) 0.0 90.0) false false)
          (`PrimitiveComponent.SetCollisionEnabled` (`self.Bottom Hitbox`) "NoCollision"))))))

(event `self.Top Hitbox.OnComponentBeginOverlap`
  (params (OverlappedComponent :type "PrimitiveComponent Object Reference") (OtherActor :type "Actor Object Reference") (OtherComp :type "PrimitiveComponent Object Reference") (OtherBodyIndex :type Integer) (bFromSweep :type Boolean) (SweepResult :type "HitResult Structure (by ref)"))
  ;[0 0.05098 0.003697] Enemy stomped
  (bind _asbp_cc_player_characher (cast `/Game/Crash_Capybara/Blueprints/BP_CC_PlayerCharacher` OtherActor))
  (`/Game/Crash_Capybara/Blueprints/BP_CC_PlayerCharacher.Bounce Off Enemy` _asbp_cc_player_characher)
  (`self.On Stomped` :!label _label_3))

(event `self.ReceiveAnyDamage`
  (params (Damage :type "Float (single-precision)") (DamageType :type "DamageType Object Reference") (InstigatedBy :type "Controller Object Reference") (DamageCauser :type "Actor Object Reference"))
  ;[0 0.05098 0.003697] Enemy stomped
  (goto _label_3))

(fn `Get Difficulty`
  (bind _charactermovement (`self.CharacterMovement`))
  (bind _asglobal_instance (cast `/Game/Global_IMC/Global_Instance` (`GameplayStatics.GetGameInstance`)))
  (switch `/Game/Ping/Blueprints/E_Difficulty` (`/Game/Global_IMC/Global_Instance.SelectedDifficulty` _asglobal_instance)
    (:`NewEnumerator0`
      (set `CharacterMovementComponent.MaxWalkSpeed` 100.0 _charactermovement))
    (:`NewEnumerator1`
      (set `CharacterMovementComponent.MaxWalkSpeed` 200.0 _charactermovement))
    (:`NewEnumerator2`
      (set `CharacterMovementComponent.MaxWalkSpeed` 300.0 _charactermovement))))

(fn `UserConstructionScript`)