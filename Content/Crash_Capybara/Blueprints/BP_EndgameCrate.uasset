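; BP_EndgameCrate is a breakable crate actor for Crash Capybara.
; Its DestroyCrate event plays audio, hides the crate mesh, turns off its physics and collision, and activates the CCNCrateBreak effect.
; The actor destroys itself after a short delay.
; The event's comment mentions spawning a plum, but the graph contains no spawn logic.
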(event `DestroyCrate`
  (bind _sm_crate_02 (`self.SM_Crate_02`))
  ;[0 0.05098 0.003697] Destroy the box and spawn a plum
  (`AudioComponent.Play` (`self.Audio`) 0.0)
  (`SceneComponent.SetHiddenInGame` (`self.SM_Crate_02`) true false)
  (`PrimitiveComponent.SetSimulatePhysics` _sm_crate_02 false)
  (`PrimitiveComponent.SetCollisionEnabled` _sm_crate_02 "NoCollision")
  (`ActorComponent.Activate` (`self.CC_N_CrateBreak`) false)
  (`KismetSystemLibrary.Delay` 1.0)
  (`self.K2_DestroyActor`))

(fn `UserConstructionScript`)