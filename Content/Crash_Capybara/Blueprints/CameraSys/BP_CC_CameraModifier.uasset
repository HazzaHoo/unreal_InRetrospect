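; BP_CC_CameraModifier is a trigger volume that changes the game camera's behavior when the player character enters it.
; On overlap it messages the current view target with its stationary, look-at, transition, easing and linked-camera settings, plus a yaw-only target transform derived from its Camera component at BeginPlay.
; ResetCamera re-sends those settings after a short delay, then calls ResetCamera on LinkedCamera.
; The construction script sizes the box from CollisionBoundary.
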(event `self.ReceiveBeginPlay`
  (set `self.TargetTransform` (`KismetMathLibrary.MakeTransform` (0.0 0.0 0.0) (`KismetMathLibrary.MakeRotator` 0.0 0.0 (+ (.yaw (.rotation (`SceneComponent.K2_GetComponentToWorld` (`self.Camera`)))) 90.0)))))

(event `ResetCamera`
  (`KismetSystemLibrary.Delay` 0.6)
  (`|ExecutionSequence`
    (:`then_0`
      (message `/Game/Crash_Capybara/Blueprints/CameraSys/BPI_CameraInterface.SetNewCameraAtributes` (`Controller.GetViewTarget` (`GameplayStatics.GetPlayerController` 0)) (`self.Stationary`) (`self.Look at Characher`) (`self.TargetTransform`) (`self.Transition Time`) (`self.Easy Function`) (`self.Linked Camera`) :!label _label))
    (:`then_1`
      (`/Game/Crash_Capybara/Blueprints/CameraSys/BP_CC_Camera.Reset Camera` (`self.Linked Camera`) self))))

(event `self.ReceiveActorBeginOverlap`
  (params (OtherActor :type "Actor Object Reference"))
  (if (== OtherActor (`GameplayStatics.GetPlayerCharacter` 0))
    (goto _label)))

(fn `UserConstructionScript`
  (`BoxComponent.SetBoxExtent` (`self.Box`) (`self.CollisionBoundary`) true))