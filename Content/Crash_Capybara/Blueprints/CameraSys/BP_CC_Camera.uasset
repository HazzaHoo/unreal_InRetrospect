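; Crash Capybara spline-rail camera that follows the player and can start as the active view target.
; Tick eases the spring arm along the spline toward the player outside the DeadZone, optionally turning to look at them.
; SetNewCameraAtributes applies new settings and runs a timeline easing arm offset and rotation, updating the character's camera-relative movement.
; ResetCamera snaps to a respawn camera, makes the player invincible and briefly pauses following.
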(event `Reset Camera`
  (params (ResetLocation :type "/Game/Crash_Capybara/Blueprints/CameraSys/BP_CC_CameraModifier Object Reference"))
  (bind _camera (`/Game/Crash_Capybara/Blueprints/CameraSys/BP_CC_CameraModifier.Camera` ResetLocation))
  ; ResetCamera
  (set `self.Respawning?` true)
  (`SceneComponent.K2_SetWorldLocationAndRotation` (`self.SpringArm`) (`SplineComponent.FindLocationClosestToWorldLocation` (`self.Spline`) (`SceneComponent.K2_GetComponentLocation` _camera) "World") (`SceneComponent.K2_GetComponentRotation` _camera) false false)
  (bind _asbp_cc_player_characher (cast `/Game/Crash_Capybara/Blueprints/BP_CC_PlayerCharacher` (`GameplayStatics.GetPlayerCharacter` 0)))
  (`/Game/Crash_Capybara/Blueprints/BP_CC_PlayerCharacher.Invinciblity` _asbp_cc_player_characher)
  (`KismetSystemLibrary.Delay` 2.0)
  (set `self.Respawning?` false))

(event `self.ReceiveBeginPlay`
  ;[0 0.05098 0.003697] c
  (`self.FirstCameraUpdate`)
  (set `self.DefouldRelativeRotation` (`SceneComponent.RelativeRotation` (`self.Camera`)))
  (if (`self.StartingCamera`)
    (`PlayerController.SetViewTargetWithBlend` (`GameplayStatics.GetPlayerController` 0) self 0.0 "VTBlend_Linear" 0.0 false)
    (set `self.Active` true)
    (`SceneComponent.K2_SetWorldLocation` (`self.SpringArm`) (`SplineComponent.FindLocationClosestToWorldLocation` (`self.Spline`) (`self.K2_GetActorLocation` (`GameplayStatics.GetPlayerCharacter` 0)) "World") false false)))

(event `self.ReceiveTick`
  (params (DeltaSeconds :type "Float (single-precision)"))
  (bind _returnvalue (`PrimitiveComponent.IsOverlappingActor` (`self.DeadZone`) (`GameplayStatics.GetPlayerCharacter` 0)))
  (bind _relativerotation (`SceneComponent.RelativeRotation` (`self.Camera`)))
  ;[0 0.05098 0.003697] Camera control system
  ;;[0 0.05098 0.003697] Camera movement system
  (if (`self.Respawning?`)
    _
    (elif (and (`self.Active`) (not (`self.Stationary`)))
      (if (or (not (`KismetMathLibrary.InRange_FloatFloat` (.x (/ (`KismetMathLibrary.Conv_Vector2DToVector` (`PlayerController.ProjectWorldLocationToScreen` (`GameplayStatics.GetPlayerController` 0) (`self.K2_GetActorLocation` (`GameplayStatics.GetPlayerCharacter` 0)) false) 3.0) (`KismetMathLibrary.Conv_Vector2DToVector` (`WidgetLayoutLibrary.GetViewportSize`) 1.0))) 0.25 0.75)) (not (`KismetMathLibrary.InRange_FloatFloat` (.y (/ (`KismetMathLibrary.Conv_Vector2DToVector` (`PlayerController.ProjectWorldLocationToScreen` (`GameplayStatics.GetPlayerController` 0) (`self.K2_GetActorLocation` (`GameplayStatics.GetPlayerCharacter` 0)) false) 3.0) (`KismetMathLibrary.Conv_Vector2DToVector` (`WidgetLayoutLibrary.GetViewportSize`) 1.0))) 0.15 0.85)))
        (if (not _returnvalue)
          (if (not _returnvalue) :!label _label
            (`SceneComponent.K2_SetWorldLocation` (`self.SpringArm`) (`KismetMathLibrary.VInterpTo` (`SplineComponent.FindLocationClosestToWorldLocation` (`self.Spline`) (`SceneComponent.K2_GetComponentLocation` (`self.SpringArm`)) "World") (`SplineComponent.FindLocationClosestToWorldLocation` (`self.Spline`) (`self.K2_GetActorLocation` (`GameplayStatics.GetPlayerCharacter` 0)) "World") (`GameplayStatics.GetWorldDeltaSeconds`) 2.4) false false)
            (if (`self.LookAtCharacher`)
              (`SceneComponent.K2_SetRelativeRotation` (`self.Camera`) (`KismetMathLibrary.RInterpTo` _relativerotation (`KismetMathLibrary.FindRelativeLookAtRotation` (`SceneComponent.K2_GetComponentToWorld` (`self.Camera`)) (`self.K2_GetActorLocation` (`GameplayStatics.GetPlayerCharacter` 0))) (`GameplayStatics.GetWorldDeltaSeconds`) 0.5) false false)
              (else
                (`SceneComponent.K2_SetRelativeRotation` (`self.Camera`) (`KismetMathLibrary.RInterpTo` _relativerotation (`self.DefouldRelativeRotation`) (`GameplayStatics.GetWorldDeltaSeconds`) 0.2) false false)))))
        (else
          (goto _label))))))

(event `TransitionCamera`
  (bind _springarm (`self.SpringArm`))
  (bind (_targettransform_location _targettransform_rotation) (`KismetMathLibrary.BreakTransform` (`self.TargetTransform`)))
  ;[0 0.05098 0.003697] Camera control system
  ;;[0 0.05098 0.003697] TransitionCamera
  (`TimelineComponent.SetPlayRate` (`self.Transform Timeline`) (/ 1.0 (`self.TransitionTime`)))
  (bind (_direction _first) (`Timeline|Transform Timeline` :!via `PlayFromStart`)
    (:`Update`
      (set `SpringArmComponent.TargetOffset` (`|EaseFunction` (`self.EasingFunctoin`) _first (`SpringArmComponent.TargetOffset` (`self.SpringArm`)) _targettransform_location) _springarm)
      (`SceneComponent.K2_SetRelativeRotation` _springarm (`|EaseFunction` (`self.EasingFunctoin`) _first (`SceneComponent.RelativeRotation` (`self.SpringArm`)) _targettransform_rotation true 1.0) false false)
      (bind _asbp_cc_player_characher (cast `/Game/Crash_Capybara/Blueprints/BP_CC_PlayerCharacher` (`GameplayStatics.GetPlayerCharacter` 0)))
      (`/Game/Crash_Capybara/Blueprints/BP_CC_PlayerCharacher.CameraTurnUpdate` _asbp_cc_player_characher (`GameplayStatics.GetPlayerCameraManager` 0)))))

(event `FirstCameraUpdate`
  ;[0 0.05098 0.003697] Camera control system
  ;;[0 0.05098 0.003697] TransitionCamera
  ;;;[0 0.05098 0.003697] First update for movements to Camera Oriantation
  (bind _asbp_cc_player_characher (cast `/Game/Crash_Capybara/Blueprints/BP_CC_PlayerCharacher` (`GameplayStatics.GetPlayerCharacter` 0)))
  (`/Game/Crash_Capybara/Blueprints/BP_CC_PlayerCharacher.CameraTurnFirstUpdate` _asbp_cc_player_characher (`GameplayStatics.GetPlayerCameraManager` 0)))

(fn `SetNewCameraAtributes`
  (params (Stationary :type Boolean) (LookAtCharacher :type Boolean) (TargetTransform :type "Transform Structure") (TransitionTime :type "Float (double-precision)") (EasyFunction :type "EEasingFunc Enum" :default "Linear") (LinkedCamera :type "/Game/Crash_Capybara/Blueprints/CameraSys/BP_CC_Camera Object Reference"))
  (returns (Success :type Boolean))
  (set `self.Stationary` Stationary)
  (set `self.LookAtCharacher` LookAtCharacher)
  (set `self.TargetTransform` TargetTransform)
  (set `self.TransitionTime` TransitionTime)
  (set `self.EasingFunctoin` EasyFunction)
  (set `self.LinkedCamer` LinkedCamera)
  (`self.TransitionCamera`)
  (return false))

(fn `UserConstructionScript`
  (set `SpringArmComponent.SocketOffset` (`self.SocketOffSet`) (`self.SpringArm`)))