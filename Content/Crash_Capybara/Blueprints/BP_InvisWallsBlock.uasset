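; BP_InvisWallsBlock is a pair of switchable invisible-wall sets with matching signs that control which path blocks the player.
; On BeginPlay, the Pt2 walls have collision off and their sign is hidden.
; When a Player-tagged actor overlaps SwitchWallsCollision, blocking and sign visibility move from the Pt1 set to the Pt2 set.
; Overlapping ResetWalls swaps them back to Pt1.
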(event `self.ReceiveBeginPlay`
  (`PrimitiveComponent.SetCollisionEnabled` (`self.InvisWall_Pt2_01`) "NoCollision")
  (`PrimitiveComponent.SetCollisionEnabled` (`self.InvisWall_Pt2_02`) "NoCollision")
  (`SceneComponent.SetHiddenInGame` (`self.Sign_Pt2_01`) true true))

(event `self.SwitchWallsCollision.OnComponentBeginOverlap`
  (params (OverlappedComponent :type "PrimitiveComponent Object Reference") (OtherActor :type "Actor Object Reference") (OtherComp :type "PrimitiveComponent Object Reference") (OtherBodyIndex :type Integer) (bFromSweep :type Boolean) (SweepResult :type "HitResult Structure (by ref)"))
  (if (`self.ActorHasTag` OtherActor "Player")
    (`PrimitiveComponent.SetCollisionEnabled` (`self.InvisWall_Pt1_01`) "NoCollision")
    (`PrimitiveComponent.SetCollisionEnabled` (`self.InvisWall_Pt1_02`) "NoCollision")
    (`PrimitiveComponent.SetCollisionEnabled` (`self.InvisWall_Pt2_01`) "QueryAndPhysics")
    (`PrimitiveComponent.SetCollisionEnabled` (`self.InvisWall_Pt2_02`) "QueryAndPhysics")
    (`SceneComponent.SetHiddenInGame` (`self.Sign_Pt2_01`) false true)
    (`SceneComponent.SetHiddenInGame` (`self.Sign_Pt1_01`) true true)))

(event `self.ResetWalls.OnComponentBeginOverlap`
  (params (OverlappedComponent :type "PrimitiveComponent Object Reference") (OtherActor :type "Actor Object Reference") (OtherComp :type "PrimitiveComponent Object Reference") (OtherBodyIndex :type Integer) (bFromSweep :type Boolean) (SweepResult :type "HitResult Structure (by ref)"))
  (if (`self.ActorHasTag` OtherActor "Player")
    (`PrimitiveComponent.SetCollisionEnabled` (`self.InvisWall_Pt2_01`) "NoCollision")
    (`PrimitiveComponent.SetCollisionEnabled` (`self.InvisWall_Pt2_02`) "NoCollision")
    (`SceneComponent.SetHiddenInGame` (`self.Sign_Pt2_01`) true true)
    (`SceneComponent.SetHiddenInGame` (`self.Sign_Pt1_01`) false true)
    (`PrimitiveComponent.SetCollisionEnabled` (`self.InvisWall_Pt1_01`) "QueryAndPhysics")
    (`PrimitiveComponent.SetCollisionEnabled` (`self.InvisWall_Pt1_02`) "QueryAndPhysics")))

(fn `UserConstructionScript`)