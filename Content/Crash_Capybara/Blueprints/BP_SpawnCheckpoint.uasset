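; Checkpoint actor for Crash Capybara that records where the player reloads and which camera box goes with that spot.
; When a Player-tagged actor overlaps its Box, it waits briefly, then stores the player's current transform as ReloadTransform and its NearestCameraBox as LastCameraBox.
; The InitialSpawn event performs the same save without the delay.
; BeginPlay caches the player and camera references, though the camera reference is unused here.
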(event `SaveNearestCameraBox`
  (set `/Game/Crash_Capybara/Blueprints/BP_CC_PlayerCharacher.LastCameraBox` (`self.NearestCameraBox`) (`self.Player Ref`)))

(event `self.ReceiveBeginPlay`
  (bind _asbp_cc_player_characher (cast `/Game/Crash_Capybara/Blueprints/BP_CC_PlayerCharacher` (`GameplayStatics.GetPlayerCharacter` 0)))
  (set `self.Player Ref` _asbp_cc_player_characher)
  (bind _returnvalue (`GameplayStatics.GetActorOfClass` "/Game/Crash_Capybara/Blueprints/CameraSys/BP_CC_Camera.BP_CC_Camera_C"))
  (set `self.CC Camera Ref` _returnvalue))

(event `InitialSpawn`
  (bind _asbp_cc_player_characher (cast `/Game/Crash_Capybara/Blueprints/BP_CC_PlayerCharacher` (`GameplayStatics.GetPlayerCharacter` 0)))
  (set `/Game/Crash_Capybara/Blueprints/BP_CC_PlayerCharacher.reloadTransform` (`self.GetTransform` _asbp_cc_player_characher) _asbp_cc_player_characher)
  (`self.SaveNearestCameraBox`))

(event `self.Box.OnComponentBeginOverlap`
  (params (OverlappedComponent :type "PrimitiveComponent Object Reference") (OtherActor :type "Actor Object Reference") (OtherComp :type "PrimitiveComponent Object Reference") (OtherBodyIndex :type Integer) (bFromSweep :type Boolean) (SweepResult :type "HitResult Structure (by ref)"))
  (if (`self.ActorHasTag` OtherActor "Player")
    (`KismetSystemLibrary.Delay` 0.05)
    (bind _asbp_cc_player_characher (cast `/Game/Crash_Capybara/Blueprints/BP_CC_PlayerCharacher` (`GameplayStatics.GetPlayerCharacter` 0)))
    (set `/Game/Crash_Capybara/Blueprints/BP_CC_PlayerCharacher.reloadTransform` (`self.GetTransform` _asbp_cc_player_characher) _asbp_cc_player_characher)
    (`self.SaveNearestCameraBox`)))

(fn `UserConstructionScript`)