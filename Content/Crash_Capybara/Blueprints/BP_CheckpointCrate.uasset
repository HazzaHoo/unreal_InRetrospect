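; BP_CheckpointCrate is a breakable checkpoint crate that records the player's respawn state when it first takes damage.
; Breaking it saves the player's transform and the crate's NearestCameraBox, plays effects and the checkpoint widget animation, then destroys the actor.
; InitialSpawn saves the same player state without breaking the crate.
; Each tick, the widget rotates to face the BP_CC_Camera found at BeginPlay.
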(event `self.ReceiveAnyDamage`
  (params (Damage :type "Float (single-precision)") (DamageType :type "DamageType Object Reference") (InstigatedBy :type "Controller Object Reference") (DamageCauser :type "Actor Object Reference"))
  (bind _wb_checkpoint (`self.WB_Checkpoint`))
  (bind _sm_crate_02 (`self.SM_Crate_02`))
  ;[0 0.05098 0.003697] Destroy the box and spawn a plum
  (`/Engine/EditorBlueprintResources/StandardMacros.DoOnce` false
    (:`Completed`
      (`KismetSystemLibrary.Delay` 0.05)
      (bind _asbp_cc_player_characher (cast `/Game/Crash_Capybara/Blueprints/BP_CC_PlayerCharacher` (`GameplayStatics.GetPlayerCharacter` 0)))
      (set `/Game/Crash_Capybara/Blueprints/BP_CC_PlayerCharacher.reloadTransform` (`self.GetTransform` _asbp_cc_player_characher) _asbp_cc_player_characher)
      (`AudioComponent.Play` (`self.CC_BoxBreak_Cue`) 0.0)
      (`GameplayStatics.PlaySound2D` "/Game/Crash_Capybara/Audio/CC_CheckpointBox.CC_CheckpointBox" 1.0 1.0 0.0 null null)
      (`SceneComponent.SetHiddenInGame` (`self.SM_Crate_02`) true true)
      (bind _aswb_checkpoint (cast `/Game/Crash_Capybara/UserInterface/WB_Checkpoint` (`WidgetComponent.GetWidget` _wb_checkpoint)))
      (`/Game/Crash_Capybara/UserInterface/WB_Checkpoint.Load Anim` _aswb_checkpoint)
      (`ActorComponent.Activate` (`self.CC_N_CrateCheckpoint`) false)
      (`ActorComponent.Activate` (`self.CC_BoxBreak_Checkpoint_Cue`) false)
      (`SceneComponent.SetHiddenInGame` _wb_checkpoint false false)
      (`PrimitiveComponent.SetSimulatePhysics` _sm_crate_02 false)
      (`PrimitiveComponent.SetCollisionEnabled` _sm_crate_02 "NoCollision")
      (`self.SaveNearestCameraBox`)
      (`KismetSystemLibrary.Delay` 1.0)
      (`self.K2_DestroyActor`))))

(event `SaveNearestCameraBox`
  (set `/Game/Crash_Capybara/Blueprints/BP_CC_PlayerCharacher.LastCameraBox` (`self.NearestCameraBox`) (`self.Player Ref`)))

(event `self.ReceiveTick`
  (params (DeltaSeconds :type "Float (single-precision)"))
  (`self.RotateWidgetToPlayer`))

(event `self.ReceiveBeginPlay`
  (bind _asbp_cc_player_characher (cast `/Game/Crash_Capybara/Blueprints/BP_CC_PlayerCharacher` (`GameplayStatics.GetPlayerCharacter` 0)))
  (set `self.Player Ref` _asbp_cc_player_characher)
  (bind _returnvalue (`GameplayStatics.GetActorOfClass` "/Game/Crash_Capybara/Blueprints/CameraSys/BP_CC_Camera.BP_CC_Camera_C"))
  (set `self.CC Camera Ref` _returnvalue))

(event `InitialSpawn`
  (bind _asbp_cc_player_characher (cast `/Game/Crash_Capybara/Blueprints/BP_CC_PlayerCharacher` (`GameplayStatics.GetPlayerCharacter` 0)))
  (set `/Game/Crash_Capybara/Blueprints/BP_CC_PlayerCharacher.reloadTransform` (`self.GetTransform` _asbp_cc_player_characher) _asbp_cc_player_characher)
  (`self.SaveNearestCameraBox`))

(fn `RotateWidgetToPlayer`
  (`SceneComponent.K2_SetWorldRotation` (`self.WB_Checkpoint`) (`KismetMathLibrary.FindLookAtRotation` (`self.K2_GetActorLocation`) (`SceneComponent.K2_GetComponentLocation` (`/Game/Crash_Capybara/Blueprints/CameraSys/BP_CC_Camera.Camera` (`self.CC Camera Ref`)))) false false))

(fn `UserConstructionScript`)