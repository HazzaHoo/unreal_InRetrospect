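; Crash Capybara progression portal with a spinning key that advances the player to the next level or exits the finished game.
; A custom MoveKeyDown event lerps the key to a marker component that is hidden at BeginPlay.
; The player's first trigger overlap checks IsGameFinished on Global_Instance.
; If set, it plays a load-out widget and opens L_Modern_Arcade; otherwise it calls NextLevel and plays the pickup sound.
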(event `MoveKeyDown`
  ; Move Key Down
  (set `self.KeyLocation` (`SceneComponent.K2_GetComponentLocation` (`self.Key_SM`)))
  (bind (_direction _lerp) (`Timeline|MoveKey`)
    (:`Update`
      (`SceneComponent.K2_SetWorldLocation` (`self.Key_SM`) (`KismetMathLibrary.VLerp` (`self.KeyLocation`) (`SceneComponent.K2_GetComponentLocation` (`self.Key_EndLocation`)) _lerp) false false))))

(event `self.ReceiveBeginPlay`
  ; Hide Key End Location
  (`SceneComponent.SetHiddenInGame` (`self.Key_EndLocation`) true false)
  ; Animation
  (bind (_direction _lerp) (`Timeline|Animation`)
    (:`Update`
      (`SceneComponent.K2_SetRelativeRotation` (`self.Key_SM`) (`KismetMathLibrary.RLerp` (`KismetMathLibrary.MakeRotator` 0.0 -90.0) (`KismetMathLibrary.MakeRotator` 0.0 -90.0 360.0) _lerp) true false))))

(event `self.PortalTrigger.OnComponentBeginOverlap`
  (params (OverlappedComponent :type "PrimitiveComponent Object Reference") (OtherActor :type "Actor Object Reference") (OtherComp :type "PrimitiveComponent Object Reference") (OtherBodyIndex :type Integer) (bFromSweep :type Boolean) (SweepResult :type "HitResult Structure (by ref)"))
  (bind _asbp_cc_player_characher (cast `/Game/Crash_Capybara/Blueprints/BP_CC_PlayerCharacher` OtherActor))
  (`/Engine/EditorBlueprintResources/StandardMacros.DoOnce` false
    (:`Completed`
      ; Collision
      (bind _asglobal_instance (cast `/Game/Global_IMC/Global_Instance` (`GameplayStatics.GetGameInstance`)))
      (if (`/Game/Global_IMC/Global_Instance.IsGameFinished?` _asglobal_instance)
        (bind _returnvalue (`|CreateWidget` "/Game/Global_Userinterface/WB_LoadInOrOut.WB_LoadInOrOut_C"))
        (`/Game/Global_Userinterface/WB_LoadInOrOut.Load Out` _returnvalue)
        (`UserWidget.AddToViewport` _returnvalue 0)
        (`KismetSystemLibrary.Delay` 0.5)
        (`GameplayStatics.OpenLevel` "L_Modern_Arcade")
        (else
          (`/Game/Crash_Capybara/Blueprints/BP_CC_PlayerCharacher.NextLevel` _asbp_cc_player_characher)
          (`GameplayStatics.PlaySound2D` "/Game/Crash_Capybara/Audio/CC_KeyPickup.CC_KeyPickup" 1.0 1.0 0.0 null null))))))

(fn `UserConstructionScript`)