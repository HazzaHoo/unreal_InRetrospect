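; Collectible plum pickup for the Crash Capybara game that credits the player character on contact.
; A sphere overlap waits briefly, then casts the other actor to BP_CC_PlayerCharacher and calls its PickupPlum.
; It then plays the sound cue, hides the plum and activates the collect effect, delaying destruction so both can play.
; The overlap collision stays enabled until the actor is destroyed.
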(event `self.Sphere.OnComponentBeginOverlap`
  (params (OverlappedComponent :type "PrimitiveComponent Object Reference") (OtherActor :type "Actor Object Reference") (OtherComp :type "PrimitiveComponent Object Reference") (OtherBodyIndex :type Integer) (bFromSweep :type Boolean) (SweepResult :type "HitResult Structure (by ref)"))
  ;[0 0.05098 0.003697] destroy a plum and collect it
  (`KismetSystemLibrary.Delay` 0.2)
  (bind _asbp_cc_player_characher (cast `/Game/Crash_Capybara/Blueprints/BP_CC_PlayerCharacher` OtherActor))
  (`/Game/Crash_Capybara/Blueprints/BP_CC_PlayerCharacher.PickupPlum` _asbp_cc_player_characher)
  (`AudioComponent.Play` (`self.CC_Plum_Cue`) 0.0)
  (`SceneComponent.SetHiddenInGame` (`self.PLUM`) true false)
  (`ActorComponent.Activate` (`self.CC_N_PlumCollect`) false)
  (`KismetSystemLibrary.Delay` 1.0)
  (`self.K2_DestroyActor`))

(fn `UserConstructionScript`)