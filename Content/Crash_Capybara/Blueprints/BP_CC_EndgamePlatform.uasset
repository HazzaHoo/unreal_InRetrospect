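; End-of-level podium for Crash Capybara that runs the end-screen sequence.
; On player overlap it raises an invisible wall, disables movement, then uses timelines to move the player to the podium and face the camera.
; It passes crate totals and itself to the end-game widget for counting, and saves a plum achievement flag when enough are collected.
; It also provides events to spawn crates and the progression portal, breaking crates that overlap its trigger.
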(event `self.ReceiveBeginPlay`
  (bind _inviswall (`self.InvisWall`))
  ; Hide Invis Wall
  (`SceneComponent.SetHiddenInGame` _inviswall true false)
  (`PrimitiveComponent.SetCollisionEnabled` _inviswall "NoCollision"))

(event `SpawnKey`
  ; Spawn Key
  (bind _returnvalue (`|SpawnActorFromClass` "/Game/Crash_Capybara/Blueprints/BP_CC_Progression_Portal.BP_CC_Progression_Portal_C" (`KismetMathLibrary.MakeTransform` (`SceneComponent.K2_GetComponentLocation` (`self.KeySpawnLocation`))) "Undefined" "MultiplyWithRoot" null null))
  (`/Game/Crash_Capybara/Blueprints/BP_CC_Progression_Portal.MoveKeyDown` _returnvalue))

(event `SpawnCrate`
  ; Spawn Crate
  (`|SpawnActorFromClass` "/Game/Crash_Capybara/Blueprints/BP_EndgameCrate.BP_EndgameCrate_C" (`SceneComponent.K2_GetComponentToWorld` (`self.CrateSpawnLocation`)) "Undefined" "MultiplyWithRoot" null null))

(event `self.SphereCollision.OnComponentBeginOverlap`
  (params (OverlappedComponent :type "PrimitiveComponent Object Reference") (OtherActor :type "Actor Object Reference") (OtherComp :type "PrimitiveComponent Object Reference") (OtherBodyIndex :type Integer) (bFromSweep :type Boolean) (SweepResult :type "HitResult Structure (by ref)"))
  (bind _arrow (`self.Arrow`))
  (bind _player_ref (`self.Player Ref`))
  (bind _player_ref_2 (`self.Player Ref`))
  (bind _player_ref_3 (`self.Player Ref`))
  ; Set Player Vars
  (bind _asbp_cc_player_characher (cast `/Game/Crash_Capybara/Blueprints/BP_CC_PlayerCharacher` OtherActor))
  (`/Engine/EditorBlueprintResources/StandardMacros.DoOnce` false
    (:`Completed`
      (`PrimitiveComponent.SetCollisionEnabled` (`self.InvisWall`) "QueryAndPhysics")
      (bind _output_get (set `self.Player Ref` _asbp_cc_player_characher))
      (set `/Game/Crash_Capybara/Blueprints/BP_CC_PlayerCharacher.InEndScreen` true _output_get)
      (set `/Game/Crash_Capybara/Blueprints/BP_CC_PlayerCharacher.EndGame` true (`self.Player Ref`))
      (set `/Game/Crash_Capybara/Blueprints/BP_CC_PlayerCharacher.EndGameWalkAnim` true _player_ref_2)
      (`CharacterMovementComponent.DisableMovement` (`Character.CharacterMovement` _player_ref_2))
      ; Move Player to Podium
      (set `self.PlayerLocation` (`SceneComponent.K2_GetComponentLocation` (`Character.CapsuleComponent` _player_ref_2)))
      (bind (_direction _lerp_) (`Timeline|MovePlayer` :!via `PlayFromStart`)
        (:`Update`
          (`self.K2_SetActorLocation` (`self.Player Ref`) (`KismetMathLibrary.VLerp` (`self.PlayerLocation`) (`SceneComponent.K2_GetComponentLocation` _arrow) _lerp_) false true)
          (`Controller.SetControlRotation` (`GameplayStatics.GetPlayerController` 0) (`KismetMathLibrary.FindLookAtRotation` (`SceneComponent.K2_GetComponentLocation` (`Actor.RootComponent` (`self.Player Ref`))) (`SceneComponent.K2_GetComponentLocation` _arrow))))
        (:`Finished`
          ; Rotate Player to Camera
          (set `/Game/Crash_Capybara/Blueprints/BP_CC_PlayerCharacher.EndGameWalkAnim` false _player_ref_3)
          (set `self.PlayerRotation` (`SceneComponent.K2_GetComponentRotation` (`Character.CapsuleComponent` _player_ref_3)))
          (bind _outactors (`GameplayStatics.GetAllActorsOfClass` "/Game/Crash_Capybara/Blueprints/CameraSys/BP_CC_Camera.BP_CC_Camera_C"))
          (bind (_direction_2 _lerp) (`Timeline|RotatePlayerToCamera`)
            (:`Update`
              (`Controller.SetControlRotation` (`GameplayStatics.GetPlayerController` 0) (`KismetMathLibrary.RLerp` (`self.PlayerRotation`) (`KismetMathLibrary.FindLookAtRotation` (`SceneComponent.K2_GetComponentLocation` (`Actor.RootComponent` (`self.Player Ref`))) (`SceneComponent.K2_GetComponentLocation` (`/Game/Crash_Capybara/Blueprints/CameraSys/BP_CC_Camera.Camera` (`|GetArrayItem` _outactors)))) _lerp)))
            (:`Finished`
              ; Set Vars and Start Crate Counting
              (set `self.CratesNeeded` (`/Game/Crash_Capybara/Blueprints/BP_CC_PlayerCharacher.CratesAmountForPortal` _player_ref))
              (set `self.Crates Destroyed` (`/Game/Crash_Capybara/Blueprints/BP_CC_PlayerCharacher.CratesDestroyed` _player_ref))
              (bind _aswb_cc_end_game (cast `/Game/Crash_Capybara/UserInterface/WB_CC_EndGame` (`WidgetComponent.GetWidget` (`self.TextWidget`))))
              (`/Game/Crash_Capybara/UserInterface/WB_CC_EndGame.CountCrates` _aswb_cc_end_game (`self.CratesNeeded`) (`self.Crates Destroyed`) self)
              (if (>= (`/Game/Crash_Capybara/Blueprints/BP_CC_PlayerCharacher.Plums` (`self.Player Ref`)) 45)
                (bind _asglobal_instance (cast `/Game/Global_IMC/Global_Instance` (`GameplayStatics.GetGameInstance`)))
                (set `/Game/Global_IMC/Global_Instance.Crash45+Plums` true _asglobal_instance)
                (bind _returnvalue (`GameplayStatics.DoesSaveGameExist` "settings"))
                (if _returnvalue
                  (bind _returnvalue_2 (`GameplayStatics.LoadGameFromSlot` "settings"))
                  (bind _assettings_save_game (cast `/Game/SettingsSaveGame` _returnvalue_2))
                  (set `/Game/SettingsSaveGame.CrashPlums` true _assettings_save_game)
                  (`GameplayStatics.SaveGameToSlot` _assettings_save_game "settings"))))))))))

(event `self.BoxBreak.OnComponentBeginOverlap`
  (params (OverlappedComponent :type "PrimitiveComponent Object Reference") (OtherActor :type "Actor Object Reference") (OtherComp :type "PrimitiveComponent Object Reference") (OtherBodyIndex :type Integer) (bFromSweep :type Boolean) (SweepResult :type "HitResult Structure (by ref)"))
  (if (`self.ActorHasTag` OtherActor "Crate")
    (bind _asbp_endgame_crate (cast `/Game/Crash_Capybara/Blueprints/BP_EndgameCrate` OtherActor))
    (`/Game/Crash_Capybara/Blueprints/BP_EndgameCrate.DestroyCrate` _asbp_endgame_crate)))

(fn `UserConstructionScript`)