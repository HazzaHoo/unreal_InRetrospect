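; Player Blueprint for the Crash Capybara minigame, handling lives, plum pickups, HUD and pause menu.
; BeginPlay adds the input mapping contexts and HUD, which updates on plum and life changes; running out of lives shows game over.
; Pause toggles a lazily created widget borrowed from SuperFabio, respawn reopens the current level, and portal overlap loads a level instance.
; Move, jump, crouch, attack and spin inputs are empty stubs; Backspace triggers debug damage.
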(event `Respawn Player`
  ; Respawn Player
  (bind _returnvalue (`GameplayStatics.GetCurrentLevelName` true))
  (`GameplayStatics.OpenLevel` (`KismetStringLibrary.Conv_StringToName` _returnvalue)))

(event `PickupPlum`
  ; Pickup Plum
  (set `self.Plums` (+ (`self.Plums`) 1))
  (`/Game/Crash_Capybara/UserInterface/WB_In-GameHUD_CrashCapybara.Show Plums` (`self.HUD Widget`)))

(event `Key|BackSpace`
  (params (Key :type "Key Structure"))
  ;[0.15 0 0 0.5] Damage Debug
  (:`Pressed`
    (`self.Player Damage`)))

(event `Player Damage`
  ; Player Damage and Gain Life
  (bind _result (`/Engine/EditorBlueprintResources/StandardMacros.DecrementInt` (`self.Lives`))
    (:`  `
      (set `self.Lives` _result :!label _label)
      (`/Game/Crash_Capybara/UserInterface/WB_In-GameHUD_CrashCapybara.Show Lives` (`self.HUD Widget`))
      (`KismetSystemLibrary.Delay` 0.5)
      (if (<= (`self.Lives`) 0)
        (bind _returnvalue (`|CreateWidget` "/Game/Crash_Capybara/UserInterface/WB_GameOverScreen_CrashCapybara.WB_GameOverScreen_CrashCapybara_C"))
        (`UserWidget.AddToViewport` _returnvalue 0)))))

(event `Add Life (X Num of Plums)`
  ; Player Damage and Gain Life
  (`/Engine/EditorBlueprintResources/StandardMacros.IncrementInt` (`self.Lives`)
    (:`  `
      (goto _label))))

(event `Close Pause Menu`
  (bind _returnvalue (`GameplayStatics.GetPlayerController` 0))
  ;[0.15 0.15 0.15 0.5 74] User-interface
  ;; Open or Close Pause Menu
  (`Widget.SetVisibility` (`self.PauseWidget`) "Hidden" :!label _label_2)
  (set `self.IsPauseMenuOpen?` false)
  (`GameplayStatics.SetGamePaused` false)
  (`WidgetBlueprintLibrary.SetInputMode_GameOnly` _returnvalue)
  (set `PlayerController.bShowMouseCursor` false _returnvalue))

(event `EnhancedInput|/Game/Global_IMC/IA_Pause`
  (params (ActionValue :type Boolean) (ElapsedSeconds :type "Float (double-precision)") (TriggeredSeconds :type "Float (double-precision)") (InputAction :type "InputAction Object Reference" :default "/Game/Global_IMC/IA_Pause.IA_Pause"))
  (bind _returnvalue (`GameplayStatics.GetPlayerController` 0))
  ;[0.15 0.15 0.15 0.5 74] User-interface
  ;; Open or Close Pause Menu
  (:`Canceled`
    (`/Engine/EditorBlueprintResources/StandardMacros.IsValid` (`self.PauseWidget`)
      (:`Is Valid`
        (if (`self.IsPauseMenuOpen?`)
          (goto _label_2)
          (else
            (`Widget.SetVisibility` (`self.PauseWidget`) "Visible"))))
      (:`Is Not Valid`
        (bind _returnvalue_2 (`|CreateWidget` "/Game/Super_Fabio/UserInterface/WB_PauseScreen_SuperFabio.WB_PauseScreen_SuperFabio_C"))
        (bind _output_get (set `self.PauseWidget` _returnvalue_2))
        (`UserWidget.AddToViewport` _output_get 1)))
    (set `self.IsPauseMenuOpen?` true)
    (`GameplayStatics.SetGamePaused` true)
    (`WidgetBlueprintLibrary.SetInputMode_GameAndUIEx` _returnvalue (`self.PauseWidget`) "DoNotLock" false)
    (set `PlayerController.bShowMouseCursor` true _returnvalue)))

(event `Spawn In-Game HUD`
  ;[0.15 0.15 0.15 0.5 74] User-interface
  ;; Spawn In Game HUD
  (bind _returnvalue (`|CreateWidget` "/Game/Super_Fabio/UserInterface/WB_In-GameHUD_SuperFabio.WB_In-GameHUD_SuperFabio_C"))
  (`UserWidget.AddToViewport` _returnvalue 0))

(event `self.ReceiveBeginPlay`
  ; Player Control
  (set `self.CC_Game` true)
  (bind _asplayer_controller (cast `PlayerController` (`self.GetController`)))
  (bind _returnvalue (pcsubsystem `EnhancedInputLocalPlayerSubsystem` _asplayer_controller))
  (`/Engine/EditorBlueprintResources/StandardMacros.IsValid` _returnvalue
    (:`Is Valid`
      (`EnhancedInputSubsystemInterface.AddMappingContext` _returnvalue "/Game/Crash_Capybara/IMC/IMC_CrashCapibara.IMC_CrashCapibara" 0 (struct))
      (`EnhancedInputSubsystemInterface.AddMappingContext` _returnvalue "/Game/Global_IMC/IMC_Global.IMC_Global" 0 (struct))
      (bind _returnvalue_2 (`|CreateWidget` "/Game/Crash_Capybara/UserInterface/WB_In-GameHUD_CrashCapybara.WB_In-GameHUD_CrashCapybara_C"))
      (bind _output_get (set `self.HUD Widget` _returnvalue_2))
      (`UserWidget.AddToViewport` _output_get 0))))

(event `EnhancedInput|/Game/Crash_Capybara/IMC/IA_CC_Attack`
  (params (ActionValue :type Boolean) (ElapsedSeconds :type "Float (double-precision)") (TriggeredSeconds :type "Float (double-precision)") (InputAction :type "InputAction Object Reference" :default "/Game/Crash_Capybara/IMC/IA_CC_Attack.IA_CC_Attack"))
  ; Player Control
)

(event `EnhancedInput|/Game/Crash_Capybara/IMC/IA_CC_Crouch`
  (params (ActionValue :type Boolean) (ElapsedSeconds :type "Float (double-precision)") (TriggeredSeconds :type "Float (double-precision)") (InputAction :type "InputAction Object Reference" :default "/Game/Crash_Capybara/IMC/IA_CC_Crouch.IA_CC_Crouch"))
  ; Player Control
)

(event `EnhancedInput|/Game/Crash_Capybara/IMC/IA_CC_Jump`
  (params (ActionValue :type Boolean) (ElapsedSeconds :type "Float (double-precision)") (TriggeredSeconds :type "Float (double-precision)") (InputAction :type "InputAction Object Reference" :default "/Game/Crash_Capybara/IMC/IA_CC_Jump.IA_CC_Jump"))
  ; Player Control
)

(event `EnhancedInput|/Game/Crash_Capybara/IMC/IA_CC_Move`
  (params (ActionValue :type "Vector2D Structure") (ElapsedSeconds :type "Float (double-precision)") (TriggeredSeconds :type "Float (double-precision)") (InputAction :type "InputAction Object Reference" :default "/Game/Crash_Capybara/IMC/IA_CC_Move.IA_CC_Move"))
  ; Player Control
)

(event `EnhancedInput|/Game/Crash_Capybara/IMC/IA_CC_Spin`
  (params (ActionValue :type Boolean) (ElapsedSeconds :type "Float (double-precision)") (TriggeredSeconds :type "Float (double-precision)") (InputAction :type "InputAction Object Reference" :default "/Game/Crash_Capybara/IMC/IA_CC_Spin.IA_CC_Spin"))
  ; Player Control
)

(event `self.ReceiveActorBeginOverlap`
  (params (OtherActor :type "Actor Object Reference"))
  ; Progression logic
  (cast `/Game/Crash_Capybara/Blueprints/BP_CC_Progression_Portal` OtherActor)
  (`LevelStreamingDynamic.LoadLevelInstance` "" (0.0 0.0 0.0) (struct) "L_CrashCapybra" null))

(fn `UserConstructionScript`)