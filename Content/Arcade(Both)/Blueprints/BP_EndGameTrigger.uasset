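; BP_EndGameTrigger is an arcade trigger that lets the player end the game through an interact prompt.
; A box overlap with a Player-tagged actor shows the text prompt and sets an in-range flag, and Tick turns that text toward the first-person camera.
; It registers the arcade input mapping on BeginPlay, and the pickup action in range opens the end-game widget and fades out the player's music.
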(event `self.ReceiveTick`
  (params (DeltaSeconds :type "Float (single-precision)"))
  (`self.RotateTextToPlayer`))

(event `self.ReceiveBeginPlay`
  (bind _returnvalue (`GameplayStatics.GetPlayerController` 0))
  ; Input Mapping Context
  (`EnhancedInputSubsystemInterface.AddMappingContext` (pcsubsystem `EnhancedInputLocalPlayerSubsystem` _returnvalue) "/Game/Arcade(Both)/IMC/IMC_Arcade_Both.IMC_Arcade_Both" 0 (struct))
  (`self.EnableInput` _returnvalue)
  (bind _asbp_arcade_player (cast `/Game/Arcade(Both)/Blueprints/BP_ArcadePlayer` (`GameplayStatics.GetPlayerCharacter` 0)))
  (set `self.Player Ref` _asbp_arcade_player))

(event `self.Box.OnComponentBeginOverlap`
  (params (OverlappedComponent :type "PrimitiveComponent Object Reference") (OtherActor :type "Actor Object Reference") (OtherComp :type "PrimitiveComponent Object Reference") (OtherBodyIndex :type Integer) (bFromSweep :type Boolean) (SweepResult :type "HitResult Structure (by ref)"))
  (if (`self.ActorHasTag` OtherActor "Player")
    (`SceneComponent.SetHiddenInGame` (`self.TextRender`) false false)
    (set `self.PlayerInRange?` true)))

(event `self.Box.OnComponentEndOverlap`
  (params (OverlappedComponent :type "PrimitiveComponent Object Reference") (OtherActor :type "Actor Object Reference") (OtherComp :type "PrimitiveComponent Object Reference") (OtherBodyIndex :type Integer))
  (if (`self.ActorHasTag` OtherActor "Player")
    (`SceneComponent.SetHiddenInGame` (`self.TextRender`) true false)
    (set `self.PlayerInRange?` false)))

(event `EnhancedInput|/Game/Arcade(Both)/IMC/IA_Arcade_Pickup`
  (params (ActionValue :type Boolean) (ElapsedSeconds :type "Float (double-precision)") (TriggeredSeconds :type "Float (double-precision)") (InputAction :type "InputAction Object Reference" :default "/Game/Arcade(Both)/IMC/IA_Arcade_Pickup.IA_Arcade_Pickup"))
  (:`Started`
    (if (`self.PlayerInRange?`)
      (bind _returnvalue (`|CreateWidget` "/Game/Arcade(Both)/User-interface/WB_EndGame.WB_EndGame_C"))
      (`UserWidget.AddToViewport` _returnvalue 0)
      (`/Game/Arcade(Both)/Blueprints/BP_ArcadePlayer.FadeMusicOut` (`self.Player Ref`) 5.0))))

(fn `RotateTextToPlayer`
  (`SceneComponent.K2_SetWorldRotation` (`self.TextRender`) (`KismetMathLibrary.FindLookAtRotation` (`SceneComponent.K2_GetComponentLocation` (`self.TextRender`)) (`SceneComponent.K2_GetComponentLocation` (`/Game/Arcade(Both)/Blueprints/BP_ArcadePlayer.FirstPersonCamera` (`self.Player Ref`)))) false false))

(fn `UserConstructionScript`)