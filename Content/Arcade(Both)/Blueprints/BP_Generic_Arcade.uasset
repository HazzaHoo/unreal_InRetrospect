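; Generic arcade machine prop with a chair that randomizes its look on BeginPlay to suit the current level.
; In the modern arcade and main menu levels it gets a random clean machine material and a random chair rotation between set limits.
; Other levels get a random dirty machine material and broken chair material, with the chair randomly fallen over, hidden without collision, or rotated as usual.
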(event `self.ReceiveBeginPlay`
  (`self.RotateChairsRandomly`))

(fn `RotateChairsRandomly`
  (bind _returnvalue (`KismetMathLibrary.RandomIntegerInRange` 0 5))
  (bind (_fallenchair_roll _fallenchair_pitch) (`KismetMathLibrary.BreakRotator` (`self.FallenChair`)))
  (bind _sm_arcadechair (`self.SM_ArcadeChair`))
  (bind _returnvalue_2 (`GameplayStatics.GetCurrentLevelName` true))
  (if (or (`KismetStringLibrary.EqualEqual_StrStr` _returnvalue_2 "L_Modern_Arcade") (`KismetStringLibrary.EqualEqual_StrStr` _returnvalue_2 "L_MainMenu"))
    (`self.Set Arcade Machine Textures` false true)
    (`SceneComponent.K2_SetRelativeRotation` (`self.SM_ArcadeChair`) (`KismetMathLibrary.RLerp` (`self.MinRotation`) (`self.MaxRotation`) (`KismetMathLibrary.RandomFloatInRange` 0.0 1.0)) false false :!label _label)
    (else
      (`PrimitiveComponent.SetMaterial` (`self.SM_ArcadeChair`) 0 "/Game/Arcade(Both)/Assets/Materials/M_BrokenChair.M_BrokenChair")
      (`self.Set Arcade Machine Textures` true)
      (if (== _returnvalue 0)
        (`SceneComponent.K2_SetRelativeRotation` (`self.SM_ArcadeChair`) (`KismetMathLibrary.MakeRotator` _fallenchair_roll _fallenchair_pitch (`KismetMathLibrary.RandomFloatInRange` 0.0 -180.0)) false false)
        (elif (== _returnvalue 1)
          (`SceneComponent.SetHiddenInGame` _sm_arcadechair true false)
          (`PrimitiveComponent.SetCollisionEnabled` _sm_arcadechair "NoCollision")
          (else
            (goto _label)))))))

(fn `Set Arcade Machine Textures`
  (params (`Broken Arcade?` :type Boolean) (`Modern Arcade?` :type Boolean))
  (bind _returnvalue (`KismetMathLibrary.RandomIntegerInRange` 0 2))
  (if `Broken Arcade?`
    (switch `int` _returnvalue
      (:`0`
        (set `self.ArcadeMaterial` "/Game/Arcade(Both)/Assets/Materials/ArcadeMachines/M_Arcade_Dirty_01.M_Arcade_Dirty_01"))
      (:`1`
        (set `self.ArcadeMaterial` "/Game/Arcade(Both)/Assets/Materials/ArcadeMachines/M_Arcade_Dirty_02.M_Arcade_Dirty_02"))
      (:`2`
        (set `self.ArcadeMaterial` "/Game/Arcade(Both)/Assets/Materials/ArcadeMachines/M_Arcade_Dirty_03.M_Arcade_Dirty_03")))
    (`PrimitiveComponent.SetMaterial` (`self.SM_ArcadeMachine_2`) 0 (`self.ArcadeMaterial`) :!label _label)
    (elif `Modern Arcade?`
      (switch `int` _returnvalue
        (:`0`
          (set `self.ArcadeMaterial` "/Game/Arcade(Both)/Assets/Materials/ArcadeMachines/M_Arcade_Clean_01.M_Arcade_Clean_01")
          (goto _label))
        (:`1`
          (set `self.ArcadeMaterial` "/Game/Arcade(Both)/Assets/Materials/ArcadeMachines/M_Arcade_Clean_02.M_Arcade_Clean_02")
          (goto _label))
        (:`2`
          (set `self.ArcadeMaterial` "/Game/Arcade(Both)/Assets/Materials/ArcadeMachines/M_Arcade_Clean_03.M_Arcade_Clean_03")
          (goto _label))))))

(fn `UserConstructionScript`)