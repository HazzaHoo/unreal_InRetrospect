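; BP_DifficultyChanger is an arcade interaction actor that lets the player open and close a difficulty screen.
; BeginPlay adds the arcade input context, enables input and creates the difficulty widget hidden.
; Sphere overlaps set the in-range flag and show or hide a prompt using the secret-collectables widget, without filtering the overlapping actor.
; While in range, the pickup input toggles the screen through its pause-menu open/close functions.
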(event `self.ReceiveBeginPlay`
  (bind _returnvalue (`GameplayStatics.GetPlayerController` 0))
  ; Input Mapping Context
  (`EnhancedInputSubsystemInterface.AddMappingContext` (pcsubsystem `EnhancedInputLocalPlayerSubsystem` _returnvalue) "/Game/Arcade(Both)/IMC/IMC_Arcade_Both.IMC_Arcade_Both" 0 (struct))
  (`self.EnableInput` _returnvalue)
  (bind _asbp_arcade_player (cast `/Game/Arcade(Both)/Blueprints/BP_ArcadePlayer` (`GameplayStatics.GetPlayerCharacter` 0)))
  (set `self.Player Ref` _asbp_arcade_player)
  (bind _returnvalue_2 (`|CreateWidget` "/Game/Arcade(Both)/User-interface/WB_DifficultyScreen.WB_DifficultyScreen_C"))
  (`UserWidget.AddToViewport` _returnvalue_2 99)
  (set `self.DiffScren Ref` _returnvalue_2)
  (`Widget.SetVisibility` _returnvalue_2 "Hidden"))

(event `EnhancedInput|/Game/Arcade(Both)/IMC/IA_Arcade_Pickup`
  (params (ActionValue :type Boolean) (ElapsedSeconds :type "Float (double-precision)") (TriggeredSeconds :type "Float (double-precision)") (InputAction :type "InputAction Object Reference" :default "/Game/Arcade(Both)/IMC/IA_Arcade_Pickup.IA_Arcade_Pickup"))
  (bind _diffscren_ref (`self.DiffScren Ref`))
  (:`Started`
    (if (`self.PlayerInRange?`)
      (switch `ESlateVisibility` (`Widget.GetVisibility` (`self.DiffScren Ref`))
        (:`Visible`
          (`/Game/Arcade(Both)/User-interface/WB_DifficultyScreen.Close Pause Menu` _diffscren_ref))
        (:`Hidden`
          (`/Game/Arcade(Both)/User-interface/WB_DifficultyScreen.Open Pause Menu` _diffscren_ref))))))

(event `self.Sphere.OnComponentBeginOverlap`
  (params (OverlappedComponent :type "PrimitiveComponent Object Reference") (OtherActor :type "Actor Object Reference") (OtherComp :type "PrimitiveComponent Object Reference") (OtherBodyIndex :type Integer) (bFromSweep :type Boolean) (SweepResult :type "HitResult Structure (by ref)"))
  (bind _returnvalue (`|CreateWidget` "/Game/Arcade(Both)/User-interface/WB_ArcadeSecretCollectables.WB_ArcadeSecretCollectables_C"))
  (`UserWidget.AddToViewport` _returnvalue 0)
  (bind _output_get (set `self.Widget Ref` _returnvalue))
  (`/Game/Arcade(Both)/User-interface/WB_ArcadeSecretCollectables.ShowPopup` _output_get (`self.TextToDisplay`))
  (set `self.PlayerInRange?` true))

(event `self.Sphere.OnComponentEndOverlap`
  (params (OverlappedComponent :type "PrimitiveComponent Object Reference") (OtherActor :type "Actor Object Reference") (OtherComp :type "PrimitiveComponent Object Reference") (OtherBodyIndex :type Integer))
  (`/Game/Arcade(Both)/User-interface/WB_ArcadeSecretCollectables.HidePopup` (stale `self.Sphere.OnComponentBeginOverlap` _output_get))
  (set `self.PlayerInRange?` false))

(fn `UserConstructionScript`)