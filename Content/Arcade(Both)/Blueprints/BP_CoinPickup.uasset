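; BP_CoinPickup is an arcade coin actor that the player can pick up while standing near it.
; A collision sphere shows interact text and sets NearCoin on the cached BP_ArcadePlayer while that player overlaps, clearing both on exit.
; Each tick rotates the text toward the player's first-person camera.
; The DestroyCoin event adds a BP_PickupCoin widget to the viewport and destroys the actor.
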(event `Destroy Coin`
  (bind _returnvalue (`|CreateWidget` "/Game/Arcade(Both)/User-interface/BP_PickupCoin.BP_PickupCoin_C"))
  (`UserWidget.AddToViewport` _returnvalue 0)
  (`self.K2_DestroyActor`))

(event `self.ReceiveBeginPlay`
  (bind _asbp_arcade_player (cast `/Game/Arcade(Both)/Blueprints/BP_ArcadePlayer` (`GameplayStatics.GetPlayerCharacter` 0)))
  (set `self.Player Ref` _asbp_arcade_player))

(event `self.ReceiveTick`
  (params (DeltaSeconds :type "Float (single-precision)"))
  (`self.Rotate Text to Camera`))

(event `self.Collision Sphere.OnComponentBeginOverlap`
  (params (OverlappedComponent :type "PrimitiveComponent Object Reference") (OtherActor :type "Actor Object Reference") (OtherComp :type "PrimitiveComponent Object Reference") (OtherBodyIndex :type Integer) (bFromSweep :type Boolean) (SweepResult :type "HitResult Structure (by ref)"))
  (if (== OtherActor (`self.Player Ref`))
    (`SceneComponent.SetHiddenInGame` (`self.Interact_Text`) false false)
    (set `self.InRange?` true)
    (set `/Game/Arcade(Both)/Blueprints/BP_ArcadePlayer.NearCoin?` true (`self.Player Ref`))))

(event `self.Collision Sphere.OnComponentEndOverlap`
  (params (OverlappedComponent :type "PrimitiveComponent Object Reference") (OtherActor :type "Actor Object Reference") (OtherComp :type "PrimitiveComponent Object Reference") (OtherBodyIndex :type Integer))
  (`SceneComponent.SetHiddenInGame` (`self.Interact_Text`) true false)
  (set `self.InRange?` false)
  (set `/Game/Arcade(Both)/Blueprints/BP_ArcadePlayer.NearCoin?` false (`self.Player Ref`)))

(fn `Rotate Text to Camera`
  (`SceneComponent.K2_SetWorldRotation` (`self.Interact_Text`) (`KismetMathLibrary.FindLookAtRotation` (`SceneComponent.K2_GetComponentLocation` (`self.Interact_Text`)) (`SceneComponent.K2_GetComponentLocation` (`/Game/Arcade(Both)/Blueprints/BP_ArcadePlayer.FirstPersonCamera` (`self.Player Ref`)))) false false))

(fn `UserConstructionScript`)