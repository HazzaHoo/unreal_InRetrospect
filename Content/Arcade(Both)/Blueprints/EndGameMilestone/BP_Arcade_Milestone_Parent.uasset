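; Parent Blueprint for arcade milestone collectables, revealed once the matching arcade game's achievement is recorded in the game instance.
; On BeginPlay it creates a hidden popup widget, then a chain of per-game booleans picks the display text and shows the Cube if that milestone flag is set.
; Sphere overlap shows the popup text only while the Cube is visible, and end overlap hides it.
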(event `self.ReceiveBeginPlay`
  (bind _asbp_game_instance (cast `/Game/Global_Userinterface/BP_GameInstance` (`GameplayStatics.GetGameInstance`)))
  (set `self.GameInstance Ref` _asbp_game_instance)
  (bind _returnvalue (`|CreateWidget` "/Game/Arcade(Both)/User-interface/WB_ArcadeSecretCollectables.WB_ArcadeSecretCollectables_C"))
  (set `self.Popup Widget Ref` _returnvalue)
  (`UserWidget.AddToViewport` _returnvalue 0)
  (`Widget.SetVisibility` _returnvalue "Hidden")
  (if (`self.Ping`)
    (set `self.TextToDisplay` (`self.PingText`))
    (if (`/Game/Global_Userinterface/BP_GameInstance.PingFlawless` (`self.GameInstance Ref`))
      (`SceneComponent.SetVisibility` (`self.Cube`) true true))
    (elif (`self.SuperFabio`)
      (set `self.TextToDisplay` (`self.SuperFabioText`))
      (if (`/Game/Global_Userinterface/BP_GameInstance.SuperFabio25+Coins` (`self.GameInstance Ref`))
        (`SceneComponent.SetVisibility` (`self.Cube`) true true))
      (elif (`self.Crash`)
        (set `self.TextToDisplay` (`self.CrashText`))
        (if (`/Game/Global_Userinterface/BP_GameInstance.Crash45+Plums` (`self.GameInstance Ref`))
          (`SceneComponent.SetVisibility` (`self.Cube`) true true))
        (elif (`self.Acoustic`)
          (set `self.TextToDisplay` (`self.AcousticText`))
          (if (`/Game/Global_Userinterface/BP_GameInstance.AcousticHighScore` (`self.GameInstance Ref`))
            (`SceneComponent.SetVisibility` (`self.Cube`) true true))
          (elif (`self.Chrono`)
            (set `self.TextToDisplay` (`self.ChronoText`))
            (if (`/Game/Global_Userinterface/BP_GameInstance.ChronoShotsFired` (`self.GameInstance Ref`))
              (`SceneComponent.SetVisibility` (`self.Cube`) true true))))))))

(event `self.Sphere.OnComponentBeginOverlap`
  (params (OverlappedComponent :type "PrimitiveComponent Object Reference") (OtherActor :type "Actor Object Reference") (OtherComp :type "PrimitiveComponent Object Reference") (OtherBodyIndex :type Integer) (bFromSweep :type Boolean) (SweepResult :type "HitResult Structure (by ref)"))
  (if (`SceneComponent.IsVisible` (`self.Cube`))
    (`/Game/Arcade(Both)/User-interface/WB_ArcadeSecretCollectables.ShowPopup` (`self.Popup Widget Ref`) (`self.TextToDisplay`))))

(event `self.Sphere.OnComponentEndOverlap`
  (params (OverlappedComponent :type "PrimitiveComponent Object Reference") (OtherActor :type "Actor Object Reference") (OtherComp :type "PrimitiveComponent Object Reference") (OtherBodyIndex :type Integer))
  (`/Game/Arcade(Both)/User-interface/WB_ArcadeSecretCollectables.HidePopup` (`self.Popup Widget Ref`)))

(fn `UserConstructionScript`)