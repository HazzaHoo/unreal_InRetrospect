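; Arcade ceiling light actor that stays steady in the modern arcade and main menu levels, and flickers with a hum in other levels.
; BeginPlay checks the level name, then either sets a high RectLight intensity or creates a dynamic emissive material and starts the hum.
; LoopFlicker re-calls itself after random delays, blinking or blacking out the light and material together.
; FadeHum fades out the hum audio.
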(event `self.ReceiveBeginPlay`
  ; Check if Broken Arcade Level
  (bind _returnvalue (`GameplayStatics.GetCurrentLevelName` true))
  (if (or (`KismetStringLibrary.EqualEqual_StrStr` _returnvalue "L_Modern_Arcade") (`KismetStringLibrary.EqualEqual_StrStr` _returnvalue "L_MainMenu"))
    ; Set Dyanmic Emmisive Light Material
    (`LightComponent.SetIntensity` (`self.RectLight`) 1000000.0)
    (else
      (bind _returnvalue_2 (`KismetMaterialLibrary.CreateDynamicMaterialInstance` "/Game/Arcade(Both)/Assets/Materials/M_EmissiveLight.M_EmissiveLight"))
      (bind _output_get (set `self.CubeDynamicMaterial` _returnvalue_2))
      (`PrimitiveComponent.SetMaterial` (`self.Cube`) 0 _output_get)
      (set `self.NormalIntensity` (`LightComponentBase.Intensity` (`self.RectLight`)))
      ; Play Hum Sound Effect
      (`AudioComponent.Play` (`self.Light_Hum_Cue`) 0.0)
      (`self.Loop Flicker`))))

(event `Loop Flicker`
  (bind _returnvalue (`KismetMathLibrary.RandomIntegerInRange` 0 5))
  ; Flicker Light Once or Twice Randomly
  (if (== _returnvalue 0)
    (`KismetSystemLibrary.Delay` 0.2)
    (elif (== _returnvalue 1)
      (`LightComponent.SetIntensity` (`self.RectLight`) 0.0)
      (`MaterialInstanceDynamic.SetScalarParameterValue` (`self.CubeDynamicMaterial`) "EmmisiveBrightness" 0.0)
      (`KismetSystemLibrary.Delay` (`KismetMathLibrary.RandomFloatInRange` 1.0 20.0))
      (else
        (`KismetSystemLibrary.Delay` (`KismetMathLibrary.RandomFloatInRange` 1.0 20.0)))))
  (`LightComponent.SetIntensity` (`self.RectLight`) 0.0)
  (`MaterialInstanceDynamic.SetScalarParameterValue` (`self.CubeDynamicMaterial`) "EmmisiveBrightness" 0.0)
  (`KismetSystemLibrary.Delay` 0.2)
  (`LightComponent.SetIntensity` (`self.RectLight`) (`self.NormalIntensity`))
  (`MaterialInstanceDynamic.SetScalarParameterValue` (`self.CubeDynamicMaterial`) "EmmisiveBrightness" 100.0)
  (`self.Loop Flicker`))

(event `Fade Hum`
  ; Flicker Light Once or Twice Randomly
  (`AudioComponent.FadeOut` (`self.Light_Hum_Cue`) 1.0 0.0 "Linear"))

(fn `UserConstructionScript`)