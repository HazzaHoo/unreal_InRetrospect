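; Arcade replay station that lets the player reopen one of five minigame levels.
; On BeginPlay it enables arcade input, creates a hidden prompt widget and uses a switch index to set the game name, screen material and target level.
; A sphere overlap with the Player tag shows the prompt and sets IsNear.
; Releasing or canceling the pickup input while near plays a load-out widget, then opens the level after a short delay.
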(event `self.ReceiveBeginPlay`
  (bind _returnvalue (`GameplayStatics.GetPlayerController` 0))
  (bind _level_image (`self.Level Image`))
  ; Enable Input
  (`EnhancedInputSubsystemInterface.AddMappingContext` (pcsubsystem `EnhancedInputLocalPlayerSubsystem` _returnvalue) "/Game/Arcade(Both)/IMC/IMC_Arcade_Both.IMC_Arcade_Both" 0 (struct))
  (`self.EnableInput` _returnvalue)
  ; Create Interact Widget
  (bind _returnvalue_2 (`|CreateWidget` "/Game/Arcade(Both)/User-interface/WB_ArcadeMachineInteract.WB_ArcadeMachineInteract_C"))
  (bind _output_get (set `self.Widget Ref` _returnvalue_2))
  (`UserWidget.AddToViewport` _output_get 0)
  (`Widget.SetVisibility` _output_get "Hidden")
  ; Select What Screen is Picked
  (switch `int` (`self.Switch Screen?(0-4)`)
    (:`0`
      (set `self.Game to Play` "Ping")
      (`PrimitiveComponent.SetMaterial` _level_image 0 "/Game/Arcade(Both)/User-interface/Thumbnails/M_PingReplay.M_PingReplay")
      (set `self.LevelToOpen` (`self.Ping_LevelName(0)`)))
    (:`1`
      (set `self.Game to Play` "Super Fabio")
      (`PrimitiveComponent.SetMaterial` _level_image 0 "/Game/Arcade(Both)/User-interface/Thumbnails/superfabio_replay_background_Mat.superfabio_replay_background_Mat")
      (set `self.LevelToOpen` (`self.SuperFabio_LevelName(1)`)))
    (:`2`
      (set `self.Game to Play` "Crash Capybara")
      (`PrimitiveComponent.SetMaterial` _level_image 0 "/Game/Arcade(Both)/User-interface/Thumbnails/CAPY_THUMBNAIL_Mat.CAPY_THUMBNAIL_Mat")
      (set `self.LevelToOpen` (`self.CrashCapybara_LevelName(2)`)))
    (:`3`
      (set `self.Game to Play` "Acoustic Vigilante")
      (`PrimitiveComponent.SetMaterial` _level_image 0 "/Game/Arcade(Both)/User-interface/Thumbnails/vigilante_THUMBNAIL_Mat.vigilante_THUMBNAIL_Mat")
      (set `self.LevelToOpen` (`self.AcousticVigilante_LevelName(3)`)))
    (:`4`
      (set `self.Game to Play` "Chrono Panic")
      (`PrimitiveComponent.SetMaterial` _level_image 0 "/Game/Arcade(Both)/User-interface/Thumbnails/chrono_THUMBNAIL_Mat.chrono_THUMBNAIL_Mat")
      (set `self.LevelToOpen` (`self.ChronoPanic_LevelName(4)`)))))

(event `self.SphereCollision.OnComponentBeginOverlap`
  (params (OverlappedComponent :type "PrimitiveComponent Object Reference") (OtherActor :type "Actor Object Reference") (OtherComp :type "PrimitiveComponent Object Reference") (OtherBodyIndex :type Integer) (bFromSweep :type Boolean) (SweepResult :type "HitResult Structure (by ref)"))
  ; Collision (Show and Hide Widget)
  (if (`self.ActorHasTag` OtherActor "Player")
    (`/Game/Arcade(Both)/User-interface/WB_ArcadeMachineInteract.UpdateText` (`self.Widget Ref`) (`self.InteractPrompt`) (`self.Game to Play`))
    (`/Game/Arcade(Both)/User-interface/WB_ArcadeMachineInteract.Open Interact` (`self.Widget Ref`))
    (set `self.IsNear?` true)))

(event `self.SphereCollision.OnComponentEndOverlap`
  (params (OverlappedComponent :type "PrimitiveComponent Object Reference") (OtherActor :type "Actor Object Reference") (OtherComp :type "PrimitiveComponent Object Reference") (OtherBodyIndex :type Integer))
  ; Collision (Show and Hide Widget)
  (`/Game/Arcade(Both)/User-interface/WB_ArcadeMachineInteract.Close Interact` (`self.Widget Ref`))
  (set `self.IsNear?` false))

(event `EnhancedInput|/Game/Arcade(Both)/IMC/IA_Arcade_Pickup`
  (params (ActionValue :type Boolean) (ElapsedSeconds :type "Float (double-precision)") (TriggeredSeconds :type "Float (double-precision)") (InputAction :type "InputAction Object Reference" :default "/Game/Arcade(Both)/IMC/IA_Arcade_Pickup.IA_Arcade_Pickup"))
  ; Interact and Open Level
  (:`Canceled`
    (if (`self.IsNear?`) :!label _label
      (bind _returnvalue (`|CreateWidget` "/Game/Global_Userinterface/WB_LoadInOrOut.WB_LoadInOrOut_C"))
      (`UserWidget.AddToViewport` _returnvalue 0)
      (`/Game/Global_Userinterface/WB_LoadInOrOut.Load Out` _returnvalue)
      (`KismetSystemLibrary.Delay` 0.5)
      (`GameplayStatics.OpenLevel` (`self.LevelToOpen`))))
  (:`Completed`
    (goto _label)))

(fn `SetImagesAndLevel`
  (params (`Level Name` :type Name) (`Level Image` :type "Material Object Reference"))
  (`PrimitiveComponent.SetMaterial` (`self.Level Image`) 0 "/Game/Arcade(Both)/User-interface/Thumbnails/M_PingReplay.M_PingReplay")
  (set `self.LevelToOpen` `Level Name`))

(fn `UserConstructionScript`)