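; Arcade machine that the player is prompted to fix and, once carrying a coin, to put the coin in.
; Sphere overlaps set the player's NearMachine flag and drive a camera-facing prompt, faded by a timeline on a dynamic material.
; FixMachine only sets the fixed flag.
; SpawnCoin places a coin at a random spawn point, passes it to the player, activates the machine audio and starts a self-recalling text blink.
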(event `TextAppear`
  (bind _textrender (`self.TextRender`))
  (`SceneComponent.SetHiddenInGame` _textrender true false)
  (`KismetSystemLibrary.Delay` 0.5)
  (`SceneComponent.SetHiddenInGame` _textrender false false)
  (`KismetSystemLibrary.Delay` 0.5)
  (`self.TextAppear`))

(event `SpawnCoin`
  ; Spawn Coin at Random Spawn Point
  (bind _outactors (`GameplayStatics.GetAllActorsOfClass` "/Game/Arcade(Both)/Blueprints/BP_CoinSpawnPoints.BP_CoinSpawnPoints_C"))
  (for (_ _array_index) _outactors
    _)
  (set `self.AmountofSpawnPoints` _array_index)
  (bind _returnvalue (`|SpawnActorFromClass` "/Game/Arcade(Both)/Blueprints/BP_CoinPickup.BP_CoinPickup_C" (`self.GetTransform` (`|GetArrayItem` _outactors (`KismetMathLibrary.RandomIntegerInRange` 0 (`self.AmountofSpawnPoints`)))) "Undefined" "MultiplyWithRoot" null null))
  (bind _asbp_arcade_player (cast `/Game/Arcade(Both)/Blueprints/BP_ArcadePlayer` (`GameplayStatics.GetPlayerCharacter` 0)))
  (set `/Game/Arcade(Both)/Blueprints/BP_ArcadePlayer.CoinRef` _returnvalue _asbp_arcade_player)
  (`ActorComponent.Activate` (`self.Retro_Arcade_Machine_Cue`) false)
  (`self.TextAppear`))

(event `Fade Text In`
  ; Fade Text In
  (bind (_direction _fadein) (`Timeline|FadeInOrOutText` :!label _label)
    (:`Update`
      (`MaterialInstanceDynamic.SetScalarParameterValue` (`self.TextMaterial`) "Fade In" _fadein))))

(event `Fade Text Out`
  ; Fade Text In
  (goto _label :!via `Reverse`))

(event `self.ReceiveBeginPlay`
  ; Get Player Ref
  (bind _outactors (`GameplayStatics.GetAllActorsOfClass` "/Game/Arcade(Both)/Blueprints/BP_ArcadePlayer.BP_ArcadePlayer_C"))
  (set `self.Player Ref` (`|GetArrayItem` _outactors))
  (bind _returnvalue (`KismetMaterialLibrary.CreateDynamicMaterialInstance` "/Game/Arcade(Both)/User-interface/M_ArcadeText.M_ArcadeText"))
  (bind _output_get (set `self.TextMaterial` _returnvalue))
  (`TextRenderComponent.SetTextMaterial` (`self.InteractText`) _output_get)
  (`TextRenderComponent.K2_SetText` (`self.InteractText`) (`KismetTextLibrary.Conv_StringToText` "Hold 'E' to Fix"))
  (`MaterialInstanceDynamic.SetScalarParameterValue` (`self.TextMaterial`) "Fade In" 0.0)
  (`SceneComponent.SetHiddenInGame` (`self.InteractText`) false false))

(event `UpdateText`
  (params (UpdateMachineText :type String))
  ; Update Text
  (`self.Fade Text Out`)
  (`KismetSystemLibrary.Delay` 0.5)
  (`TextRenderComponent.K2_SetText` (`self.InteractText`) (`KismetTextLibrary.Conv_StringToText` UpdateMachineText))
  (`self.Fade Text In`))

(event `self.Sphere.OnComponentBeginOverlap`
  (params (OverlappedComponent :type "PrimitiveComponent Object Reference") (OtherActor :type "Actor Object Reference") (OtherComp :type "PrimitiveComponent Object Reference") (OtherBodyIndex :type Integer) (bFromSweep :type Boolean) (SweepResult :type "HitResult Structure (by ref)"))
  (bind _player_ref (`self.Player Ref`))
  (bind _player_ref_2 (`self.Player Ref`))
  ; Machine Collision
  (if (and (== OtherActor _player_ref) (`/Game/Arcade(Both)/Blueprints/BP_ArcadePlayer.GotCoin?` _player_ref))
    (set `/Game/Arcade(Both)/Blueprints/BP_ArcadePlayer.NearMachine?` true _player_ref_2)
    (`self.UpdateText` "'E' to put coin in")
    (elif (`self.MachineFixed`)
      (set `/Game/Arcade(Both)/Blueprints/BP_ArcadePlayer.NearMachine?` true _player_ref_2)
      (else
        (`self.Fade Text In`)
        (set `/Game/Arcade(Both)/Blueprints/BP_ArcadePlayer.NearMachine?` true _player_ref_2)))))

(event `self.Sphere.OnComponentEndOverlap`
  (params (OverlappedComponent :type "PrimitiveComponent Object Reference") (OtherActor :type "Actor Object Reference") (OtherComp :type "PrimitiveComponent Object Reference") (OtherBodyIndex :type Integer))
  (bind _player_ref (`self.Player Ref`))
  ; Machine Collision
  (set `/Game/Arcade(Both)/Blueprints/BP_ArcadePlayer.NearMachine?` false _player_ref)
  (`/Game/Arcade(Both)/Blueprints/BP_ArcadePlayer.HideProgressBar` _player_ref)
  (`self.Fade Text Out`))

(event `Fix Machine`
  ; Fix Machine
  (set `self.MachineFixed` true))

(event `self.ReceiveTick`
  (params (DeltaSeconds :type "Float (single-precision)"))
  ; Rotate Text to Cam
  (`self.Rotate Text to Camera`))

(fn `Rotate Text to Camera`
  (`SceneComponent.K2_SetWorldRotation` (`self.InteractText`) (`KismetMathLibrary.FindLookAtRotation` (`SceneComponent.K2_GetComponentLocation` (`self.InteractText`)) (`SceneComponent.K2_GetComponentLocation` (`/Game/Arcade(Both)/Blueprints/BP_ArcadePlayer.FirstPersonCamera` (`self.Player Ref`)))) false false))

(fn `UserConstructionScript`)