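; BP_MilestoneItems is an arcade actor that displays trophy items for milestones earned across several games: Ping, SuperFabio, Crash, Acoustic and Chrono.
; On BeginPlay it casts the game instance to BP_GameInstance and reads one milestone flag per game.
; Each set flag unhides its matching mesh or sprite and that component's children.
; The check runs only once, at BeginPlay.
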(event `self.ReceiveBeginPlay`
  (bind _asbp_game_instance (cast `/Game/Global_Userinterface/BP_GameInstance` (`GameplayStatics.GetGameInstance`)))
  (bind _output_get (set `self.GameInstanceRef` _asbp_game_instance))
  (if (`/Game/Global_Userinterface/BP_GameInstance.PingFlawless` _output_get)
    (`SceneComponent.SetHiddenInGame` (`self.SM_Ping`) false true))
  (if (`/Game/Global_Userinterface/BP_GameInstance.SuperFabio25+Coins` _output_get)
    (`SceneComponent.SetHiddenInGame` (`self.Sprite_Coin`) false true))
  (if (`/Game/Global_Userinterface/BP_GameInstance.Crash45+Plums` _output_get)
    (`SceneComponent.SetHiddenInGame` (`self.SM_Plum`) false true))
  (if (`/Game/Global_Userinterface/BP_GameInstance.AcousticHighScore` _output_get)
    (`SceneComponent.SetHiddenInGame` (`self.SM_Acoustic`) false true))
  (if (`/Game/Global_Userinterface/BP_GameInstance.ChronoShotsFired` _output_get)
    (`SceneComponent.SetHiddenInGame` (`self.SM_Chrono`) false true)))

(fn `UserConstructionScript`)