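; BP_CC_Progression_Portal is a placeholder progression portal for Crash Capibara that starts dormant.
; BeginPlay deactivates the PortalTrigger component and hides the placeholder render in game.
; An unconnected activation branch compares placeholder score and spawn threshold variables, so the portal never appears through this graph.
; As written, that branch would activate and show the portal while the score is below the threshold.
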(event `self.ReceiveBeginPlay`
  ; Set to hidden at start of game
  (`|ExecutionSequence`
    (:`then_0`
      (`ActorComponent.SetActive` (`self.PortalTrigger`) false false))
    (:`then_1`
      (`SceneComponent.SetHiddenInGame` (`self.PlaceHolder_PortalRender`) true false))))

(fn `UserConstructionScript`)