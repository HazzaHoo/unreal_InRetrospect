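; Player Blueprint for the Crash Capibara game, handling input setup, pausing and progression.
; On BeginPlay it sets the CCGame flag and adds the game-specific and global Enhanced Input mapping contexts; attack, crouch, jump, move and spin events are empty stubs.
; The pause action toggles WBP_PauseMenu, game pause, cursor and input mode, passing CCGame into the widget's ChronoPanic input.
; Overlapping a progression portal loads L_CrashCapybra as a level instance.
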(event `self.ReceiveBeginPlay`
  ; Player Control
  (set `self.CC_Game` true)
  (bind _asplayer_controller (cast `PlayerController` (`self.GetController`)))
  (bind _returnvalue (pcsubsystem `EnhancedInputLocalPlayerSubsystem` _asplayer_controller))
  (`/Engine/EditorBlueprintResources/StandardMacros.IsValid` _returnvalue
    (:`Is Valid`
      (`EnhancedInputSubsystemInterface.AddMappingContext` _returnvalue "/Game/Crash_Capibara/IMC/IMC_CrashCapibara.IMC_CrashCapibara" 0 (struct))
      (`EnhancedInputSubsystemInterface.AddMappingContext` _returnvalue "/Game/Global_IMC/IMC_Global.IMC_Global" 0 (struct)))))

(event `EnhancedInput|/Game/Crash_Capibara/IMC/IA_CC_Attack`
  (params (ActionValue :type Boolean) (ElapsedSeconds :type "Float (double-precision)") (TriggeredSeconds :type "Float (double-precision)") (InputAction :type "InputAction Object Reference" :default "/Game/Crash_Capibara/IMC/IA_CC_Attack.IA_CC_Attack"))
  ; Player Control
)

(event `EnhancedInput|/Game/Crash_Capibara/IMC/IA_CC_Crouch`
  (params (ActionValue :type Boolean) (ElapsedSeconds :type "Float (double-precision)") (TriggeredSeconds :type "Float (double-precision)") (InputAction :type "InputAction Object Reference" :default "/Game/Crash_Capibara/IMC/IA_CC_Crouch.IA_CC_Crouch"))
  ; Player Control
)

(event `EnhancedInput|/Game/Crash_Capibara/IMC/IA_CC_Jump`
  (params (ActionValue :type Boolean) (ElapsedSeconds :type "Float (double-precision)") (TriggeredSeconds :type "Float (double-precision)") (InputAction :type "InputAction Object Reference" :default "/Game/Crash_Capibara/IMC/IA_CC_Jump.IA_CC_Jump"))
  ; Player Control
)

(event `EnhancedInput|/Game/Crash_Capibara/IMC/IA_CC_Move`
  (params (ActionValue :type "Vector2D Structure") (ElapsedSeconds :type "Float (double-precision)") (TriggeredSeconds :type "Float (double-precision)") (InputAction :type "InputAction Object Reference" :default "/Game/Crash_Capibara/IMC/IA_CC_Move.IA_CC_Move"))
  ; Player Control
)

(event `EnhancedInput|/Game/Crash_Capibara/IMC/IA_CC_Spin`
  (params (ActionValue :type Boolean) (ElapsedSeconds :type "Float (double-precision)") (TriggeredSeconds :type "Float (double-precision)") (InputAction :type "InputAction Object Reference" :default "/Game/Crash_Capibara/IMC/IA_CC_Spin.IA_CC_Spin"))
  ; Player Control
)

(event `EnhancedInput|/Game/Global_IMC/IA_Pause`
  (params (ActionValue :type Boolean) (ElapsedSeconds :type "Float (double-precision)") (TriggeredSeconds :type "Float (double-precision)") (InputAction :type "InputAction Object Reference" :default "/Game/Global_IMC/IA_Pause.IA_Pause"))
  (bind _returnvalue (`GameplayStatics.GetPlayerController` 0))
  ;[0.15 0 0 0.5] Call Pause Menu
  (:`Completed`
    (if (not (`self.IsPauseMenuOpen`))
      (set `self.IsPauseMenuOpen` true)
      (bind _returnvalue_2 (`|CreateWidget` "/Game/Global_Userinterface/Pause/WBP_PauseMenu.WBP_PauseMenu_C" _returnvalue false false (`self.CC_Game`)))
      (bind _output_get (set `self.UnpauseMenuWidget` _returnvalue_2))
      (`UserWidget.AddToViewport` _output_get 0)
      (`WidgetBlueprintLibrary.SetInputMode_GameAndUIEx` _returnvalue null)
      (set `PlayerController.bShowMouseCursor` true (`GameplayStatics.GetPlayerController` 0))
      (`GameplayStatics.SetGamePaused` true)
      (else
        (set `self.IsPauseMenuOpen` false)
        (`Widget.RemoveFromParent` (`self.UnpauseMenuWidget`))
        (`GameplayStatics.SetGamePaused` false)
        (`WidgetBlueprintLibrary.SetInputMode_GameOnly` _returnvalue)
        (set `PlayerController.bShowMouseCursor` false (`GameplayStatics.GetPlayerController` 0))))))

(event `self.ReceiveActorBeginOverlap`
  (params (OtherActor :type "Actor Object Reference"))
  ; Progression logic
  (cast `/Game/Crash_Capibara/Blueprints/BP_CC_Progression_Portal` OtherActor)
  (`LevelStreamingDynamic.LoadLevelInstance` "" (0.0 0.0 0.0) (struct) "L_CrashCapybra" null))

(fn `UserConstructionScript`)